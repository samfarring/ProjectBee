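; Background bee AI controller that runs a behavior tree and tracks a simple state enum for the pawn.
; A looping timer pushes the current state to the pawn's state text display.
; When perception senses another background AI, it picks one of two reaction states based on the aggression flag, then a timer restores the default state.
; Getters expose the perception target and current state.
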(event OnPerceptionUpdated(AIPerception)
  (params (UpdatedActors :type Array%20of%20Actor%20Object%20References))
  (for _array_element UpdatedActors
    (bind _info (Class|AIPerceptionComponent|GetActorsPerception (Variables|Default|GetAIPerception) _array_element))
    (Variables|Perception|SetPerceptionTarget (.Target (Utilities|Struct|BreakActorPerceptionBlueprintInfo _info)))
    (if (== (Utilities|GetClass (.Target (Utilities|Struct|BreakActorPerceptionBlueprintInfo _info))) "/Game/ProjectBee/Blueprints/AI/Character/BP_BackgroundAI_Base.BP_BackgroundAI_Base_C")
      (if (Variables|States|GetIsAggressive)
        (Variables|States|SetStates "NewEnumerator3")
        (else
          (Variables|States|SetStates "NewEnumerator2")))
      (Utilities|Time|SetTimerbyEvent (EventDispatchers|CreateEvent :!event Custom|ResetState) (Variables|Timer|GetResetTime))
      (Development|PrintString "Hello"))))

(event Custom|AI_Tick
  (Class|IAI|SetStateText(Message) (Pawn|GetControlledPawn) (Variables|States|GetStates)))

(event Custom|ResetState
  (Variables|States|SetStates "NewEnumerator1"))

(event EventBeginPlay
  (Utilities|Time|SetTimerbyEvent (EventDispatchers|CreateEvent :!event Custom|AI_Tick) (Variables|Tick|GetAITickRate) true)
  (CallFunction|InitVariables)
  (AI|RunBehaviorTree "/Game/ProjectBee/Blueprints/AI/Tree/AI_BaseTree.AI_BaseTree"))

(fn ConstructionScript)

(fn InitVariables
  (Variables|States|SetStates "NewEnumerator1"))

(fn GetPerceptionTarget
  (return (Variables|Perception|GetPerceptionTarget)))

(fn GetStateChange
  (return (Variables|States|GetStates)))