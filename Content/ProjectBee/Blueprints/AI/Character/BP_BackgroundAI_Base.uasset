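; BP_BackgroundAI_Base is a base character for background AI that reacts to being stung.
; On begin play it passes itself to its AI controller through InitMessage, and events let its state text and walk speed be set.
; Any damage counts a sting and shows a sting text for two seconds; health subtraction is left unconnected.
; GetPerceptionTarget and GetStateChange return only empty or default values.
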(event EventSetStateText
  (params (State :type AI_States%20Enum :default "NewEnumerator0"))
  (Rendering|Components|TextRender|SetText (Variables|Default|GetStateText) (Utilities|Text|ToText(String) (Utilities|String|ToString(Byte) State))))

(event EventSetCharacterSpeed
  (params (Speed :type Float%20%28single-precision%29))
  (Variables|/Script/Engine.CharacterMovementComponent|SetMaxWalkSpeed (Variables|Character|GetCharacterMovement) Speed))

(event Game|Damage|EventAnyDamage
  (params (Damage :type Float%20%28single-precision%29) (DamageType :type Damage%20Type%20Object%20Reference) (InstigatedBy :type Controller%20Object%20Reference) (DamageCauser :type Actor%20Object%20Reference))
  (bind _stungtext (Variables|Default|GetStungText))
  (Development|PrintString "Stung")
  (Math|Integer|IncrementInt (Variables|Combat|GetStungAmount)
    (:%20%20
      (Rendering|SetVisibility _stungtext true false)
      (Utilities|FlowControl|Delay 2.0)
      (Rendering|SetVisibility _stungtext false false))))

(event EventBeginPlay
  (bind _self self)
  (Class|IAI|Init(Message) (AI|GetAIController _self) _self))

(fn ConstructionScript)

(fn GetPerceptionTarget
  (return 0))

(fn GetStateChange
  (return "NewEnumerator0"))