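; Quest actor that becomes available at BeginPlay and starts its quest when its QuestZone is overlapped.
; StatusChange stores the quest status and keeps zone collision query-enabled only while Available.
; For a Location first objective, it spawns a visible sphere trigger at runtime, which prints "quest over" and destroys itself on overlap.
; Player filtering is unfinished, and completion never updates the status.
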(event OnComponentBeginOverlap(QuestZone)
  (params (OverlappedComponent :type Primitive%20Component%20Object%20Reference) (OtherActor :type Actor%20Object%20Reference) (OtherComp :type Primitive%20Component%20Object%20Reference) (OtherBodyIndex :type Integer) (bFromSweep :type Boolean) (SweepResult :type Hit%20Result%20Structure%20%28by%20ref%29))
  (Utilities|FlowControl|DoOnce false
    (:Completed
      (if (== OtherActor 0)
        _
        (else
          _))
      (Development|PrintString "quest started")
      (CallFunction|StatusChange "NewEnumerator3")
      (switch Utilities|FlowControl|Switch|SwitchonObjectiveTypes (.Type (Utilities|Struct|BreakQuestStruct (Utilities|Array|Get(acopy) (Variables|Objectives|GetObjectives))))
        (:NewEnumerator2
          (Utilities|FlowControl|DoOnce false
            (:Completed
              (bind _returnvalue (AddComponent|AddSphereComponent false (Math|Conversions|ToTransform(Vector) (Variables|Default|GetLocation))))
              (Collision|AssignOnComponentBeginOverlap _returnvalue (delegate Custom|OnComponentBeginOverlap_Event_1))
              (Components|Sphere|SetSphereRadius _returnvalue 128.0 true)
              (Rendering|SetVisibility _returnvalue true false)
              (Development|SetHiddeninGame _returnvalue false false)
              (Development|PrintString "quest created"))))))))

(event OnComponentEndOverlap(QuestZone)
  (params (OverlappedComponent :type Primitive%20Component%20Object%20Reference) (OtherActor :type Actor%20Object%20Reference) (OtherComp :type Primitive%20Component%20Object%20Reference) (OtherBodyIndex :type Integer))
  (Utilities|FlowControl|DoOnce false) ; enters at Reset
)

(event Custom|OnComponentBeginOverlap_Event_1
  (params (OverlappedComponent :type Primitive%20Component%20Object%20Reference) (OtherActor :type Actor%20Object%20Reference) (OtherComp :type Primitive%20Component%20Object%20Reference) (OtherBodyIndex :type Integer) (bFromSweep :type Boolean) (SweepResult :type Hit%20Result%20Structure%20%28by%20ref%29))
  (Development|PrintString "quest over")
  (Components|DestroyComponent (stale OnComponentBeginOverlap(QuestZone) _returnvalue)))

(event EventBeginPlay
  (CallFunction|StatusChange "NewEnumerator1"))

(fn ConstructionScript)

(fn StatusChange
  (params (NewStatus :type QuestStatus%20Enum :default "NewEnumerator0"))
  (Collision|SetCollisionEnabled (Variables|Default|GetQuestZone) (Utilities|Select :Index NewStatus :NewEnumerator0 "NoCollision" :NewEnumerator1 "QueryOnly" :NewEnumerator2 "NoCollision" :NewEnumerator3 "NoCollision" :NewEnumerator4 "NoCollision"))
  (Variables|QuestDetails|SetQuestStatus NewStatus)
  (return))