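; Player controller Blueprint that forwards player input to the bee character, Bee_BP.
; It caches the controlled pawn at BeginPlay and casts it to Bee_BP on each input event.
; Turn, look and movement axes pass straight to matching functions on the bee, while holding Left Alt toggles its AltCamera flag on and releasing it turns the flag off.
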(event EventBeginPlay
  (Variables|Default|SetControlledPawn (Pawn|GetControlledPawn)))

(event Input|AxisEvents|InputAxisTurn
  (params (AxisValue :type Float%20%28single-precision%29))
  (bind _asbee_bp (Utilities|Casting|CastToBee_BP (Variables|Default|GetControlledPawn)))
  (Default|Turn _asbee_bp AxisValue))

(event Input|AxisEvents|InputAxisLookUp
  (params (AxisValue :type Float%20%28single-precision%29))
  (bind _asbee_bp (Utilities|Casting|CastToBee_BP (Variables|Default|GetControlledPawn)))
  (Default|LookUp _asbee_bp AxisValue))

(event Input|AxisEvents|InputAxisMoveForward
  (params (AxisValue :type Float%20%28single-precision%29))
  (bind _asbee_bp (Utilities|Casting|CastToBee_BP (Variables|Default|GetControlledPawn)))
  (Default|MoveForward _asbee_bp AxisValue))

(event Input|AxisEvents|InputAxisMoveRight
  (params (AxisValue :type Float%20%28single-precision%29))
  (bind _asbee_bp (Utilities|Casting|CastToBee_BP (Variables|Default|GetControlledPawn)))
  (Default|MoveRight _asbee_bp AxisValue))

(event Input|KeyboardEvents|LeftAlt
  (params (Key :type Key%20Structure))
  (bind _controlledpawn (Variables|Default|GetControlledPawn))
  (:Pressed
    (bind _asbee_bp (Utilities|Casting|CastToBee_BP _controlledpawn))
    (Variables|/Game/ProjectBee/Blueprints/Character/Bee_BP.Bee_BP_C|SetAltCamera _asbee_bp true))
  (:Released
    (bind _asbee_bp_2 (Utilities|Casting|CastToBee_BP _controlledpawn))
    (Variables|/Game/ProjectBee/Blueprints/Character/Bee_BP.Bee_BP_C|SetAltCamera _asbee_bp_2 false)))

(fn ConstructionScript)