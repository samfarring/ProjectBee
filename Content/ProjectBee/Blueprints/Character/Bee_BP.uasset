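; Bee_BP is the player-controllable bee, driven by axis inputs for looking and moving.
; Turn and LookUp feed controller yaw and pitch.
; MoveForward adds movement input along the forward vector of the full control rotation, pitch included, so the input direction follows the view up and down.
; MoveRight is an empty stub, and a duplicate movement node is left unconnected.
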(event Custom|MoveRight
  (params (AxisValue :type Float%20%28single-precision%29)))

(event Custom|Turn
  (params (AxisValue :type Float%20%28single-precision%29))
  (Pawn|Input|AddControllerYawInput AxisValue))

(event Custom|LookUp
  (params (AxisValue :type Float%20%28single-precision%29))
  (Pawn|Input|AddControllerPitchInput AxisValue))

(event Custom|MoveForward
  (params (AxisValue :type Float%20%28single-precision%29))
  (bind _returnvalue (Pawn|GetControlRotation :!class /Script/Engine.Pawn))
  (bind (_roll _pitch _yaw) (Math|Rotator|BreakRotator _returnvalue))
  (Pawn|Input|AddMovementInput (Math|Vector|GetForwardVector (Math|Rotator|MakeRotator _roll _pitch _yaw)) AxisValue false))

(fn ConstructionScript)