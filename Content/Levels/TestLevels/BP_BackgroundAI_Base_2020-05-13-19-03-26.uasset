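; Base character for background AI that can be stung by damage and marked as a target, with text labels showing state, stung and target status.
; On BeginPlay it passes itself to its AI controller, and exposes events to set state text and walk speed.
; Damage increments a sting count, calls OnStung, clears target status and shows stung text until a timer hides it.
; Getters expose itself and chaseability; perception and state getters are stubs.
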(event Custom|StungReset
  (Rendering|SetVisibility (Variables|Default|GetStungText) false false))

(event EventSetStateText
  (params (State :type E_AI_States%20Enum :default "NewEnumerator0"))
  (Rendering|Components|TextRender|SetText (Variables|Default|GetStateText) (Utilities|Text|ToText(String) (Utilities|String|ToString(Byte) State))))

(event EventSetCharacterSpeed
  (params (Speed :type Float%20%28single-precision%29))
  (Variables|/Script/Engine.CharacterMovementComponent|SetMaxWalkSpeed (Variables|Character|GetCharacterMovement) Speed))

(event Game|Damage|EventAnyDamage
  (params (Damage :type Float%20%28single-precision%29) (DamageType :type Damage%20Type%20Object%20Reference) (InstigatedBy :type Controller%20Object%20Reference) (DamageCauser :type Actor%20Object%20Reference))
  (Development|PrintString "Stung")
  (Math|Integer|IncrementInt (Variables|Combat|GetStungAmount)
    (:%20%20
      (Rendering|SetVisibility (Variables|Default|GetStungText) true false)
      (Utilities|Time|SetTimerbyEvent (delegate Custom|StungReset) (Variables|Combat|GetStingResetTime))
      (Default|CallOnStung)
      (if (Variables|Combat|GetIsTarget)
        (bind _output_get (Variables|Combat|SetIsTarget false))
        (Rendering|SetVisibility (Variables|Default|GetTargetText) _output_get false)))))

(event EventBeginPlay
  (bind _self self)
  (Class|IAI|Init(Message) (AI|GetAIController _self) _self))

(event EventAssignTarget
  (bind _output_get (Variables|Combat|SetIsTarget true))
  (Rendering|SetVisibility (Variables|Default|GetTargetText) _output_get false))

(fn ConstructionScript)

(fn GetCharacter
  (return self))

(fn GetIsChaseable
  (return (Variables|Combat|GetIsChaseable)))

(fn GetPerceptionTarget
  (return 0))

(fn GetStateChange
  (return "NewEnumerator0"))