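; Stamina pickup Blueprint that restores stamina to a character, built on a parent class whose construction script it calls.
; The Pickup function adds the pickup's Stamina amount to the character's Stamina, capping the result at StaminaMax.
; It always returns true, even when stamina is already full.
; The event graph holds only disabled placeholder events, so the function contains all the logic in this file.
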(event EventBeginPlay)

(event Collision|EventActorBeginOverlap
  (params (OtherActor :type Actor%20Object%20Reference)))

(event EventTick
  (params (DeltaSeconds :type Float%20%28single-precision%29)))

(fn ConstructionScript
  (|CallParentFunction))

(fn Pickup
  (if (> (+ (Variables|/Game/Blueprints/Character/BeeCharacter_BP.BeeCharacter_BP_C|GetStamina (Variables|Default|GetCharacter)) (Variables|Default|GetStamina+)) (Variables|/Game/Blueprints/Character/BeeCharacter_BP.BeeCharacter_BP_C|GetStaminaMax (Variables|Default|GetCharacter)))
    (Variables|/Game/Blueprints/Character/BeeCharacter_BP.BeeCharacter_BP_C|SetStamina (Variables|Default|GetCharacter) (Variables|/Game/Blueprints/Character/BeeCharacter_BP.BeeCharacter_BP_C|GetStaminaMax (Variables|Default|GetCharacter)))
    (return true)
    (else
      (Variables|/Game/Blueprints/Character/BeeCharacter_BP.BeeCharacter_BP_C|SetStamina (Variables|Default|GetCharacter) (+ (Variables|/Game/Blueprints/Character/BeeCharacter_BP.BeeCharacter_BP_C|GetStamina (Variables|Default|GetCharacter)) (Variables|Default|GetStamina+)))
      (return true))))