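; Game mode for the bee game that handles checkpoint saving and loading plus death screens.
; Save and load events store the pawn's location in a BP_BeeSave slot and move the bee back to it.
; BeginPlay binds every checkpoint's save event so the latest saved one changes status and others reset.
; Death shows a UI-only screen, with a one-in-ten chance of an alternate variant, though the MS1 variant is unreachable.
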(event Custom|SetCheckpoint
  (params (Checkpoint :type BP%20Checkpoint%20Object%20Reference))
  (Variables|/Game/Blueprints/Checkpoint/BP_Checkpoint.BP_Checkpoint_C|SetCheckpointStatus Checkpoint "NewEnumerator2")
  (for _array_element (Variables|Default|GetCheckpoints)
    (if (!= _array_element Checkpoint)
      (Variables|/Game/Blueprints/Checkpoint/BP_Checkpoint.BP_Checkpoint_C|SetCheckpointStatus _array_element "NewEnumerator1"))))

(event EventCheckpointSave
  ;[1 1 1] Checkpoint save
  (Utilities|FlowControl|Sequence
    (:then_0
      (Variables|Default|SetBeeLocation (Transformation|GetActorLocation (Game|Player|GetPlayerPawn 0))))
    (:then_1
      (bind _returnvalue (SaveGame|DoesSaveGameExist (Variables|Default|GetSaveSlot)))
      (if _returnvalue
        (bind _returnvalue_2 (SaveGame|LoadGamefromSlot (Variables|Default|GetSaveSlot)))
        (bind _asbp_bee_save (Utilities|Casting|CastToBP_BeeSave _returnvalue_2))
        (Variables|/Game/Blueprints/Checkpoint/BP_BeeSave.BP_BeeSave_C|SetBeeLocation _asbp_bee_save (Variables|Default|GetBeeLocation))
        (SaveGame|SaveGametoSlot _asbp_bee_save (Variables|Default|GetSaveSlot))
        (else
          (bind _returnvalue_3 (SaveGame|CreateSaveGameObject "/Game/Blueprints/Checkpoint/BP_BeeSave.BP_BeeSave_C"))
          (Variables|/Game/Blueprints/Checkpoint/BP_BeeSave.BP_BeeSave_C|SetBeeLocation _returnvalue_3 (Variables|Default|GetBeeLocation))
          (SaveGame|SaveGametoSlot _returnvalue_3 (Variables|Default|GetSaveSlot)))))))

(event EventBeginPlay
  (bind _outactors (Actor|GetAllActorsOfClass "/Game/Blueprints/Checkpoint/BP_Checkpoint.BP_Checkpoint_C"))
  (bind _output_get (Variables|Default|SetCheckpoints _outactors))
  (for _array_element _output_get
    (Variables|/Game/Blueprints/Checkpoint/BP_Checkpoint.BP_Checkpoint_C|SetCheckpointStatus _array_element "NewEnumerator1")
    (EventDispatchers|BindEventtoOnCheckpointSaved _array_element (delegate Custom|SetCheckpoint))))

(event EventBeeDeath
  (Utilities|RandomDeathScreen))

(event EventCheckpointLoad
  ;[1 1 1] Checkpoint Load
  (bind _returnvalue (SaveGame|DoesSaveGameExist (Variables|Default|GetSaveSlot)))
  (if _returnvalue
    (bind _returnvalue_2 (SaveGame|LoadGamefromSlot (Variables|Default|GetSaveSlot)))
    (bind _asbp_bee_save (Utilities|Casting|CastToBP_BeeSave _returnvalue_2))
    (bind _asbee_character_bp (Utilities|Casting|CastToBeeCharacter_BP (Game|Player|GetPlayerPawn 0)))
    (Transformation|SetActorLocation _asbee_character_bp (Variables|/Game/Blueprints/Checkpoint/BP_BeeSave.BP_BeeSave_C|GetBeeLocation _asbp_bee_save) false false)))

(fn ConstructionScript)