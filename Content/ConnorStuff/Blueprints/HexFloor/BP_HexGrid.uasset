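; BP_HexGrid is a hex floor Blueprint that lays out a grid of static mesh tiles in its construction script.
; Nested loops over GridX and GridY add one static mesh component per cell, positioned by SpacingX and SpacingY.
; Odd X columns are shifted along Y by Offset to produce the staggered hex pattern.
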(fn ConstructionScript
  (for _index (range 0 (Variables|Default|GetGridX))
    (for _index_2 (range 0 (Variables|Default|GetGridY))
      (AddComponent|AddStaticMeshComponent false (Math|Transform|MakeTransform (Math|Vector|SelectVector (Math|Vector|MakeVector (* _index (Variables|Default|GetSpacingX)) (* _index_2 (Variables|Default|GetSpacingY)) 0.0) (Math|Vector|MakeVector (* _index (Variables|Default|GetSpacingX)) (+ (Variables|Default|GetOffset) (* _index_2 (Variables|Default|GetSpacingY))) 0.0) (== (Math|Integer|%(Integer) _index 2) 0)) "0, 0, 0" "1,1,1")))))