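; GM_Bee is a game mode that shows a death screen when its BeeDeath event fires.
; RandomDeathScreen rolls a one-in-ten chance for a rare screen, picked evenly between the DS and MGS3 variants, and otherwise shows the standard W_DeathScreen.
; Each branch creates the widget for player 0, adds it to the viewport, sets UI-only input focused on it and shows the mouse cursor.
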(event EventBeeDeath
  (Utilities|RandomDeathScreen))

(fn ConstructionScript)