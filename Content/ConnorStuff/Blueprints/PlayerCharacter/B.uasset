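; Player pawn B, driven as a physics sphere with mouse look and a HUD widget created at begin play.
; Movement axes apply forces to Sphere1 along the control rotation, while Tick applies a custom Gravity force.
; Space spends Stamina on an upward impulse-like force, briefly zeroing Gravity behind a DoOnce that resets after the delay.
; StaminaRegen is an empty stub, so this graph never restores stamina.
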(event Custom|StaminaRegen)

(event EventBeginPlay
  (bind _returnvalue (UserInterface|CreateWidget "/Game/UI/HUD.HUD_C" (Game|GetPlayerController 0)))
  (UserInterface|Viewport|AddtoViewport _returnvalue 0))

(event EventTick
  (params (DeltaSeconds :type Float%20%28single-precision%29))
  (Physics|AddForce (Variables|Default|GetSphere1) (Variables|Default|GetGravity) "None" false))

(event Input|AxisEvents|InputAxisMouseX
  (params (AxisValue :type Float%20%28single-precision%29))
  (Pawn|Input|AddControllerYawInput AxisValue))

(event Input|AxisEvents|InputAxisMouseY
  (params (AxisValue :type Float%20%28single-precision%29))
  (Pawn|Input|AddControllerPitchInput AxisValue))

(event Input|AxisEvents|InputAxisMoveForward
  (params (AxisValue :type Float%20%28single-precision%29))
  (Physics|AddForce (Variables|Default|GetSphere1) (* (* (Math|Vector|GetForwardVector (Pawn|GetControlRotation :!class /Script/Engine.Pawn)) AxisValue) 1e+04) "None" false))

(event Input|AxisEvents|InputAxisMoveRight
  (params (AxisValue :type Float%20%28single-precision%29))
  (Physics|AddForce (Variables|Default|GetSphere1) (* (* (Math|Vector|GetRightVector (Pawn|GetControlRotation :!class /Script/Engine.Pawn)) AxisValue) 1e+04) "None" false))

(event Input|KeyboardEvents|SpaceBar
  (params (Key :type Key%20Structure))
  (bind _stamina (Variables|Default|GetStamina))
  (:Pressed
    (if (not (< _stamina 1))
      (Utilities|FlowControl|DoOnce false :!label _label
        (:Completed
          (Math|Integer|DecrementInt _stamina
            (:%20%20
              (Physics|AddForce (Variables|Default|GetSphere1) "0, 0,300000.000000" "None" false)
              (Variables|Default|SetGravity "0, 0, 0")
              (Utilities|FlowControl|Delay 0.2)
              (Variables|Default|SetGravity "0, 0,-10000.000000")
              (goto _label Reset))))))))

(fn ConstructionScript)