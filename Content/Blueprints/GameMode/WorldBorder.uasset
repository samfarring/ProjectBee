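; World border actor that warns the player bee when it strays outside a sphere.
; Leaving the sphere changes the bee camera's post-process saturation, zeroing green and blue, and shows a warning widget; re-entering restores saturation and removes the widget.
; Two DoOnce nodes reset each other so enter and exit effects alternate.
; The construction script sizes the sphere from the tutorial or world radius.
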(event OnComponentEndOverlap(Sphere)
  (params (OverlappedComponent :type Primitive%20Component%20Object%20Reference) (OtherActor :type Actor%20Object%20Reference) (OtherComp :type Primitive%20Component%20Object%20Reference) (OtherBodyIndex :type Integer))
  (Utilities|FlowControl|Sequence
    (:then_0
      (Utilities|FlowControl|DoOnce false
        (:Completed
          ;[1 1 1] Saturating the view (UI Red ring needed with a text warning the player)
          (bind _asbee_character_bp (Utilities|Casting|CastToBeeCharacter_BP OtherActor))
          (Variables|/Script/Engine.CameraComponent|SetPostProcessSettings (Variables|/Game/Blueprints/Character/BeeCharacter_BP.BeeCharacter_BP_C|GetCamera _asbee_character_bp) (Utilities|Struct|MakePostProcessSettings (Math|Vector4|MakeVector4 1.0 0.0 0.0 1.0)))
          (bind _returnvalue (UserInterface|CreateWidget "/Game/Widgets/W_Warning.W_Warning_C"))
          (UserInterface|Viewport|AddtoViewport _returnvalue 0))))
    (:then_1
      (Utilities|FlowControl|DoOnce false) ; enters at Reset
    )))

(event OnComponentBeginOverlap(Sphere)
  (params (OverlappedComponent :type Primitive%20Component%20Object%20Reference) (OtherActor :type Actor%20Object%20Reference) (OtherComp :type Primitive%20Component%20Object%20Reference) (OtherBodyIndex :type Integer) (bFromSweep :type Boolean) (SweepResult :type Hit%20Result%20Structure%20%28by%20ref%29))
  (Utilities|FlowControl|Sequence
    (:then_0
      (Utilities|FlowControl|DoOnce false
        (:Completed
          ;[1 1 1] Saturating the view (UI Red ring needed with a text warning the player)
          (bind _asbee_character_bp (Utilities|Casting|CastToBeeCharacter_BP OtherActor))
          (Variables|/Script/Engine.CameraComponent|SetPostProcessSettings (Variables|/Game/Blueprints/Character/BeeCharacter_BP.BeeCharacter_BP_C|GetCamera _asbee_character_bp) (Utilities|Struct|MakePostProcessSettings (Math|Vector4|MakeVector4 1.0 1.0 1.0 1.0)))
          (Utilities|IsValid (stale OnComponentEndOverlap(Sphere) _returnvalue)
            (:Is%20Valid
              (Widget|RemovefromParent (stale OnComponentEndOverlap(Sphere) _returnvalue)))))))
    (:then_1
      (Utilities|FlowControl|DoOnce false) ; enters at Reset
    )))

(fn ConstructionScript
  (if (Variables|Default|GetInTutorial?)
    (Components|Sphere|SetSphereRadius (Variables|Default|GetSphere) (Math|Conversions|ToFloat(Integer) (Variables|Default|GetTutorialRadius)) true)
    (else
      (Components|Sphere|SetSphereRadius (Variables|Default|GetSphere) (Math|Conversions|ToFloat(Integer) (Variables|Default|GetWorldRadius)) true))))