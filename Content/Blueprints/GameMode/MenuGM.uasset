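; Main menu game mode that runs the front end: music, menu widgets, a live backdrop and the hand-off to gameplay.
; Main menu dispatchers drive Options, Credits, Quit and Play, which shows a loading screen that opens L_PersistentLevel when ready.
; When LiveMenuLevel is set, a looping timer blends the menu controller between random level cameras.
; Shuffled AI spawners populate the scene with NPCs, capped per location by AISpawnValues.
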(event Custom|PressedPlay
  (bind _returnvalue (Game|GetPlayerController 0))
  (Utilities|FlowControl|DoOnce false
    (:Completed
      (Input|SetInputModeGameOnly _returnvalue)
      (Variables|/Script/Engine.PlayerController|SetbShowMouseCursor _returnvalue false)
      (bind _returnvalue_2 (UserInterface|CreateWidget "/Game/Widgets/W_loadingScreen.W_loadingScreen_C"))
      (EventDispatchers|BindEventtoReadytoOpenLevelDispatch _returnvalue_2 (EventDispatchers|CreateEvent :!event Custom|ReadyToOpenLevel))
      (Default|InitLoadingScreen _returnvalue_2)
      (UserInterface|Viewport|AddtoViewport _returnvalue_2 0))))

(event Custom|BindMenuEvents
  (EventDispatchers|BindEventtoPressedPlayDispatch (Variables|Default|GetmainMenuWigRef) (EventDispatchers|CreateEvent :!event Custom|PressedPlay))
  (EventDispatchers|BindEventtoPressedOptionsDispatch (Variables|Default|GetmainMenuWigRef) (EventDispatchers|CreateEvent :!event Custom|PressedOptions))
  (EventDispatchers|BindEventtoPressedQuitDispatch (Variables|Default|GetmainMenuWigRef) (EventDispatchers|CreateEvent :!event Custom|PressedQuit))
  (EventDispatchers|BindEventtoPressedCreditsDispatch (Variables|Default|GetmainMenuWigRef) (EventDispatchers|CreateEvent :!event Custom|PressedCredits)))

(event Custom|AISpawning
  (bind _outactors (Actor|GetAllActorsOfClass "/Game/Blueprints/AI/BP_AISpawner.BP_AISpawner_C"))
  (bind _output_get (Variables|Default|SetAISpawners _outactors))
  (bind _keys (Utilities|Map|Keys (Variables|Default|GetAISpawnValues)))
  (for _array_element _keys
    (Variables|Default|SetSpawnCount 0)
    (Utilities|Array|Shuffle _output_get)
    (bind _array_element_2 (Utilities|Array|ForEachLoopwithBreak _output_get)
      (:LoopBody
        (if (Utilities|Enum|Equal(Enum) (Variables|/Game/Blueprints/AI/BP_AISpawner.BP_AISpawner_C|GetLocation _array_element_2) _array_element)
          (bind _result (Math|Integer|IncrementInt (Variables|Default|GetSpawnCount))
            (:%20%20
              (if (not (> _result (.Value (Utilities|Map|Find (Variables|Default|GetAISpawnValues) _array_element))))
                (Default|SpawnNPC _array_element_2)))))))))

(event Custom|PressedOptions
  (bind _returnvalue (UserInterface|CreateWidget "/Game/Widgets/Menu/W_OptionsMenu.W_OptionsMenu_C"))
  (bind _output_get (Variables|Default|SetOptionsWidget _returnvalue))
  (Default|Init _output_get false)
  (EventDispatchers|BindEventtoOnReturntoMenu _output_get (EventDispatchers|CreateEvent :!event Custom|Return))
  (UserInterface|Viewport|AddtoViewport _output_get 0)
  (Widget|RemovefromParent (Variables|Default|GetmainMenuWigRef)))

(event Custom|PressedQuit
  (Game|QuitGame 0 "Quit" false))

(event Custom|Init_MenuGM
  (bind _optionswidget (Variables|Default|GetOptionsWidget))
  (bind _returnvalue (UserInterface|CreateWidget "/Game/Widgets/Menu/W_MainMenu.W_MainMenu_C"))
  (bind _output_get (Variables|Default|SetmainMenuWigRef _returnvalue))
  (UserInterface|Viewport|AddtoViewport _output_get 0)
  (Default|InitMainMenu _output_get)
  (CallFunction|BindMenuEvents)
  (Variables|/Script/Engine.PlayerController|SetbShowMouseCursor (Game|GetPlayerController 0) true)
  (Utilities|IsValid _optionswidget
    (:Is%20Valid
      (Widget|RemovefromParent _optionswidget))))

(event Custom|ReadyToOpenLevel
  (Game|OpenLevel(byName) "L_PersistentLevel" true (Variables|Level|GetOptions)))

(event Custom|LiveCameras
  (bind _cameraactors (Variables|Default|GetCameraActors))
  (Utilities|Time|SetTimerbyEvent (delegate Custom|CameraSwitch) (Variables|Default|GetCameraChangeTime) true)
  (Class|IMainMenu|ChangeCamera(Message) (Variables|Default|GetMenuCon) (Utilities|Array|Get(acopy) _cameraactors (Math|Random|RandomInteger (- (Utilities|Array|Length _cameraactors) 1))) 0.0))

(event Custom|CameraSwitch
  (bind _cameraactors (Variables|Default|GetCameraActors))
  (Class|IMainMenu|ChangeCamera(Message) (Variables|Default|GetMenuCon) (Utilities|Array|Get(acopy) _cameraactors (Math|Random|RandomInteger (- (Utilities|Array|Length _cameraactors) 1))) 2.0))

(event Custom|Return
  (bind _optionswidget (Variables|Default|GetOptionsWidget))
  (bind _returnvalue (UserInterface|CreateWidget "/Game/Widgets/Menu/W_MainMenu.W_MainMenu_C"))
  (bind _output_get (Variables|Default|SetmainMenuWigRef _returnvalue))
  (UserInterface|Viewport|AddtoViewport _output_get 0)
  (Default|InitMainMenu _output_get)
  (CallFunction|BindMenuEvents)
  (Variables|/Script/Engine.PlayerController|SetbShowMouseCursor (Game|GetPlayerController 0) true)
  (Utilities|IsValid _optionswidget
    (:Is%20Valid
      (Widget|RemovefromParent _optionswidget))))

(event Custom|PressedCredits
  (bind _returnvalue (UserInterface|CreateWidget "/Game/Widgets/Menu/W_credits.W_credits_C"))
  (Default|InitCreditsScreen _returnvalue)
  (UserInterface|Viewport|AddtoViewport _returnvalue 1))

(event EventDeleteSave
  (SaveGame|DeleteGameinSlot (Variables|Default|GetSaveSlotName)))

(event EventBeginPlay
  ;[1 1 1] Stream Level Delay
  (Utilities|FlowControl|Delay 0.2)
  (Input|SetInputModeUIOnly (Game|GetPlayerController 0) 0 "DoNotLock")
  (CallFunction|InitMenuGM)
  (Default|CreateTransitionWidget (.AsBee%20Instance (Utilities|Casting|CastToBeeInstance (Game|GetGameInstance))))
  (CallFunction|LiveCameraSetUp)
  (CallFunction|AISpawning)
  (Audio|PlaySound2D "/Game/Audio/Soundtracks/MainMenuCue.MainMenuCue" 1.0 1.0 0.0 0 0)
  ;[1 1 1] Border BUg
  (bind _foundwidgets (Widget|GetAllWidgetsOfClass "/Game/Widgets/W_Warning.W_Warning_C" true))
  (for _array_element _foundwidgets
    (Widget|RemovefromParent _array_element)))

(event EventOpenLevel
  (bind _optionswidget (Variables|Default|GetOptionsWidget))
  (bind _returnvalue (UserInterface|CreateWidget "/Game/Widgets/Menu/W_MainMenu.W_MainMenu_C"))
  (bind _output_get (Variables|Default|SetmainMenuWigRef _returnvalue))
  (UserInterface|Viewport|AddtoViewport _output_get 0)
  (Default|InitMainMenu _output_get)
  (CallFunction|BindMenuEvents)
  (Variables|/Script/Engine.PlayerController|SetbShowMouseCursor (Game|GetPlayerController 0) true)
  (Utilities|IsValid _optionswidget
    (:Is%20Valid
      (Widget|RemovefromParent _optionswidget))))

(event EventLoadMenu
  (Game|OpenLevel(byName) "L_PersistentLevel" true "?game=/Game/Blueprints/GameMode/MenuGM.MenuGM_C"))

(fn ConstructionScript)

(fn LiveCameraSetUp
  (if (Variables|Default|GetLiveMenuLevel)
    (bind _outactors (Actor|GetAllActorsOfClass "/Game/Blueprints/Cameras/CameraActor.CameraActor_C"))
    (Variables|Default|SetCameraActors _outactors)
    (bind _outactors_2 (Actor|GetAllActorsOfClass "/Game/Blueprints/Character/BP_MenuController.BP_MenuController_C"))
    (Variables|Default|SetMenuCon (Utilities|Array|Get(acopy) _outactors_2))
    (CallFunction|LiveCameras)))