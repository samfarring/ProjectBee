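; Main gameplay game mode for the bee game, running level setup, play timer, pause, death, ending credits and return to menu.
; BeginPlay restores checkpoint position, time and stings from BP_BeeSave, then binds checkpoints and world borders and starts music.
; Shuffled spawners place NPCs up to per-location quotas and respawn them in the same location on death.
; Separate events save quest and quit-game progress; bee death picks a standard or random alternate screen.
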(event Custom|UI_CreateLoadingScreen
  ;[1 1 1] Create Loading Screen
  (if (Variables|Default|GetUIDebug)
    (bind _returnvalue (UserInterface|CreateWidget "/Game/Widgets/W_loadingScreen.W_loadingScreen_C" 0 true))
    (Default|InitLoadingScreen _returnvalue)
    (UserInterface|Viewport|AddtoViewport _returnvalue 1)
    (EventDispatchers|BindEventtoEnteredLevelDispatch _returnvalue (delegate Custom|DestroyLoadingScreen))))

(event Custom|SetCheckpoint
  (params (Checkpoint :type BP%20Checkpoint%20Object%20Reference))
  ;[1 1 1] Set Checkpoint
  (Variables|/Game/Blueprints/Checkpoint/BP_Checkpoint.BP_Checkpoint_C|SetCheckpointStatus Checkpoint "NewEnumerator2")
  (for _array_element (Variables|Default|GetCheckpoints)
    (if (!= _array_element Checkpoint)
      (Variables|/Game/Blueprints/Checkpoint/BP_Checkpoint.BP_Checkpoint_C|SetCheckpointStatus _array_element "NewEnumerator1"))))

(event Custom|AISpawning
  ;[1 1 1] Initial AI Spawn
  (bind _outactors (Actor|GetAllActorsOfClass "/Game/Blueprints/AI/BP_AISpawner.BP_AISpawner_C"))
  (bind _output_get (Variables|Default|SetAISpawners _outactors))
  (bind _keys (Utilities|Map|Keys (Variables|Default|GetAISpawnValues)))
  (for _array_element _keys
    (Variables|Default|SetSpawnCount 0)
    (Utilities|Array|Shuffle _output_get)
    (bind _array_element_2 (Utilities|Array|ForEachLoopwithBreak _output_get)
      (:LoopBody
        (if (Utilities|Enum|Equal(Enum) (Variables|/Game/Blueprints/AI/BP_AISpawner.BP_AISpawner_C|GetLocation _array_element_2) _array_element)
          (bind _result (Math|Integer|IncrementInt (Variables|Default|GetSpawnCount))
            (:%20%20
              (if (not (> _result (.Value (Utilities|Map|Find (Variables|Default|GetAISpawnValues) _array_element))))
                (Default|SpawnNPC _array_element_2))))))
      (:Completed
        (bind _outactors_2 (Actor|GetAllActorsOfClass "/Game/Blueprints/AI/Character/BP_Civilian.BP_Civilian_C"))
        (for _array_element_3 _outactors_2
          (EventDispatchers|BindEventtoOnDead _array_element_3 (EventDispatchers|CreateEvent :!event Custom|OnAIDead)))))))

(event Custom|LoadQuitGame
  ;[1 1 1] Load Quit Game
  (bind _returnvalue (SaveGame|DoesSaveGameExist (Variables|Default|GetSaveSlot)))
  (if _returnvalue
    (bind _returnvalue_2 (SaveGame|LoadGamefromSlot (Variables|Default|GetSaveSlot)))
    (bind _asbp_bee_save (Utilities|Casting|CastToBP_BeeSave _returnvalue_2))
    (Variables|Default|SetTimerSec (Variables|/Game/Blueprints/Checkpoint/BP_BeeSave.BP_BeeSave_C|GetGameTimeSec _asbp_bee_save))
    (Variables|Default|SetTimerMin (Variables|/Game/Blueprints/Checkpoint/BP_BeeSave.BP_BeeSave_C|GetGameTimeMin _asbp_bee_save))
    (Variables|Default|SetTimerHour (Variables|/Game/Blueprints/Checkpoint/BP_BeeSave.BP_BeeSave_C|GetGameTimeHour _asbp_bee_save))
    (bind _asbee_character_bp (Utilities|Casting|CastToBeeCharacter_BP (Game|Player|GetPlayerPawn 0)))
    (Variables|/Game/Blueprints/Character/BeeCharacter_BP.BeeCharacter_BP_C|SetStingCounter _asbee_character_bp (Variables|/Game/Blueprints/Checkpoint/BP_BeeSave.BP_BeeSave_C|GetBeeStingCounter _asbp_bee_save))))

(event Custom|OnAIDead
  (params (Actor :type BP%20Background%20AI%20Base%20Object%20Reference))
  (bind _aispawners (Variables|Default|GetAISpawners))
  ;[1 1 1] Bind AI on Death
  (Utilities|Array|Shuffle _aispawners)
  (bind _array_element (Utilities|Array|ForEachLoopwithBreak _aispawners :!label _label)
    (:LoopBody
      (if (Utilities|Enum|Equal(Enum) (Variables|/Game/Blueprints/AI/BP_AISpawner.BP_AISpawner_C|GetLocation _array_element) (Variables|/Game/Blueprints/AI/Character/BP_BackgroundAI_Base.BP_BackgroundAI_Base_C|GetBaseLocation Actor))
        (Variables|Default|SetSelectedSpawner _array_element)
        (goto _label Break)))
    (:Completed
      (bind _spawned (Default|SpawnNPC (Variables|Default|GetSelectedSpawner)))
      (EventDispatchers|BindEventtoOnDead _spawned (EventDispatchers|CreateEvent :!event Custom|OnAIDead)))))

(event Custom|SaveQuestProgress
  ;[1 1 1] Save quest progress (I havent tested this so it may or may not work)
  (bind _outactors (Actor|GetAllActorsOfClass "/Game/Blueprints/QuestSystem/BP_QuestActor.BP_QuestActor_C"))
  (for _array_element _outactors
    (if (Utilities|Enum|Equal(Enum) (Variables|/Game/Blueprints/QuestSystem/BP_QuestActor.BP_QuestActor_C|GetQuestStatus _array_element) "NewEnumerator4")
      (Utilities|Array|AddUnique (Variables|Default|GetCompletedQuests) _array_element)
      (bind _returnvalue (SaveGame|DoesSaveGameExist (Variables|Default|GetSaveSlot)))
      (if _returnvalue
        (bind _returnvalue_2 (SaveGame|LoadGamefromSlot (Variables|Default|GetSaveSlot)))
        (bind _asbp_bee_save (Utilities|Casting|CastToBP_BeeSave _returnvalue_2))
        (Variables|/Game/Blueprints/Checkpoint/BP_BeeSave.BP_BeeSave_C|SetCompletedQuests _asbp_bee_save (Variables|Default|GetCompletedQuests))
        (SaveGame|SaveGametoSlot _returnvalue_2 (Variables|Default|GetSaveSlot))
        (else
          (bind _returnvalue_3 (SaveGame|CreateSaveGameObject "/Game/Blueprints/Checkpoint/BP_BeeSave.BP_BeeSave_C"))
          (bind _asbp_bee_save_2 (Utilities|Casting|CastToBP_BeeSave _returnvalue_3))
          (Variables|/Game/Blueprints/Checkpoint/BP_BeeSave.BP_BeeSave_C|SetCompletedQuests _asbp_bee_save_2 (Variables|Default|GetCompletedQuests))
          (SaveGame|SaveGametoSlot _returnvalue_3 (Variables|Default|GetSaveSlot)))))))

(event Custom|LoadQuestProgress
  ;[1 1 1] Load quest progress (Once again i have not saved this so it may or may not work)
  (bind _returnvalue (SaveGame|DoesSaveGameExist (Variables|Default|GetSaveSlot)))
  (if _returnvalue
    (bind _returnvalue_2 (SaveGame|LoadGamefromSlot (Variables|Default|GetSaveSlot)))
    (bind _asbp_bee_save (Utilities|Casting|CastToBP_BeeSave _returnvalue_2))
    (bind _outactors (Actor|GetAllActorsOfClass "/Game/Blueprints/QuestSystem/BP_QuestActor.BP_QuestActor_C"))
    (for _array_element _outactors
      (if (Utilities|Array|ContainsItem (Variables|/Game/Blueprints/Checkpoint/BP_BeeSave.BP_BeeSave_C|GetCompletedQuests _asbp_bee_save) _array_element)
        (Variables|/Game/Blueprints/QuestSystem/BP_QuestActor.BP_QuestActor_C|SetQuestStatus _array_element "NewEnumerator4")))))

(event Custom|UIBounds
  (bind _foundwidgets (Widget|GetAllWidgetsOfClass "/Game/Widgets/W_UIManager.W_UIManager_C" true))
  (Default|ReturnBounds (Utilities|Array|Get(acopy) _foundwidgets)))

(event Custom|PlayerStings
  ;[1 1 1] BeginPlay
  ;;[1 1 1] Da Fuck is this for?
  (bind _result (Math|Integer|IncrementInt (Variables|Default|GetStingCounter))))

(event Custom|DestroyLoadingScreen
  ;[1 1 1] Create Loading Screen
  (Widget|RemovefromParent (stale Custom|UI_CreateLoadingScreen _returnvalue)))

(event Custom|TimerStart
  ;[1 1 1] Timer (Now with less sarcasm)
  (Utilities|Time|SetTimerbyEvent (delegate Custom|Timer) 1.0 true))

(event Custom|Timer
  ;[1 1 1] Timer (Now with less sarcasm)
  (if (not (Variables|Default|GetGamePaused?))
    (Variables|Default|SetTimerSec (+ (Variables|Default|GetTimerSec) 1))
    (if (> (Variables|Default|GetTimerSec) 59)
      (Variables|Default|SetTimerSec 0)
      (Variables|Default|SetTimerMin (+ (Variables|Default|GetTimerMin) 1))
      (if (> (Variables|Default|GetTimerMin) 59)
        (Variables|Default|SetTimerMin 0)
        (Variables|Default|SetTimerHour (+ (Variables|Default|GetTimerHour) 1))))))

(event Custom|ReadyToOpenLevel
  (CallFunction|LoadMenu))

(event Custom|OutOfBounds
  (params (Tutorial :type Boolean))
  ;[1 1 1] Out Of Bounds volume?
  (bind _outvol (Class|IInstance|GetVolume(Message) (Game|GetGameInstance)))
  (Audio|SetSoundMixClassOverride "/Game/Audio/MasterSoundMix.MasterSoundMix" "/Game/Audio/Soundtracks/MusicSoundClass.MusicSoundClass" _outvol 1.0 1.0 true))

(event Custom|OnReturn
  ;[1 1 1] Out Of Bounds volume?
  (bind _outvol (Class|IInstance|GetVolume(Message) (Game|GetGameInstance)))
  (Audio|SetSoundMixClassOverride "/Game/Audio/MasterSoundMix.MasterSoundMix" "/Game/Audio/Soundtracks/MusicSoundClass.MusicSoundClass" _outvol 1.0 1.0 true))

(event Custom|LoadCheckpoint
  ;[1 1 1] Checkpoint Load
  (bind _returnvalue (SaveGame|DoesSaveGameExist (Variables|Default|GetSaveSlot)))
  (if _returnvalue
    (bind _returnvalue_2 (SaveGame|LoadGamefromSlot (Variables|Default|GetSaveSlot)))
    (bind _asbp_bee_save (Utilities|Casting|CastToBP_BeeSave _returnvalue_2))
    (bind _asbee_character_bp (Utilities|Casting|CastToBeeCharacter_BP (Game|Player|GetPlayerPawn 0)))
    (Transformation|SetActorLocation _asbee_character_bp (Variables|/Game/Blueprints/Checkpoint/BP_BeeSave.BP_BeeSave_C|GetBeeLocation _asbp_bee_save) false true)))

(event Custom|QuitGameSave
  ;[1 1 1] Quit Game Save logic (Do you think other games have save logic thats this loooooooooooooong?)
  (bind _returnvalue (SaveGame|DoesSaveGameExist (Variables|Default|GetSaveSlot)))
  (if _returnvalue
    (bind _returnvalue_2 (SaveGame|LoadGamefromSlot (Variables|Default|GetSaveSlot)))
    (bind _asbp_bee_save (Utilities|Casting|CastToBP_BeeSave _returnvalue_2))
    (Variables|/Game/Blueprints/Checkpoint/BP_BeeSave.BP_BeeSave_C|SetGameTimeSec _asbp_bee_save (Variables|Default|GetTimerSec))
    (Variables|/Game/Blueprints/Checkpoint/BP_BeeSave.BP_BeeSave_C|SetGameTimeMin _asbp_bee_save (Variables|Default|GetTimerMin))
    (Variables|/Game/Blueprints/Checkpoint/BP_BeeSave.BP_BeeSave_C|SetGameTimeHour _asbp_bee_save (Variables|Default|GetTimerHour))
    (bind _asbee_character_bp (Utilities|Casting|CastToBeeCharacter_BP (Game|Player|GetPlayerPawn 0)))
    (Variables|/Game/Blueprints/Checkpoint/BP_BeeSave.BP_BeeSave_C|SetBeeStingCounter _asbp_bee_save (Variables|/Game/Blueprints/Character/BeeCharacter_BP.BeeCharacter_BP_C|GetStingCounter _asbee_character_bp))
    (SaveGame|SaveGametoSlot _returnvalue_2 (Variables|Default|GetSaveSlot))
    (else
      (bind _returnvalue_3 (SaveGame|CreateSaveGameObject "/Game/Blueprints/Checkpoint/BP_BeeSave.BP_BeeSave_C"))
      (Variables|/Game/Blueprints/Checkpoint/BP_BeeSave.BP_BeeSave_C|SetGameTimeSec _returnvalue_3 (Variables|Default|GetTimerSec))
      (Variables|/Game/Blueprints/Checkpoint/BP_BeeSave.BP_BeeSave_C|SetGameTimeMin _returnvalue_3 (Variables|Default|GetTimerMin))
      (Variables|/Game/Blueprints/Checkpoint/BP_BeeSave.BP_BeeSave_C|SetGameTimeHour _returnvalue_3 (Variables|Default|GetTimerHour))
      (bind _asbee_character_bp_2 (Utilities|Casting|CastToBeeCharacter_BP (Game|Player|GetPlayerPawn 0)))
      (Variables|/Game/Blueprints/Checkpoint/BP_BeeSave.BP_BeeSave_C|SetBeeStingCounter _returnvalue_3 (Variables|/Game/Blueprints/Character/BeeCharacter_BP.BeeCharacter_BP_C|GetStingCounter _asbee_character_bp_2))
      (SaveGame|SaveGametoSlot _returnvalue_3 (Variables|Default|GetSaveSlot)))))

(event EventGameEnd
  (Class|ICharacter|GameEnd(Message) (Game|Player|GetPlayerPawn 0))
  (Utilities|FlowControl|Sequence
    (:then_0
      (Utilities|FlowControl|Delay 2.0)
      (bind _returnvalue (UserInterface|CreateWidget "/Game/Widgets/W_BlackScreen.W_BlackScreen_C"))
      (UserInterface|Viewport|AddtoViewport _returnvalue 0)
      (Utilities|FlowControl|Delay (Class|WidgetAnimation|GetEndTime (Variables|/Game/Widgets/W_BlackScreen.W_BlackScreen_C|GetFadeToBlack _returnvalue)))
      (bind _returnvalue_2 (UserInterface|CreateWidget "/Game/Widgets/Menu/W_credits.W_credits_C"))
      (Widget|RemovefromParent _returnvalue)
      (Default|InitCreditsScreen _returnvalue_2 true)
      (UserInterface|Viewport|AddtoViewport _returnvalue_2 0))
    (:then_1
      (bind _time (Timeline|Timeline_0 Play)
        (:Update
          (Utilities|Time|SetGlobalTimeDilation _time))
        (:Finished
          (Utilities|FlowControl|Delay 1.0)
          (Utilities|Time|SetGlobalTimeDilation 1.0))))))

(event EventBeginPlay
  ;[1 1 1] BeginPlay
  (Variables|Default|SetGamePaused? false)
  (Input|SetInputModeGameOnly (Game|GetPlayerController 0))
  (CallFunction|UICreateLoadingScreen)
  (Class|GameplayStatics|SetBaseSoundMix "/Game/Audio/MasterSoundMix.MasterSoundMix")
  ;;[1 1 1] Volume
  (bind _outvol (Class|IInstance|GetVolume(Message) (Game|GetGameInstance)))
  (Audio|SetSoundMixClassOverride "/Game/Audio/MasterSoundMix.MasterSoundMix" "/Game/Audio/Soundtracks/MusicSoundClass.MusicSoundClass" _outvol 1.0 1.0 true)
  (CallFunction|SetTutorial)
  (CallFunction|LoadCheckpoint)
  (CallFunction|BoundsInit)
  (CallFunction|CheckpointInit)
  (CallFunction|LoadQuitGame)
  (CallFunction|TimerStart)
  (CallFunction|AISpawning)
  (CallFunction|SetMusic)
  ;;[1 1 1] Da Fuck is this for?
  (bind _asbee_character_bp (Utilities|Casting|CastToBeeCharacter_BP (Game|Player|GetPlayerPawn 0)))
  (EventDispatchers|BindEventtoOnSting _asbee_character_bp (delegate Custom|PlayerStings)))

(event EventPauseGame
  ;[1 1 1] Game Pause/Resume
  (Utilities|Time|SetGlobalTimeDilation 0.0)
  (Variables|Default|SetGamePaused? true))

(event EventResumeGame
  ;[1 1 1] Game Pause/Resume
  (Utilities|Time|SetGlobalTimeDilation 1.0)
  (Variables|Default|SetGamePaused? false))

(event EventMissionSave)

(event EventMissionLoad)

(event EventCollectibleSave)

(event EventCollectibleLoad)

(event EventLoadMenu
  ;[1 1 1] Load Menu
  (Game|OpenLevel(byName) "L_PersistentLevel" true "?game=/Game/Blueprints/GameMode/MenuGM.MenuGM_C"))

(event EventReturntoMenu
  (bind _warningwidgetref (Variables|Default|GetWarningWidgetRef))
  ;[1 1 1] Return to Menu
  (Utilities|Time|SetGlobalTimeDilation 1.0)
  (Utilities|IsValid _warningwidgetref
    (:Is%20Valid
      (Widget|RemovefromParent _warningwidgetref)
      (CallFunction|LoadMenu))))

(event EventBeeDeath
  ;[1 1 1] Bee Death
  (Audio|SetSoundMixClassOverride "/Game/Audio/MasterSoundMix.MasterSoundMix" "/Game/Audio/Soundtracks/MusicSoundClass.MusicSoundClass" 0.0 1.0 1.0 true)
  (Audio|PlaySound2D "/Game/Audio/SFX/Tim/snd_beeDeath.snd_beeDeath" 1.0 1.0 0.0 0 0)
  (Default|CallOnBeeDeath)
  (Utilities|RandomDeathScreen))

(event EventPrepareEnd
  (Class|GameplayStatics|SetBaseSoundMix "/Game/Audio/MasterSoundMix.MasterSoundMix")
  (Audio|SetSoundMixClassOverride "/Game/Audio/MasterSoundMix.MasterSoundMix" "/Game/Audio/MasterSoundClass.MasterSoundClass" 0.0 1.0 1.0 true))

(event EventSetDizzy
  (params (Dizzy :type Boolean))
  (Variables|Default|SetIsDizzy Dizzy))

(event EventEndGameClicked
  (Variables|/Script/Engine.PlayerController|SetbShowMouseCursor (Game|GetPlayerController 0) false)
  (bind _returnvalue (UserInterface|CreateWidget "/Game/Widgets/W_loadingScreen.W_loadingScreen_C"))
  (EventDispatchers|BindEventtoReadytoOpenLevelDispatch _returnvalue (delegate Custom|ReadyToOpenLevel))
  (Default|InitLoadingScreen _returnvalue)
  (UserInterface|Viewport|AddtoViewport _returnvalue 0)
  (Audio|PlaySound2D "/Game/Audio/SFX/Menus/MenuSelectCue.MenuSelectCue" 1.0 1.0 0.0 0 0))

(event EventReloadGame
  ;[1 1 1] Reload Game
  (Game|OpenLevel(byName) "L_PersistentLevel" true "?game=/Game/Blueprints/GameMode/GM_Bee.GM_Bee_C"))

(event EventStartCredits
  (bind _creditscroll (Timeline|Timeline_1 PlayFromStart)
    (:Update
      (Default|CallOnUpdateCredits _creditscroll))
    (:Finished
      (Variables|/Script/Engine.PlayerController|SetbShowMouseCursor (Game|GetPlayerController 0) false)
      (bind _returnvalue (UserInterface|CreateWidget "/Game/Widgets/W_loadingScreen.W_loadingScreen_C"))
      (EventDispatchers|BindEventtoReadytoOpenLevelDispatch _returnvalue (delegate Custom|ReadyToOpenLevel))
      (Default|InitLoadingScreen _returnvalue)
      (UserInterface|Viewport|AddtoViewport _returnvalue 0)
      (Audio|PlaySound2D "/Game/Audio/SFX/Menus/MenuSelectCue.MenuSelectCue" 1.0 1.0 0.0 0 0))))

(fn ConstructionScript)

(fn CheckpointInit
  (bind _outactors (Actor|GetAllActorsOfClass "/Game/Blueprints/Checkpoint/BP_Checkpoint.BP_Checkpoint_C"))
  (bind _output_get (Variables|Default|SetCheckpoints _outactors))
  (for _array_element _output_get
    (Variables|/Game/Blueprints/Checkpoint/BP_Checkpoint.BP_Checkpoint_C|SetCheckpointStatus _array_element "NewEnumerator1")
    (EventDispatchers|BindEventtoOnCheckpointSaved _array_element (EventDispatchers|CreateEvent :!event Custom|SetCheckpoint))))

(fn BoundsInit
  (bind _outactors (Actor|GetAllActorsOfClass "/Game/Blueprints/GameMode/WorldBorder.WorldBorder_C"))
  (for _array_element _outactors
    (EventDispatchers|BindEventtoOnOutOfBounds _array_element (EventDispatchers|CreateEvent :!event Custom|OutOfBounds))
    (EventDispatchers|BindEventtoOnReturn _array_element (EventDispatchers|CreateEvent :!event Custom|OnReturn))))

(fn SetMusic
  (bind _outactors (Actor|GetAllActorsOfClass "/Game/Blueprints/Managers/MusicManager.MusicManager_C"))
  (for _array_element _outactors
    (Default|Music _array_element)))

(fn SetTutorial
  (bind _asbee_instance (Utilities|Casting|CastToBeeInstance (Game|GetGameInstance)))
  (if (not (Variables|/Game/Blueprints/Instance/BeeInstance.BeeInstance_C|GetTutorialEnabled _asbee_instance))
    (bind _outactors (Actor|GetAllActorsOfClass "/Game/Blueprints/GameMode/WorldBorder.WorldBorder_C"))
    (for _array_element _outactors
      (if (Variables|/Game/Blueprints/GameMode/WorldBorder.WorldBorder_C|GetInTutorial? _array_element)
        (Actor|DestroyActor _array_element)))))

(fn CreditTimePassed
  (return 0.0))

(fn GetDizzy
  (return (Variables|Default|GetIsDizzy)))