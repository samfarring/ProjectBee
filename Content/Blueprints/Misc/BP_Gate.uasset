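; Gate set piece where a beekeeper pops up and two metal gates are blasted open as the bee player approaches.
; BeginPlay stores the BeeKeeper's location and hides it below, then a sphere overlap with BeeCharacter_BP restores it and plays a van jump-out animation.
; The overlap also opens a Gate node fed by Tick, which is never closed, so both gates receive an impulse along the Arrow every frame thereafter.
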(event OnComponentBeginOverlap(Sphere)
  (params (OverlappedComponent :type Primitive%20Component%20Object%20Reference) (OtherActor :type Actor%20Object%20Reference) (OtherComp :type Primitive%20Component%20Object%20Reference) (OtherBodyIndex :type Integer) (bFromSweep :type Boolean) (SweepResult :type Hit%20Result%20Structure%20%28by%20ref%29))
  (Utilities|Casting|CastToBeeCharacter_BP OtherActor)
  (Transformation|SetRelativeLocation (Variables|Default|GetBeeKeeper) (Variables|Default|GetBeginLocation) false false)
  (Components|Animation|PlayAnimation (Variables|Default|GetBeeKeeper) "/Game/ArtAssets/Animations/Beekeeper/Sequences/BeeKeeperJumpOuttaVan_EnginerReady.BeeKeeperJumpOuttaVan_EnginerReady" false)
  (Utilities|FlowControl|Gate true) ; enters at Open
)

(event EventBeginPlay
  (bind _beekeeper (Variables|Default|GetBeeKeeper))
  (Variables|Default|SetBeginLocation (Variables|/Script/Engine.SceneComponent|GetRelativeLocation _beekeeper))
  (Transformation|SetRelativeLocation _beekeeper "0, 0,-300.000000" false false))

(event EventTick
  (params (DeltaSeconds :type Float%20%28single-precision%29))
  (Utilities|FlowControl|Gate true
    (:Exit
      (Physics|AddImpulse (Variables|Default|Geta_MetalGate1) (* (Math|Vector|GetForwardVector (Variables|Default|GetArrow)) 1e+04) "None" false))))

(fn ConstructionScript)