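; MusicManager is a manager Blueprint that plays the in-game music and background world ambience and controls music volume.
; On BeginPlay it sets a base sound mix, starts music after a delay if enabled, and plays the atmosphere cue as 2D sound.
; SetQuiet and SetLoud events mute or restore the music by overriding the music sound class within the soundtrack mix, leaving the ambience call untouched.
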(event Custom|Music
  (if (Variables|Default|GetEnableMusic)
    (Utilities|FlowControl|Delay (Variables|Default|GetStartDelay))
    (Audio|PlaySound2D "/Game/Audio/Soundtracks/InGameMusicCue.InGameMusicCue" 1.0 1.0 0.0 0 0)))

(event Custom|Atmosphere
  (Audio|PlaySound2D "/Game/Audio/SFX/Ambience/BackgroundWorld_Cue.BackgroundWorld_Cue" 1.0 1.0 0.0 0 0))

(event Custom|SetQuiet
  (Audio|SetSoundMixClassOverride "/Game/Audio/SoundtrackMix.SoundtrackMix" "/Game/Audio/Soundtracks/MusicSoundClass.MusicSoundClass" 0.0 1.0 1.0 true))

(event Custom|SetLoud
  (Audio|SetSoundMixClassOverride "/Game/Audio/SoundtrackMix.SoundtrackMix" "/Game/Audio/Soundtracks/MusicSoundClass.MusicSoundClass" 1.0 1.0 1.0 true))

(event EventBeginPlay
  (Class|GameplayStatics|SetBaseSoundMix "/Game/Audio/SoundtrackMix.SoundtrackMix")
  (CallFunction|Music)
  (CallFunction|Atmosphere))

(fn ConstructionScript)