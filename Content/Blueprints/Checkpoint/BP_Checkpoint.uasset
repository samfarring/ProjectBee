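; BP_Checkpoint is a checkpoint actor that saves the bee character's position when the bee overlaps it.
; On overlap by a BeeCharacter_BP, it captures player pawn 0's location rather than its own.
; It writes that location into the existing BP_BeeSave in SaveSlot, or creates one if none exists, then saves.
; Debug strings report overlap, save and failed cast; restoring the position is not handled here.
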(event Collision|EventActorBeginOverlap
  (params (OtherActor :type Actor%20Object%20Reference))
  (if (== (Utilities|GetClass OtherActor) "/Game/Blueprints/Character/BeeCharacter_BP.BeeCharacter_BP_C")
    (Utilities|FlowControl|Sequence
      (:then_0
        (Development|PrintString "Pens")
        (bind _asbee_character_bp (Utilities|Casting|CastToBeeCharacter_BP (Game|Player|GetPlayerPawn 0)))
        (Variables|Default|SetBeeLocation (Transformation|GetActorLocation _asbee_character_bp)))
      (:then_1
        (bind _returnvalue (SaveGame|DoesSaveGameExist (Variables|Default|GetSaveSlot)))
        (if _returnvalue
          (bind _returnvalue_2 (SaveGame|LoadGamefromSlot (Variables|Default|GetSaveSlot)))
          (bind _asbp_bee_save (Utilities|Casting|CastToBP_BeeSave _returnvalue_2)
            (:then
              (Variables|/Game/Blueprints/Checkpoint/BP_BeeSave.BP_BeeSave_C|SetBeeLocation _asbp_bee_save (Variables|Default|GetBeeLocation))
              (SaveGame|SaveGametoSlot _asbp_bee_save (Variables|Default|GetSaveSlot))
              (Development|PrintString "PensButTheGameSaved"))
            (:CastFailed
              (Development|PrintString "BrokeAsHell")))
          (else
            (bind _returnvalue_3 (SaveGame|CreateSaveGameObject "/Game/Blueprints/Checkpoint/BP_BeeSave.BP_BeeSave_C"))
            (Variables|/Game/Blueprints/Checkpoint/BP_BeeSave.BP_BeeSave_C|SetBeeLocation _returnvalue_3 (Variables|Default|GetBeeLocation))
            (SaveGame|SaveGametoSlot _returnvalue_3 (Variables|Default|GetSaveSlot))
            (Development|PrintString "PensButTheGameSaved")))))))

(fn ConstructionScript)