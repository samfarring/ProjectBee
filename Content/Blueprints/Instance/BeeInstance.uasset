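; BeeInstance holds shared game state: the current checkpoint, master volume and whether the tutorial is enabled.
; Simple setter events store each value, and GetVolume returns the master volume.
; The level transition UI is unfinished: CreateTransitionWidget is empty, and the logic that creates the W_loadingScreen widget and adds it to the viewport is disconnected.
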(event Custom|CreateTransitionWidget
  ;[0.2529 0 1] Tim - Level Transition UI (not ready)
)

(event EventSetVolume
  (params (InVol :type Float%20%28single-precision%29))
  (Variables|Settings|SetMasterVolume InVol))

(event EventSetCurrentStats
  (params (LastCheckpoint :type Vector :default "0, 0, 0"))
  (Variables|Default|SetCurrentCheckpoint LastCheckpoint))

(event EventEnableTutorial
  (params (Enabled :type Boolean))
  (Variables|Default|SetTutorialEnabled Enabled))

(fn GetVolume
  (return (Variables|Settings|GetMasterVolume)))