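; BP_Spire is a breakable puzzle spire that, when damaged while stingable, splits and topples its top toward a goal location.
; BeginPlay hides the base and top pieces 1000 units down; the first valid hit destroys the intact mesh and restores them.
; The top then simulates physics while the FallAlpha timeline steers its X and Y toward GoalLocation.
; ChangeToStingable switches collision channel and enables damage, though BeginPlay currently forces Stingable on for testing.
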(event Custom|ChangeToStingable
  ;[1 1 1] The bee keeper needs to feed to this event
  (Utilities|FlowControl|DoOnce false
    (:Completed
      (Collision|SetCollisionObjectType (Variables|Default|GetSpire) "ECC_GameTraceChannel2")
      (Variables|Default|SetStingable? true))))

(event Game|Damage|EventAnyDamage
  (params (Damage :type Float%20%28single-precision%29) (DamageType :type Damage%20Type%20Object%20Reference) (InstigatedBy :type Controller%20Object%20Reference) (DamageCauser :type Actor%20Object%20Reference))
  (bind _toplocation (Variables|Default|GetTopLocation))
  (bind _goallocation (Variables|Default|GetGoalLocation))
  (bind _spiretop (Variables|Default|GetSpireTop))
  (bind _spiretop_2 (Variables|Default|GetSpireTop))
  (bind _returnvalue (Transformation|GetWorldLocation _goallocation))
  (bind _relativelocation (Variables|/Script/Engine.SceneComponent|GetRelativeLocation _spiretop))
  (if (Variables|Default|GetStingable?)
    (Utilities|FlowControl|DoOnce false
      (:Completed
        (Components|DestroyComponent (Variables|Default|GetSpire))
        (Transformation|SetRelativeLocation (Variables|Default|GetSpireBase) (Variables|Default|GetBaseLocation) false false)
        (Transformation|SetRelativeLocation _spiretop_2 (+ (Variables|Default|GetTopLocation) "0, 0,10.000000") false false)
        (Utilities|FlowControl|Delay 0.2)
        (Physics|SetSimulatePhysics _spiretop_2 true)
        (Variables|Default|SetFalling? true)
        (bind _alpha (Timeline|FallAlpha PlayFromStart)
          (:Update
            (Transformation|SetWorldLocation (Variables|Default|GetSpireTop) (Math|Vector|Lerp(Vector) (Math|Vector|MakeVector (.x _toplocation) (.y _toplocation) (.z _relativelocation)) (Math|Vector|MakeVector (.x _returnvalue) (.y _returnvalue) (.z _relativelocation)) _alpha) false false)))))))

(event EventBeginPlay
  (Variables|Default|SetTopLocation (Variables|/Script/Engine.SceneComponent|GetRelativeLocation (Variables|Default|GetSpireTop)))
  (Variables|Default|SetBaseLocation (Variables|/Script/Engine.SceneComponent|GetRelativeLocation (Variables|Default|GetSpireBase)))
  (Transformation|SetRelativeLocation (Variables|Default|GetSpireBase) "0, 0,-1000.000000" false false)
  (Physics|SetSimulatePhysics (Variables|Default|GetSpireTop) false)
  ;[1 1 1] FOR TESTING- Remove this later
  (Variables|Default|SetStingable? true))

(fn ConstructionScript)