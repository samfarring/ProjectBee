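; Poppable balloon puzzle actor that pops when it takes any damage.
; On damage, it notifies a valid Quest through StingQuestReturn and plays the pop sound, then in all cases spawns an explosion emitter and destroys itself.
; The construction script runs the parent's script and applies the BalloonColour material to the balloon, while the StingNPC event is left empty.
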(event Game|Damage|EventAnyDamage
  (params (Damage :type Float%20%28single-precision%29) (DamageType :type Damage%20Type%20Object%20Reference) (InstigatedBy :type Controller%20Object%20Reference) (DamageCauser :type Actor%20Object%20Reference))
  (bind _balloonpop (Variables|Default|GetBalloonPop))
  (bind _returnvalue (Transformation|GetWorldLocation _balloonpop))
  (Utilities|IsValid (stale EventStingNPC Quest)
    (:Is%20Valid
      (Default|StingQuestReturn (stale EventStingNPC Quest))
      (Audio|PlaySoundatLocation "/Game/Audio/SFX/Misc/snd_Balloon_pop.snd_Balloon_pop" _returnvalue "0, 0, 0" 1.0 1.0 0.0 0 0 0))
    (:Is%20Not%20Valid
      _))
  (Effects|SpawnEmitteratLocation "/Game/Blueprints/Particles/Explosion.Explosion" _returnvalue)
  (Actor|DestroyActor))

(event EventStingNPC
  (params (Quest :type BP%20Quest%20Actor%20Object%20Reference)))

(fn ConstructionScript
  (|CallParentFunction)
  (Rendering|Material|SetMaterial (Variables|Default|GetBalloon) 0 (Variables|Default|GetBalloonColour)))