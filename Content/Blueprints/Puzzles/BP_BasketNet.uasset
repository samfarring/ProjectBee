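; BP_BasketNet is a basketball net puzzle actor that celebrates when a grabbable basketball lands in it.
; Its Sphere overlap accepts only BP_Grabbale_BasketBall actors and stores the ball in BasketRef.
; It then spawns a firework emitter at the Cube's transform, plays two audio components and destroys the emitter after a short delay.
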(event OnComponentBeginOverlap(Sphere)
  (params (OverlappedComponent :type Primitive%20Component%20Object%20Reference) (OtherActor :type Actor%20Object%20Reference) (OtherComp :type Primitive%20Component%20Object%20Reference) (OtherBodyIndex :type Integer) (bFromSweep :type Boolean) (SweepResult :type Hit%20Result%20Structure%20%28by%20ref%29))
  (bind _cube (Variables|Default|GetCube))
  (bind _asbp_grabbale_basket_ball (Utilities|Casting|CastToBP_Grabbale_BasketBall OtherActor))
  (Variables|Default|SetBasketRef _asbp_grabbale_basket_ball)
  (bind _returnvalue (Effects|SpawnEmitteratLocation "/Game/Blueprints/Particles/Firework.Firework" (Transformation|GetWorldLocation _cube) (Transformation|GetWorldRotation _cube)))
  (Audio|Components|Audio|Play (Variables|Default|GetAudio) 0.0)
  (Utilities|FlowControl|Delay 1.0)
  (Components|DestroyComponent _returnvalue))

(fn ConstructionScript)