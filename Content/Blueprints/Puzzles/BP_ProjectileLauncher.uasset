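; BP_ProjectileLauncher is a puzzle turret that tracks the bee character and shoots tennis projectiles at it.
; Overlapping one sphere starts a looping timer that rotates the root toward the bee, gated to run only while it stays inside.
; Overlapping the other sphere opens a gate for delayed firing, which spawns an aimed projectile and explosion effect at the barrel, then sets another timer.
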(event OnComponentBeginOverlap(Sphere1)
  (params (OverlappedComponent :type Primitive%20Component%20Object%20Reference) (OtherActor :type Actor%20Object%20Reference) (OtherComp :type Primitive%20Component%20Object%20Reference) (OtherBodyIndex :type Integer) (bFromSweep :type Boolean) (SweepResult :type Hit%20Result%20Structure%20%28by%20ref%29))
  (bind _defaultsceneroot (Variables|Default|GetDefaultSceneRoot))
  ;[1 1 1] Bee Tracking
  (bind _asbee_character_bp (Utilities|Casting|CastToBeeCharacter_BP OtherActor))
  (Variables|Default|SetBeeChar _asbee_character_bp)
  (Utilities|Time|SetTimerbyEvent (delegate Custom|BeeTrack) 0.05 true)
  (Utilities|FlowControl|Gate true) ; enters at Open
)

(event OnComponentBeginOverlap(Sphere)
  (params (OverlappedComponent :type Primitive%20Component%20Object%20Reference) (OtherActor :type Actor%20Object%20Reference) (OtherComp :type Primitive%20Component%20Object%20Reference) (OtherBodyIndex :type Integer) (bFromSweep :type Boolean) (SweepResult :type Hit%20Result%20Structure%20%28by%20ref%29))
  (bind _gunbarrel (Variables|Default|GetGunBarrel))
  (bind _gunbarrel_2 (Variables|Default|GetGunBarrel))
  (bind _returnvalue (Transformation|GetWorldLocation _gunbarrel_2))
  (Variables|Default|SetTargetFound true)
  (bind _asbee_character_bp (Utilities|Casting|CastToBeeCharacter_BP OtherActor))
  (Variables|Default|SetBeeChar _asbee_character_bp)
  (Utilities|Time|SetTimerbyEvent (delegate Custom|Fire) 1.0)
  (Utilities|FlowControl|Gate true) ; enters at Open
)

(event OnComponentEndOverlap(Sphere1)
  (params (OverlappedComponent :type Primitive%20Component%20Object%20Reference) (OtherActor :type Actor%20Object%20Reference) (OtherComp :type Primitive%20Component%20Object%20Reference) (OtherBodyIndex :type Integer))
  (bind _defaultsceneroot (Variables|Default|GetDefaultSceneRoot))
  ;[1 1 1] Bee Tracking
  (Utilities|Casting|CastToBeeCharacter_BP OtherActor)
  (Utilities|FlowControl|Gate true) ; enters at Close
)

(event OnComponentEndOverlap(Sphere)
  (params (OverlappedComponent :type Primitive%20Component%20Object%20Reference) (OtherActor :type Actor%20Object%20Reference) (OtherComp :type Primitive%20Component%20Object%20Reference) (OtherBodyIndex :type Integer))
  (bind _gunbarrel (Variables|Default|GetGunBarrel))
  (bind _gunbarrel_2 (Variables|Default|GetGunBarrel))
  (bind _returnvalue (Transformation|GetWorldLocation _gunbarrel_2))
  (Variables|Default|SetTargetFound false)
  (Utilities|Casting|CastToBeeCharacter_BP OtherActor)
  (Utilities|FlowControl|Gate true) ; enters at Close
)

(event Custom|Fire
  (bind _gunbarrel (Variables|Default|GetGunBarrel))
  (bind _gunbarrel_2 (Variables|Default|GetGunBarrel))
  (bind _returnvalue (Transformation|GetWorldLocation _gunbarrel_2))
  (Utilities|FlowControl|Gate true
    (:Exit
      (Game|SpawnActorfromClass "/Game/Blueprints/Puzzles/BP_TennisProjectile.BP_TennisProjectile_C" (Math|Transform|MakeTransform _returnvalue (Math|Rotator|FindLookatRotation _returnvalue (Transformation|GetActorLocation (Variables|Default|GetBeeChar))) "1,1,1") "Undefined" self 0)
      (Effects|SpawnEmitteratLocation "/Game/Blueprints/Particles/Explosion.Explosion" (Transformation|GetWorldLocation _gunbarrel) (Transformation|GetWorldRotation _gunbarrel))
      (Utilities|Time|SetTimerbyEvent (EventDispatchers|CreateEvent :!event Custom|Fire) (Variables|Default|GetTime)))))

(event Custom|BeeTrack
  (bind _defaultsceneroot (Variables|Default|GetDefaultSceneRoot))
  ;[1 1 1] Bee Tracking
  (Utilities|FlowControl|Gate true
    (:Exit
      (Transformation|SetWorldRotation _defaultsceneroot (Math|Rotator|FindLookatRotation (Transformation|GetWorldLocation _defaultsceneroot) (Transformation|GetActorLocation (Variables|Default|GetBeeChar))) false false))))

(fn ConstructionScript)