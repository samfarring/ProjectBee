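; Football goal puzzle actor that detects a grabbable football entering its trigger Box and keeps score.
; A scored ball fires a firework emitter at the Cube and calls EventFiringReturn on Quest.
; After a short delay it removes the firework, increments Score, destroys the ball and spawns a replacement soccer ball at CentreCircle.
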(event OnComponentBeginOverlap(Box)
  (params (OverlappedComponent :type Primitive%20Component%20Object%20Reference) (OtherActor :type Actor%20Object%20Reference) (OtherComp :type Primitive%20Component%20Object%20Reference) (OtherBodyIndex :type Integer) (bFromSweep :type Boolean) (SweepResult :type Hit%20Result%20Structure%20%28by%20ref%29))
  (bind _cube (Variables|Default|GetCube))
  (bind _centrecircle (Variables|Default|GetCentreCircle))
  (bind _asbp_grabbable_football (Utilities|Casting|CastToBP_Grabbable_Football OtherActor))
  (Variables|Default|SetFootballRef _asbp_grabbable_football)
  (bind _returnvalue (Effects|SpawnEmitteratLocation "/Game/Blueprints/Particles/Firework.Firework" (Transformation|GetWorldLocation _cube) (Transformation|GetWorldRotation _cube)))
  (Default|EventFiringReturn (stale EventEventFiring Quest))
  (Utilities|FlowControl|Delay 1.0)
  (Components|DestroyComponent _returnvalue)
  (Variables|Default|SetScore (+ (Variables|Default|GetScore) 1))
  (Actor|DestroyActor _asbp_grabbable_football)
  (Game|SpawnActorfromClass "/Game/Blueprints/Grabbables/BP_Grabbable_Football.BP_Grabbable_Football_C" (Math|Transform|MakeTransform (Transformation|GetWorldLocation _centrecircle) (Transformation|GetWorldRotation _centrecircle) "1,1,1") "Undefined" 0 "/Game/ArtAssets/Models/Soccerball.Soccerball" 0))

(event EventBeginPlay
  (Variables|Default|SetScore (Variables|Default|GetScore)))

(event EventEventFiring
  (params (Quest :type BP%20Quest%20Actor%20Object%20Reference) (Bee :type Bee%20Character%20BP%20Object%20Reference)))

(fn ConstructionScript)