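; Tree Blueprint that holds a referenced beehive in place and drops it when the tree's mesh is hit.
; BeginPlay moves the hive to a scene component with physics off and WorldDynamic collision ignored.
; The first hit, not yet filtered to a specific NPC, enables hive physics and starts a looping velocity check.
; Once the hive stops moving downward, HitFloor restores WorldDynamic blocking and clears the timer.
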(event OnComponentHit(StaticMesh)
  (params (HitComponent :type Primitive%20Component%20Object%20Reference) (OtherActor :type Actor%20Object%20Reference) (OtherComp :type Primitive%20Component%20Object%20Reference) (NormalImpulse :type Vector :default "0, 0, 0") (Hit :type Hit%20Result%20Structure%20%28by%20ref%29))
  (bind _beehivereference (Variables|Default|GetBeeHiveReference))
  (bind _staticmesh (Variables|/Game/Blueprints/Grabbables/BP_Grabbable.BP_Grabbable_C|GetStaticMesh _beehivereference))
  ;[1 1 1] Needs to check that its hit by the specific NPC
  (Utilities|FlowControl|DoOnce false
    (:Completed
      (Utilities|Time|SetTimerbyFunctionName 0 "CheckIfFalling" 0.1 true)
      (Physics|SetSimulatePhysics _staticmesh true)
      (Collision|SetCollisionResponsetoChannel _staticmesh "ECC_WorldDynamic" "ECR_Ignore"))))

(event Custom|HitFloor
  (Collision|SetCollisionResponsetoChannel (Variables|/Game/Blueprints/Grabbables/BP_Grabbable.BP_Grabbable_C|GetStaticMesh (Variables|Default|GetBeeHiveReference)) "ECC_WorldDynamic" "ECR_Block")
  (Utilities|Time|ClearTimerbyFunctionName 0 "CheckIfFalling"))

(event EventBeginPlay
  (bind _beehivereference (Variables|Default|GetBeeHiveReference))
  (bind _staticmesh (Variables|/Game/Blueprints/Grabbables/BP_Grabbable.BP_Grabbable_C|GetStaticMesh _beehivereference))
  (Transformation|SetActorLocation _beehivereference (Transformation|GetWorldLocation (Variables|Default|GetScene)) false false)
  (Collision|SetCollisionResponsetoChannel _staticmesh "ECC_WorldDynamic" "ECR_Ignore")
  (Physics|SetSimulatePhysics _staticmesh false))

(fn ConstructionScript)

(fn CheckifFalling
  (if (not (< (.z (Transformation|GetVelocity (Variables|Default|GetBeeHiveReference))) 0.0))
    (Utilities|FlowControl|DoOnce false
      (:Completed
        (CallFunction|HitFloor)
        (return)))))