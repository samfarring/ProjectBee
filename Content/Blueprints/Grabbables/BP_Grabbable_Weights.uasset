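; BP_Grabbable_Weights is a grabbable weight that completes a quest event once it is held for 10 seconds without release.
; EventFiring starts a looping Check timer, which passes through a gate opened on grab and a DoOnce to start the countdown.
; Releasing cancels the countdown, closes the gate and resets the DoOnce.
; When the countdown ends, it calls EventFiringReturn on the Quest and stops polling.
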(event Custom|Check
  (Utilities|FlowControl|Gate true
    (:Exit
      (Utilities|FlowControl|DoOnce false
        (:Completed
          (bind _returnvalue (Utilities|Time|SetTimerbyEvent (delegate Custom|Timer) 1e+01))
          (Variables|Default|SetTimerHandle _returnvalue))))))

(event Custom|Timer
  (Default|EventFiringReturn (stale EventEventFiring Quest))
  (Utilities|Time|ClearandInvalidateTimerbyHandle (stale EventEventFiring _returnvalue)))

(event EventGrabStart
  (Utilities|FlowControl|Gate true) ; enters at Open
)

(event EventGrabEnd
  (Utilities|Time|ClearandInvalidateTimerbyHandle (Variables|Default|GetTimerHandle))
  (Utilities|FlowControl|Sequence
    (:then_0
      (Utilities|FlowControl|Gate true) ; enters at Close
    )
    (:then_1
      (Utilities|FlowControl|DoOnce false) ; enters at Reset
    )))

(event EventEventFiring
  (params (Quest :type BP%20Quest%20Actor%20Object%20Reference) (Bee :type Bee%20Character%20BP%20Object%20Reference))
  (bind _returnvalue (Utilities|Time|SetTimerbyEvent (delegate Custom|Check) 0.1 true)))

(fn ConstructionScript
  (|CallParentFunction))