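; Player controller for the bee character that relays movement, camera, zoom, roll, boost, respawn and interact input to the pawn via interface messages.
; Wine pickup scrambles the movement axes and inverts strafe, while holding Gravity blocks movement, interact and auto-move.
; Sting uses press timers to choose between a normal sting and a charged super sting, cancelled on early release.
; A FlipFlop toggles the pause menu, slowing time on open.
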(event Custom|IsSupSting
  (Variables|Default|SetIsSuperSting true)
  (Class|IControls|SuperSting(Message) (Pawn|GetControlledPawn)))

(event Custom|InCharge?
  (Variables|Default|SetIsChargeComplete true))

(event EventBeginPlay
  (Input|EnableInput (Game|GetPlayerController 0)))

(event EventWinePickup
  (params (PickedUp :type Boolean))
  ;[0 1 0.4249] Action Inputs
  (Variables|Default|SetIsWineActive PickedUp))

(event EventPauseGame
  (bind _returnvalue (Game|GetPlayerController 0))
  (bind _returnvalue_2 (Game|GetPlayerController 0))
  (Utilities|FlowControl|FlipFlop
    (:A
      (bind _returnvalue_3 (UserInterface|CreateWidget "/Game/Widgets/Menu/W_PauseMenu.W_PauseMenu_C" 0 true))
      (bind _output_get (Variables|Default|SetPauseMenu _returnvalue_3))
      (UserInterface|Viewport|AddtoViewport _returnvalue_3 0)
      (Input|SetInputModeGameandUI _returnvalue_2 _output_get "DoNotLock" true)
      (Variables|/Script/Engine.PlayerController|SetbShowMouseCursor _returnvalue_2 true)
      (Class|IGameMode|PauseGame(Message) (Game|GetGameMode))
      (Utilities|Time|SetGlobalTimeDilation 0.1))
    (:B
      (Class|IGameMode|ResumeGame(Message) (Game|GetGameMode))
      (Input|EnableInput _returnvalue _returnvalue)
      (Input|SetInputModeGameOnly _returnvalue)
      (Variables|/Script/Engine.PlayerController|SetbShowMouseCursor _returnvalue false)
      (Widget|RemovefromParent (Variables|Default|GetPauseMenu)))))

(event Input|ActionEvents|InputActionSting
  (params (Key :type Key%20Structure)))

(event Input|ActionEvents|InputActionInteract
  (params (Key :type Key%20Structure))
  ;[0 1 0.4249] Action Inputs
  (:Pressed
    (if (not (Variables|Default|GetIsGravity))
      (Class|IControls|Interact(Message) (Pawn|GetControlledPawn)))))

(event Input|ActionEvents|InputActionRollLeft
  (params (Key :type Key%20Structure))
  ;[0 1 0.4249] Action Inputs
  (:Pressed
    (Class|IControls|RollLeft(Message) (Pawn|GetControlledPawn))))

(event Input|ActionEvents|InputActionRollRight
  (params (Key :type Key%20Structure))
  ;[0 1 0.4249] Action Inputs
  (:Pressed
    (Class|IControls|RollRight(Message) (Pawn|GetControlledPawn))))

(event Input|ActionEvents|InputActionRespawn
  (params (Key :type Key%20Structure))
  ;[0 1 0.4249] Action Inputs
  (:Pressed
    (Class|IControls|Respawn(Message) (Pawn|GetControlledPawn))))

(event Input|ActionEvents|InputActionSting
  (params (Key :type Key%20Structure))
  (bind _returnvalue (Pawn|GetControlledPawn))
  (:Pressed
    (Variables|Default|SetIsSuperSting false)
    (Variables|Default|SetIsChargeComplete false)
    (bind _returnvalue_2 (Utilities|Time|SetTimerbyEvent (delegate Custom|IsSupSting) (Variables|Default|GetSuperStingTime)))
    (bind _returnvalue_3 (Utilities|Time|SetTimerbyEvent (delegate Custom|InCharge?) 3.0)))
  (:Released
    (Utilities|Time|ClearandInvalidateTimerbyHandle _returnvalue_2)
    (Utilities|Time|ClearandInvalidateTimerbyHandle _returnvalue_3)
    (if (Variables|Default|GetIsSuperSting)
      (if (Variables|Default|GetIsChargeComplete)
        (Variables|Default|SetIsSuperSting false)
        (Variables|Default|SetIsChargeComplete false)
        (else
          (Variables|Default|SetIsSuperSting false)
          (Variables|Default|SetIsChargeComplete false)
          (Class|IControls|StopCharge(Message) _returnvalue)))
      (else
        (Variables|Default|SetIsSuperSting false)
        (Variables|Default|SetIsChargeComplete false)
        (Class|IControls|Sting(Message) _returnvalue)))))

(event Input|ActionEvents|InputActionZoomIn
  (params (Key :type Key%20Structure))
  ;[0 1 0.4249] Action Inputs
  (:Pressed
    (Class|IControls|Zoomin(Message) (Pawn|GetControlledPawn))))

(event Input|ActionEvents|InputActionZoomOut
  (params (Key :type Key%20Structure))
  ;[0 1 0.4249] Action Inputs
  (:Pressed
    (Class|IControls|ZoomOut(Message) (Pawn|GetControlledPawn))))

(event Input|ActionEvents|InputActionrightClick
  (params (Key :type Key%20Structure))
  ;[0.521 0.2623 1] Tim-minimapstuff
)

(event Input|ActionEvents|InputActionPauseMenu
  (params (Key :type Key%20Structure))
  (bind _returnvalue (Game|GetPlayerController 0))
  (bind _returnvalue_2 (Game|GetPlayerController 0))
  (:Pressed
    (Utilities|FlowControl|FlipFlop
      (:A
        (bind _returnvalue_3 (UserInterface|CreateWidget "/Game/Widgets/Menu/W_PauseMenu.W_PauseMenu_C" 0 true))
        (bind _output_get (Variables|Default|SetPauseMenu _returnvalue_3))
        (UserInterface|Viewport|AddtoViewport _returnvalue_3 0)
        (Input|SetInputModeGameandUI _returnvalue_2 _output_get "DoNotLock" true)
        (Variables|/Script/Engine.PlayerController|SetbShowMouseCursor _returnvalue_2 true)
        (Class|IGameMode|PauseGame(Message) (Game|GetGameMode))
        (Utilities|Time|SetGlobalTimeDilation 0.1))
      (:B
        (Class|IGameMode|ResumeGame(Message) (Game|GetGameMode))
        (Input|EnableInput _returnvalue _returnvalue)
        (Input|SetInputModeGameOnly _returnvalue)
        (Variables|/Script/Engine.PlayerController|SetbShowMouseCursor _returnvalue false)
        (Widget|RemovefromParent (Variables|Default|GetPauseMenu))))))

(event Input|ActionEvents|InputActionGravity
  (params (Key :type Key%20Structure))
  ;[0 1 0.4249] Action Inputs
  (:Pressed
    (bind _asbee_character_bp (Utilities|Casting|CastToBeeCharacter_BP (Pawn|GetControlledPawn)))
    (if (not (Variables|/Game/Blueprints/Character/BeeCharacter_BP.BeeCharacter_BP_C|GetIsAutoMove _asbee_character_bp))
      (Variables|Default|SetIsGravity true)
      (Class|IControls|ToggleGravity(Message) (Pawn|GetControlledPawn) (stale _output_get) :!label _label)))
  (:Released
    (if (not (Variables|/Game/Blueprints/Character/BeeCharacter_BP.BeeCharacter_BP_C|GetIsAutoMove _asbee_character_bp))
      (bind _output_get (Variables|Default|SetIsGravity false))
      (goto _label))))

(event Input|ActionEvents|InputActionZoomReset
  (params (Key :type Key%20Structure))
  ;[0 1 0.4249] Action Inputs
  (:Pressed
    (Class|IControls|ZoomReset(Message) (Pawn|GetControlledPawn))))

(event Input|ActionEvents|InputActionSprintAction
  (params (Key :type Key%20Structure))
  ;[0 1 0.4249] Action Inputs
  (:Pressed
    (Class|IControls|Boost(Message) (Pawn|GetControlledPawn) (CallFunction|CheckInputValue 0.0))))

(event Input|ActionEvents|InputActionAutoMove
  (params (Key :type Key%20Structure))
  ;[0 1 0.4249] Action Inputs
  (:Pressed
    (if (not (Variables|Default|GetIsGravity))
      (Class|IControls|AutoMove(Message) (Pawn|GetControlledPawn)))))

(event Input|AxisEvents|InputAxisTurn
  (params (AxisValue :type Float%20%28single-precision%29))
  ;[0 1 0.4249] Axis Inputs
  (Class|IControls|Turn(Message) (Pawn|GetControlledPawn) AxisValue))

(event Input|AxisEvents|InputAxisLookUp
  (params (AxisValue :type Float%20%28single-precision%29))
  ;[0 1 0.4249] Axis Inputs
  (Class|IControls|LookUp(Message) (Pawn|GetControlledPawn) AxisValue))

(event Input|AxisEvents|InputAxisMoveForward
  (params (AxisValue :type Float%20%28single-precision%29))
  (bind _returnvalue (Pawn|GetControlledPawn))
  ;[0 1 0.4249] Axis Inputs
  (if (and (CallFunction|CheckInputValue AxisValue) (not (Variables|Default|GetIsGravity)))
    (if (Variables|Default|GetIsWineActive)
      (Class|IControls|MoveRight(Message) _returnvalue AxisValue)
      (else
        (Class|IControls|MoveForward(Message) _returnvalue AxisValue)))))

(event Input|AxisEvents|InputAxisMoveRight
  (params (AxisValue :type Float%20%28single-precision%29))
  (bind _returnvalue (Pawn|GetControlledPawn))
  ;[0 1 0.4249] Axis Inputs
  (if (and (CallFunction|CheckInputValue AxisValue) (not (Variables|Default|GetIsGravity)))
    (if (Variables|Default|GetIsWineActive)
      (Class|IControls|MoveUp(Message) _returnvalue AxisValue)
      (else
        (Class|IControls|MoveRight(Message) _returnvalue AxisValue)))))

(event Input|AxisEvents|InputAxisMoveUp
  (params (AxisValue :type Float%20%28single-precision%29))
  (bind _returnvalue (Pawn|GetControlledPawn))
  ;[0 1 0.4249] Axis Inputs
  (if (and (CallFunction|CheckInputValue AxisValue) (not (Variables|Default|GetIsGravity)))
    (if (Variables|Default|GetIsWineActive)
      (Class|IControls|MoveForward(Message) _returnvalue AxisValue)
      (else
        (Class|IControls|MoveUp(Message) _returnvalue AxisValue)))))

(event Input|AxisEvents|InputAxisStrafeRight
  (params (AxisValue :type Float%20%28single-precision%29))
  ;[0 1 0.4249] Axis Inputs
  (if (and (CallFunction|CheckInputValue AxisValue) (not (Variables|Default|GetIsGravity)))
    (Class|IControls|StrafeRight(Message) (Pawn|GetControlledPawn) (Math|Float|SelectFloat (* AxisValue -1.0) AxisValue (Variables|Default|GetIsWineActive)))))

(event Input|AxisEvents|InputAxisSprint
  (params (AxisValue :type Float%20%28single-precision%29))
  ;[0 1 0.4249] Action Inputs
)

(event Input|AxisEvents|InputAxisSprint
  (params (AxisValue :type Float%20%28single-precision%29))
  ;[0.521 0.2623 1] Tim-minimapstuff
  (Variables|Default|SetsprintAxis AxisValue))

(event Input|KeyboardEvents|LeftAlt
  (params (Key :type Key%20Structure))
  (bind _returnvalue (Pawn|GetControlledPawn))
  ;[0 1 0.4249] Action Inputs
  (:Pressed
    (bind _asbee_character_bp (Utilities|Casting|CastToBeeCharacter_BP _returnvalue))
    (Variables|/Game/Blueprints/Character/BeeCharacter_BP.BeeCharacter_BP_C|SetAltCamera _asbee_character_bp true))
  (:Released
    (bind _asbee_character_bp_2 (Utilities|Casting|CastToBeeCharacter_BP _returnvalue))
    (Variables|/Game/Blueprints/Character/BeeCharacter_BP.BeeCharacter_BP_C|SetAltCamera _asbee_character_bp_2 false)))

(event Input|KeyboardEvents|P
  (params (Key :type Key%20Structure))
  (bind _returnvalue (Game|GetPlayerController 0))
  (bind _returnvalue_2 (Game|GetPlayerController 0))
  (:Pressed
    (Utilities|FlowControl|FlipFlop
      (:A
        (bind _returnvalue_3 (UserInterface|CreateWidget "/Game/Widgets/Menu/W_PauseMenu.W_PauseMenu_C" 0 true))
        (bind _output_get (Variables|Default|SetPauseMenu _returnvalue_3))
        (UserInterface|Viewport|AddtoViewport _returnvalue_3 0)
        (Input|SetInputModeGameandUI _returnvalue_2 _output_get "DoNotLock" true)
        (Variables|/Script/Engine.PlayerController|SetbShowMouseCursor _returnvalue_2 true)
        (Class|IGameMode|PauseGame(Message) (Game|GetGameMode))
        (Utilities|Time|SetGlobalTimeDilation 0.1))
      (:B
        (Class|IGameMode|ResumeGame(Message) (Game|GetGameMode))
        (Input|EnableInput _returnvalue _returnvalue)
        (Input|SetInputModeGameOnly _returnvalue)
        (Variables|/Script/Engine.PlayerController|SetbShowMouseCursor _returnvalue false)
        (Widget|RemovefromParent (Variables|Default|GetPauseMenu))))))

(fn ConstructionScript)

(fn CheckInputValue
  (params (AxisValue :type Float%20%28single-precision%29))
  (return (not (Math|Float|InRange(Float) AxisValue -0.1 0.1))))

(fn GetBeePlayer
  (params (InActor :type Actor%20Object%20Reference))
  (return false 0 0))

(fn GetPlayerCon
  (return self))