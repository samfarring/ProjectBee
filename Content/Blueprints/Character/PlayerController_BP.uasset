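; Player controller for the bee character that relays movement, look, strafe, interact and sting input to the controlled pawn.
; Input events forward as messages to the pawn, so those actions need no cast to a specific class.
; Left Alt is the exception, casting to BeeCharacter_BP to set AltCamera while held.
; GetPlayerCon returns this controller, and GetBeePlayer returns IsBee as false.
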(event Input|ActionEvents|InputActionSting
  (params (Key :type Key%20Structure))
  (:Pressed
    (Class|IMovement|Sting(Message) (Pawn|GetControlledPawn))))

(event Input|ActionEvents|InputActionLeft
  (params (Key :type Key%20Structure))
  ;[0 1 0.143] Bee Movement
  (:Pressed
    (Class|IMovement|StrafeLeft(Message) (Pawn|GetControlledPawn))))

(event Input|ActionEvents|InputActionRight
  (params (Key :type Key%20Structure))
  ;[0 1 0.143] Bee Movement
  (:Pressed
    (Class|IMovement|StrafeRight(Message) (Pawn|GetControlledPawn))))

(event Input|ActionEvents|InputActionInteract
  (params (Key :type Key%20Structure))
  (:Pressed
    (Class|IMovement|Interact(Message) (Pawn|GetControlledPawn))))

(event Input|AxisEvents|InputAxisTurn
  (params (AxisValue :type Float%20%28single-precision%29))
  ;[0 1 0.143] Bee Movement
  (Class|IMovement|Turn(Message) (Pawn|GetControlledPawn) AxisValue))

(event Input|AxisEvents|InputAxisLookUp
  (params (AxisValue :type Float%20%28single-precision%29))
  ;[0 1 0.143] Bee Movement
  (Class|IMovement|LookUp(Message) (Pawn|GetControlledPawn) AxisValue))

(event Input|AxisEvents|InputAxisMoveForward
  (params (AxisValue :type Float%20%28single-precision%29))
  ;[0 1 0.143] Bee Movement
  (Class|IMovement|MoveForward(Message) (Pawn|GetControlledPawn) AxisValue))

(event Input|AxisEvents|InputAxisMoveRight
  (params (AxisValue :type Float%20%28single-precision%29))
  ;[0 1 0.143] Bee Movement
  (Class|IMovement|MoveRight(Message) (Pawn|GetControlledPawn) AxisValue))

(event Input|KeyboardEvents|LeftAlt
  (params (Key :type Key%20Structure))
  (bind _returnvalue (Pawn|GetControlledPawn))
  (:Pressed
    (bind _asbee_character_bp (Utilities|Casting|CastToBeeCharacter_BP _returnvalue))
    (Variables|/Game/Blueprints/Character/BeeCharacter_BP.BeeCharacter_BP_C|SetAltCamera _asbee_character_bp true))
  (:Released
    (bind _asbee_character_bp_2 (Utilities|Casting|CastToBeeCharacter_BP _returnvalue))
    (Variables|/Game/Blueprints/Character/BeeCharacter_BP.BeeCharacter_BP_C|SetAltCamera _asbee_character_bp_2 false)))

(fn ConstructionScript)

(fn GetBeePlayer
  (params (InActor :type Actor%20Object%20Reference))
  (return false 0 0))

(fn GetPlayerCon
  (return self))