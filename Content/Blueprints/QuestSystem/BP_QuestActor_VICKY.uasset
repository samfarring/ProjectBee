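; Quest actor that starts when the bee player enters its QuestZone and runs a list of Location, Sting, Chase and Fetch objectives in order.
; Each objective spawns a runtime goal sphere as trigger or NPC search area; Sting and Chase message a random or specified NPC.
; Dispatchers broadcast progress, and interface messages update the player's quest display.
; Sting advances immediately after messaging; older AITarget logic remains unwired.
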(event OnComponentBeginOverlap(QuestZone)
  (params (OverlappedComponent :type Primitive%20Component%20Object%20Reference) (OtherActor :type Actor%20Object%20Reference) (OtherComp :type Primitive%20Component%20Object%20Reference) (OtherBodyIndex :type Integer) (bFromSweep :type Boolean) (SweepResult :type Hit%20Result%20Structure%20%28by%20ref%29))
  (bind _objectives (Variables|Objectives|GetObjectives))
  (bind _objectivecounter (Variables|Objectives|GetObjectiveCounter))
  (bind _objectives_2 (Variables|Objectives|GetObjectives))
  (bind _objectivecounter_2 (Variables|Objectives|GetObjectiveCounter))
  (bind _objectives_3 (Variables|Objectives|GetObjectives))
  (bind _objectivecounter_3 (Variables|Objectives|GetObjectiveCounter))
  (bind _objectives_4 (Variables|Objectives|GetObjectives))
  (bind _objectivecounter_4 (Variables|Objectives|GetObjectiveCounter))
  (bind _output (Utilities|Array|Get(acopy) _objectives_2 _objectivecounter_2))
  (bind _output_2 (Utilities|Array|Get(acopy) _objectives_3 _objectivecounter_3))
  (bind _output_3 (Utilities|Array|Get(acopy) _objectives_4 _objectivecounter_4))
  (bind _output_4 (Utilities|Array|Get(acopy) _objectives _objectivecounter))
  (bind _questdetails (Utilities|Struct|BreakQuestStructVICKY _output_2))
  (bind (_objectivetext _type _iscomplete) (Utilities|Struct|BreakQuestStructVICKY _output))
  (bind _questdetails_2 (Utilities|Struct|BreakQuestStructVICKY _output_3))
  (bind _questdetails_3 (Utilities|Struct|BreakQuestStructVICKY _output_4))
  (bind (_targetnpctosting _randomnpc _fetchitem _goallocation _questgoalsize) (Utilities|Struct|BreakQuestDetails _questdetails))
  (bind (_targetnpctosting_2 _randomnpc_2 _fetchitem_2 _goallocation_2 _questgoalsize_2) (Utilities|Struct|BreakQuestDetails _questdetails_2))
  (bind (_targetnpctosting_3 _randomnpc_3 _fetchitem_3 _goallocation_3 _questgoalsize_3) (Utilities|Struct|BreakQuestDetails _questdetails_3))
  (bind _asbee_character_bp (Utilities|Casting|CastToBeeCharacter_BP OtherActor))
  (Variables|Objectives|SetOverlapRef _asbee_character_bp)
  (bind _isbee (Class|ICharacter|GetBeePlayer(Message) _asbee_character_bp _asbee_character_bp))
  (Utilities|FlowControl|DoOnce false
    (:Completed
      (if _isbee
        (Variables|Objectives|SetObjectiveLength (Utilities|Array|Length (Variables|Objectives|GetObjectives)))
        (CallFunction|StatusChange "NewEnumerator3")
        (if (not _iscomplete)
          (Utilities|FlowControl|DoOnce false
            (:Completed
              (switch Utilities|FlowControl|Switch|SwitchonObjectiveTypes _type
                (:NewEnumerator2
                  ;[1 1 1] Go To Location
                  (bind _returnvalue (AddComponent|AddSphereComponent false (Math|Conversions|ToTransform(Vector) _goallocation_2)))
                  (Collision|AssignOnComponentBeginOverlap _returnvalue (delegate Custom|OnComponentBeginOverlap_Event_1))
                  (CallFunction|SetGoalSphere _returnvalue _questgoalsize_2)
                  (CallFunction|StartObjective)
                  (CallFunction|UINewQuest))
                (:NewEnumerator4
                  ;[1 1 1] Sting
                  (CallFunction|StartObjective)
                  (CallFunction|UINewQuest)
                  (if _randomnpc_3
                    (bind _returnvalue_2 (AddComponent|AddSphereComponent false (Math|Conversions|ToTransform(Vector) _goallocation_3)))
                    (CallFunction|SetGoalSphere _returnvalue_2 _questgoalsize_3)
                    (bind _output_get (Variables|Default|SetNPCTargets (Collision|GetOverlappingActors _returnvalue_2 "/Script/Engine.Character" :!class /Script/Engine.PrimitiveComponent)))
                    (Utilities|Array|RemoveItem _output_get (Game|Player|GetPlayerPawn 0))
                    ;[1 1 1] This and the other Sting message may need to be changed to be like the chase function, however that may mean we need to copy and paste that function into each thing that can be stung, unless we can just do it all into the actual Interface BP
                    (Class|IStingable|StingNPC(Message) (Utilities|Array|Get(acopy) (Variables|Default|GetNPCTargets) (Math|Random|RandomInteger (- (Utilities|Array|Length (Variables|Default|GetNPCTargets)) 1))))
                    (Components|DestroyComponent _returnvalue_2)
                    (else
                      (Class|IStingable|StingNPC(Message) _targetnpctosting_3)))
                  (bind _result (Math|Integer|IncrementInt (Variables|Objectives|GetObjectiveCounter))
                    (:%20%20
                      (if (== _result (Variables|Objectives|GetObjectiveLength))
                        (CallFunction|CompleteQuest)
                        (else
                          (CallFunction|NewObjective))))))
                (:NewEnumerator5
                  (bind _returnvalue_3 (AddComponent|AddSphereComponent false (Math|Conversions|ToTransform(Vector) _goallocation)))
                  (CallFunction|SetGoalSphere _returnvalue_3 _questgoalsize)
                  (CallFunction|StartObjective)
                  (CallFunction|UINewQuest)
                  (if _randomnpc
                    (bind _output_get_2 (Variables|Default|SetNPCTargets (Collision|GetOverlappingActors _returnvalue_3 "/Script/Engine.Character" :!class /Script/Engine.PrimitiveComponent)))
                    (Utilities|Array|RemoveItem _output_get_2 (Game|Player|GetPlayerPawn 0))
                    (Variables|Default|SetNPCTarget (Utilities|Array|Get(acopy) (Variables|Default|GetNPCTargets) (Math|Random|RandomInteger (- (Utilities|Array|Length (Variables|Default|GetNPCTargets)) 1))))
                    (bind _out_of_zone_ (Class|IStingable|ChaseNPCFunction(Message) (Utilities|Array|Get(acopy) (Variables|Default|GetNPCTargets) (Math|Random|RandomInteger (- (Utilities|Array|Length (Variables|Default|GetNPCTargets)) 1))) _returnvalue_3))
                    (if _out_of_zone_
                      (Components|DestroyComponent _returnvalue_3 :!label _label)
                      (bind _result_2 (Math|Integer|IncrementInt (Variables|Objectives|GetObjectiveCounter))
                        (:%20%20
                          (if (== _result_2 (Variables|Objectives|GetObjectiveLength))
                            (CallFunction|CompleteQuest)
                            (else
                              (CallFunction|NewObjective))))))
                    (else
                      (Variables|Default|SetNPCTarget _targetnpctosting)
                      (bind _out_of_zone__2 (Class|IStingable|ChaseNPCFunction(Message) _targetnpctosting _returnvalue_3))
                      (if _out_of_zone__2
                        (goto _label)))))
                (:NewEnumerator6
                  (bind _returnvalue_4 (AddComponent|AddSphereComponent false (Math|Conversions|ToTransform(Vector) (.GoalLocation (Utilities|Struct|BreakQuestDetails (.QuestDetails (Utilities|Struct|BreakQuestStructVICKY (Utilities|Array|Get(acopy) (Variables|Objectives|GetObjectives) (Variables|Objectives|GetObjectiveCounter)))))))))
                  (Collision|BindEventtoOnComponentBeginOverlap _returnvalue_4 (delegate Custom|BeginOver))
                  (CallFunction|SetGoalSphere _returnvalue_4 (Utilities|Struct|BreakQuestDetails (Utilities|Struct|BreakQuestStructVICKY (Utilities|Array|Get(acopy) (Variables|Objectives|GetObjectives) (Variables|Objectives|GetObjectiveCounter)))))
                  (CallFunction|StartObjective)
                  (CallFunction|UINewQuest))))))))))

(event OnComponentEndOverlap(QuestZone)
  (params (OverlappedComponent :type Primitive%20Component%20Object%20Reference) (OtherActor :type Actor%20Object%20Reference) (OtherComp :type Primitive%20Component%20Object%20Reference) (OtherBodyIndex :type Integer))
  (bind _objectives (Variables|Objectives|GetObjectives))
  (bind _objectivecounter (Variables|Objectives|GetObjectiveCounter))
  (bind _objectives_2 (Variables|Objectives|GetObjectives))
  (bind _objectivecounter_2 (Variables|Objectives|GetObjectiveCounter))
  (bind _objectives_3 (Variables|Objectives|GetObjectives))
  (bind _objectivecounter_3 (Variables|Objectives|GetObjectiveCounter))
  (bind _objectives_4 (Variables|Objectives|GetObjectives))
  (bind _objectivecounter_4 (Variables|Objectives|GetObjectiveCounter))
  (bind _output (Utilities|Array|Get(acopy) _objectives_2 _objectivecounter_2))
  (bind _output_2 (Utilities|Array|Get(acopy) _objectives_3 _objectivecounter_3))
  (bind _output_3 (Utilities|Array|Get(acopy) _objectives_4 _objectivecounter_4))
  (bind _output_4 (Utilities|Array|Get(acopy) _objectives _objectivecounter))
  (bind _questdetails (Utilities|Struct|BreakQuestStructVICKY _output_2))
  (bind (_objectivetext _type _iscomplete) (Utilities|Struct|BreakQuestStructVICKY _output))
  (bind _questdetails_2 (Utilities|Struct|BreakQuestStructVICKY _output_3))
  (bind _questdetails_3 (Utilities|Struct|BreakQuestStructVICKY _output_4))
  (bind (_targetnpctosting _randomnpc _fetchitem _goallocation _questgoalsize) (Utilities|Struct|BreakQuestDetails _questdetails))
  (bind (_targetnpctosting_2 _randomnpc_2 _fetchitem_2 _goallocation_2 _questgoalsize_2) (Utilities|Struct|BreakQuestDetails _questdetails_2))
  (bind (_targetnpctosting_3 _randomnpc_3 _fetchitem_3 _goallocation_3 _questgoalsize_3) (Utilities|Struct|BreakQuestDetails _questdetails_3))
  (Utilities|FlowControl|DoOnce false) ; enters at Reset
)

(event Custom|StungTarget
  ;[1 1 1] Old
  (bind _result (Math|Integer|IncrementInt (Variables|Objectives|GetObjectiveCounter))
    (:%20%20
      (if (== _result (Variables|Objectives|GetObjectiveLength))
        (CallFunction|CompleteQuest)
        (else
          (CallFunction|NewObjective))))))

(event Custom|NextObjective
  (bind _objectives (Variables|Objectives|GetObjectives))
  (bind _objectivecounter (Variables|Objectives|GetObjectiveCounter))
  (bind _objectives_2 (Variables|Objectives|GetObjectives))
  (bind _objectivecounter_2 (Variables|Objectives|GetObjectiveCounter))
  (bind _objectives_3 (Variables|Objectives|GetObjectives))
  (bind _objectivecounter_3 (Variables|Objectives|GetObjectiveCounter))
  (bind _output (Utilities|Array|Get(acopy) _objectives_2 _objectivecounter_2))
  (bind _output_2 (Utilities|Array|Get(acopy) _objectives_3 _objectivecounter_3))
  (bind _output_3 (Utilities|Array|Get(acopy) _objectives _objectivecounter))
  (bind _questdetails (Utilities|Struct|BreakQuestStructVICKY _output))
  (bind _questdetails_2 (Utilities|Struct|BreakQuestStructVICKY _output_2))
  (bind _questdetails_3 (Utilities|Struct|BreakQuestStructVICKY _output_3))
  (bind (_targetnpctosting _randomnpc _fetchitem _goallocation _questgoalsize) (Utilities|Struct|BreakQuestDetails _questdetails))
  (bind (_targetnpctosting_2 _randomnpc_2 _fetchitem_2 _goallocation_2 _questgoalsize_2) (Utilities|Struct|BreakQuestDetails _questdetails_2))
  (bind (_targetnpctosting_3 _randomnpc_3 _fetchitem_3 _goallocation_3 _questgoalsize_3) (Utilities|Struct|BreakQuestDetails _questdetails_3))
  (Utilities|FlowControl|Sequence
    (:then_0
      (goto _label Reset))
    (:then_1
      (Utilities|FlowControl|DoOnce false :!label _label
        (:Completed
          (switch Utilities|FlowControl|Switch|SwitchonObjectiveTypes (.Type (Utilities|Struct|BreakQuestStructVICKY (Utilities|Array|Get(acopy) (Variables|Objectives|GetObjectives) (Variables|Objectives|GetObjectiveCounter))))
            (:NewEnumerator2
              ;[1 1 1] Go To Location
              (bind _returnvalue (AddComponent|AddSphereComponent false (Math|Conversions|ToTransform(Vector) _goallocation_2)))
              (Collision|AssignOnComponentBeginOverlap _returnvalue (delegate Custom|OnComponentBeginOverlap_Event_1))
              (CallFunction|SetGoalSphere _returnvalue _questgoalsize_2)
              (CallFunction|StartObjective)
              (CallFunction|UINewQuest))
            (:NewEnumerator4
              ;[1 1 1] Sting
              (CallFunction|StartObjective)
              (CallFunction|UINewQuest)
              (if _randomnpc_3
                (bind _returnvalue_2 (AddComponent|AddSphereComponent false (Math|Conversions|ToTransform(Vector) _goallocation_3)))
                (CallFunction|SetGoalSphere _returnvalue_2 _questgoalsize_3)
                (bind _output_get (Variables|Default|SetNPCTargets (Collision|GetOverlappingActors _returnvalue_2 "/Script/Engine.Character" :!class /Script/Engine.PrimitiveComponent)))
                (Utilities|Array|RemoveItem _output_get (Game|Player|GetPlayerPawn 0))
                ;[1 1 1] This and the other Sting message may need to be changed to be like the chase function, however that may mean we need to copy and paste that function into each thing that can be stung, unless we can just do it all into the actual Interface BP
                (Class|IStingable|StingNPC(Message) (Utilities|Array|Get(acopy) (Variables|Default|GetNPCTargets) (Math|Random|RandomInteger (- (Utilities|Array|Length (Variables|Default|GetNPCTargets)) 1))))
                (Components|DestroyComponent _returnvalue_2)
                (else
                  (Class|IStingable|StingNPC(Message) _targetnpctosting_3)))
              (bind _result (Math|Integer|IncrementInt (Variables|Objectives|GetObjectiveCounter))
                (:%20%20
                  (if (== _result (Variables|Objectives|GetObjectiveLength))
                    (CallFunction|CompleteQuest)
                    (else
                      (CallFunction|NewObjective))))))
            (:NewEnumerator5
              (bind _returnvalue_3 (AddComponent|AddSphereComponent false (Math|Conversions|ToTransform(Vector) _goallocation)))
              (CallFunction|SetGoalSphere _returnvalue_3 _questgoalsize)
              (CallFunction|StartObjective)
              (CallFunction|UINewQuest)
              (if _randomnpc
                (bind _output_get_2 (Variables|Default|SetNPCTargets (Collision|GetOverlappingActors _returnvalue_3 "/Script/Engine.Character" :!class /Script/Engine.PrimitiveComponent)))
                (Utilities|Array|RemoveItem _output_get_2 (Game|Player|GetPlayerPawn 0))
                (Variables|Default|SetNPCTarget (Utilities|Array|Get(acopy) (Variables|Default|GetNPCTargets) (Math|Random|RandomInteger (- (Utilities|Array|Length (Variables|Default|GetNPCTargets)) 1))))
                (bind _out_of_zone_ (Class|IStingable|ChaseNPCFunction(Message) (Utilities|Array|Get(acopy) (Variables|Default|GetNPCTargets) (Math|Random|RandomInteger (- (Utilities|Array|Length (Variables|Default|GetNPCTargets)) 1))) _returnvalue_3))
                (if _out_of_zone_
                  (Components|DestroyComponent _returnvalue_3 :!label _label_2)
                  (bind _result_2 (Math|Integer|IncrementInt (Variables|Objectives|GetObjectiveCounter))
                    (:%20%20
                      (if (== _result_2 (Variables|Objectives|GetObjectiveLength))
                        (CallFunction|CompleteQuest)
                        (else
                          (CallFunction|NewObjective))))))
                (else
                  (Variables|Default|SetNPCTarget _targetnpctosting)
                  (bind _out_of_zone__2 (Class|IStingable|ChaseNPCFunction(Message) _targetnpctosting _returnvalue_3))
                  (if _out_of_zone__2
                    (goto _label_2)))))
            (:NewEnumerator6
              (bind _returnvalue_4 (AddComponent|AddSphereComponent false (Math|Conversions|ToTransform(Vector) (.GoalLocation (Utilities|Struct|BreakQuestDetails (.QuestDetails (Utilities|Struct|BreakQuestStructVICKY (Utilities|Array|Get(acopy) (Variables|Objectives|GetObjectives) (Variables|Objectives|GetObjectiveCounter)))))))))
              (Collision|BindEventtoOnComponentBeginOverlap _returnvalue_4 (delegate Custom|BeginOver))
              (CallFunction|SetGoalSphere _returnvalue_4 (Utilities|Struct|BreakQuestDetails (Utilities|Struct|BreakQuestStructVICKY (Utilities|Array|Get(acopy) (Variables|Objectives|GetObjectives) (Variables|Objectives|GetObjectiveCounter)))))
              (CallFunction|StartObjective)
              (CallFunction|UINewQuest))))))))

(event Custom|BeginOver
  (params (OverlappedComponent :type Primitive%20Component%20Object%20Reference) (OtherActor :type Actor%20Object%20Reference) (OtherComp :type Primitive%20Component%20Object%20Reference) (OtherBodyIndex :type Integer) (bFromSweep :type Boolean) (SweepResult :type Hit%20Result%20Structure%20%28by%20ref%29))
  (for _array_element (Collision|GetOverlappingActors OverlappedComponent "/Game/Blueprints/Grabbables/BP_Grabbable.BP_Grabbable_C" :!class /Script/Engine.PrimitiveComponent)
    (if (== (.FetchItem (Utilities|Struct|BreakQuestDetails (.QuestDetails (Utilities|Struct|BreakQuestStructVICKY (Utilities|Array|Get(acopy) (Variables|Objectives|GetObjectives) (Variables|Objectives|GetObjectiveCounter)))))) _array_element)
      (EventDispatchers|UnbindallEventsfromOnComponentBeginOverlap (stale OnComponentBeginOverlap(QuestZone) _returnvalue_4))
      (Components|DestroyComponent (stale OnComponentBeginOverlap(QuestZone) _returnvalue_4))
      (bind _result (Math|Integer|IncrementInt (Variables|Objectives|GetObjectiveCounter))
        (:%20%20
          (if (== _result (Variables|Objectives|GetObjectiveLength))
            (CallFunction|CompleteQuest)
            (else
              (CallFunction|NewObjective))))))))

(event Custom|Overlap
  (params (OverlappedComponent :type Primitive%20Component%20Object%20Reference) (OtherActor :type Actor%20Object%20Reference) (OtherComp :type Primitive%20Component%20Object%20Reference) (OtherBodyIndex :type Integer) (bFromSweep :type Boolean) (SweepResult :type Hit%20Result%20Structure%20%28by%20ref%29))
  ;[1 1 1] Old
  ;;[1 1 1] Chase
  (if (== OtherActor (Variables|AI|GetAITarget))
    (bind _result (Math|Integer|IncrementInt (Variables|Objectives|GetObjectiveCounter))
      (:%20%20
        (if (== _result (Variables|Objectives|GetObjectiveLength))
          (CallFunction|CompleteQuest)
          (else
            (CallFunction|NewObjective)))))))

(event Custom|OnComponentBeginOverlap_Event_1
  (params (OverlappedComponent :type Primitive%20Component%20Object%20Reference) (OtherActor :type Actor%20Object%20Reference) (OtherComp :type Primitive%20Component%20Object%20Reference) (OtherBodyIndex :type Integer) (bFromSweep :type Boolean) (SweepResult :type Hit%20Result%20Structure%20%28by%20ref%29))
  ;[1 1 1] Go To Location
  (bind _isbee (Class|ICharacter|GetBeePlayer(Message) OtherActor OtherActor))
  (if _isbee
    (EventDispatchers|UnbindallEventsfromOnComponentBeginOverlap (stale OnComponentBeginOverlap(QuestZone) _returnvalue))
    (Components|DestroyComponent (stale OnComponentBeginOverlap(QuestZone) _returnvalue))
    (bind _result (Math|Integer|IncrementInt (Variables|Objectives|GetObjectiveCounter))
      (:%20%20
        (if (== _result (Variables|Objectives|GetObjectiveLength))
          (CallFunction|CompleteQuest)
          (else
            (CallFunction|NewObjective)))))))

(event EventBeginPlay
  (CallFunction|StatusChange "NewEnumerator1"))

(fn ConstructionScript
  (Components|Sphere|SetSphereRadius (Variables|Default|GetQuestZone) (Variables|QuestDetails|GetQuestActivationRadius) true))

(fn StatusChange
  (params (NewStatus :type QuestStatus%20Enum :default "NewEnumerator0"))
  (Collision|SetCollisionEnabled (Variables|Default|GetQuestZone) (Utilities|Select :Index NewStatus :NewEnumerator0 "NoCollision" :NewEnumerator1 "QueryOnly" :NewEnumerator2 "NoCollision" :NewEnumerator3 "NoCollision" :NewEnumerator4 "NoCollision"))
  (Variables|QuestDetails|SetQuestStatus NewStatus)
  (return))

(fn CompleteQuest
  (Default|CallOnFinishQuest (Variables|Objectives|GetObjectives))
  (CallFunction|StatusChange "NewEnumerator4")
  (Variables|QuestDetails|SetIsComplete true)
  (Development|PrintString "quest completed"))

(fn UINewQuest
  (bind _overlapref (Variables|Objectives|GetOverlapRef))
  (bind _description (Variables|QuestDetails|GetDescription))
  (bind _objectivecounter (Variables|Objectives|GetObjectiveCounter))
  (bind _title (Variables|QuestDetails|GetTitle))
  (bind _goal (Variables|Default|GetGoal))
  (bind _returnvalue (> _objectivecounter 0))
  (bind _returnvalue_2 (Transformation|GetWorldLocation _goal))
  (switch Utilities|FlowControl|Switch|SwitchonObjectiveTypes (.Type (Utilities|Struct|BreakQuestStructVICKY (Utilities|Array|Get(acopy) (Variables|Objectives|GetObjectives) _objectivecounter)))
    (:NewEnumerator2
      (Class|ICharacter|NewQuestSet(Message) _overlapref _title _description _returnvalue_2 _returnvalue :!label _label))
    (:NewEnumerator4
      (Class|ICharacter|NewQuestSet(Message) _overlapref _title _description (Transformation|GetActorLocation (Variables|Default|GetNPCTarget)) _returnvalue))
    (:NewEnumerator5
      (goto _label))
    (:NewEnumerator6
      (Class|ICharacter|NewQuestSet(Message) _overlapref _title _description _returnvalue_2 _returnvalue))))

(fn NewObjective
  (bind _objectives (Variables|Objectives|GetObjectives))
  (bind _objectivecounter (Variables|Objectives|GetObjectiveCounter))
  (bind _returnvalue (+ _objectivecounter 1))
  (bind _output (Utilities|Array|Get(acopy) _objectives _returnvalue))
  (Utilities|Struct|SetmembersinQuestStructVICKY _output true)
  (Default|CallOnObjectiveCompleted _output)
  (CallFunction|NextObjective))

(fn StartObjective
  (bind _objectives (Variables|Objectives|GetObjectives))
  (Default|CallOnStartNewQuest (select (Variables|Objectives|GetCanWorkOnMultipleObjectes) _objectives (Utilities|Array|MakeArray (Utilities|Array|Get(acopy) _objectives (Variables|Objectives|GetObjectiveCounter))))))

(fn SetGoalSphere
  (params (SphereReference :type Sphere%20Component%20Object%20Reference) (SphereRadius :type Float%20%28single-precision%29))
  (Variables|Default|SetGoal SphereReference)
  (Components|Sphere|SetSphereRadius SphereReference SphereRadius true)
  (Collision|SetCollisionResponsetoChannel SphereReference "ECC_Camera" "ECR_Ignore")
  (Rendering|SetVisibility SphereReference true false)
  (Development|SetHiddeninGame SphereReference false false)
  (return))

(fn ChaseNPCFunction
  (params (Zone :type Sphere%20Component%20Object%20Reference))
  (return false))