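; Quest NPC actor that uses a thought bubble to show the item wanted for Fetch objectives and dances when its quest finishes.
; It shows the bubble at start for a Fetch objective and binds to its parent's quest events.
; On each completed objective it hides the bubble, then re-shows it with the current Fetch item's mesh pushed into the child actor.
; Finishing the quest loops a dance animation and hides the bubble.
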(event Custom|OnFinishQuest_Event_0
  (params (CompletedObjectives :type Array%20of%20Quest%20Struct%20Structures))
  (Components|Animation|PlayAnimation (Variables|Default|GetSkeletalMesh) "/Game/ArtAssets/Animations/Man/Sequences/MaleDanceExportNewDance.MaleDanceExportNewDance" true)
  (Rendering|SetVisibility (Variables|Default|GetThoughtBubble) false false))

(event Custom|NextObj
  (params (Objective :type Quest%20Struct%20Structure))
  (bind _objectivecounter (Variables|Default|GetObjectiveCounter))
  (bind _thoughtbubble (Variables|Default|GetThoughtBubble))
  (bind _objectives (Variables|Default|GetObjectives))
  (bind _output (Utilities|Array|Get(acopy) _objectives _objectivecounter))
  (bind _childactor (Variables|/Script/Engine.ChildActorComponent|GetChildActor _thoughtbubble))
  (bind (_objectivetext _type _iscomplete _questdetails) (Utilities|Struct|BreakQuestStruct _output))
  (bind _fetchitem (Utilities|Struct|BreakQuestDetails _questdetails))
  (bind _static_mesh_to_display (Variables|/Game/Blueprints/Grabbables/BP_Grabbable.BP_Grabbable_C|GetStatic%20Mesh%20To%20Display _fetchitem))
  ;[1 1 1] This isnt outputting the current objective
  (Rendering|SetVisibility (Variables|Default|GetThoughtBubble) false false)
  (switch Utilities|FlowControl|Switch|SwitchonObjectiveTypes _type
    (:NewEnumerator6
      (Utilities|IsValid _childactor
        (:Is%20Valid
          (bind _asbp_thought_bubble_parent (Utilities|Casting|CastToBP_ThoughtBubble_Parent _childactor))
          (Variables|/Game/Blueprints/QuestSystem/ThoughtBubbles/BP_ThoughtBubble_Parent.BP_ThoughtBubble_Parent_C|SetDisplayItem _asbp_thought_bubble_parent _static_mesh_to_display)
          (Components|StaticMesh|SetStaticMesh (Variables|/Game/Blueprints/QuestSystem/ThoughtBubbles/BP_ThoughtBubble_Parent.BP_ThoughtBubble_Parent_C|GetStaticMesh _asbp_thought_bubble_parent) _static_mesh_to_display)
          (Rendering|SetVisibility (Variables|Default|GetThoughtBubble) true false))))))

(event EventBeginPlay
  (|CallParentFunction)
  (EventDispatchers|BindEventtoOnObjectiveCompleted (delegate Custom|NextObj))
  (EventDispatchers|AssignOnFinishQuest (delegate Custom|OnFinishQuest_Event_0))
  (switch Utilities|FlowControl|Switch|SwitchonObjectiveTypes (.Type (Utilities|Struct|BreakQuestStruct (Utilities|Array|Get(acopy) (Variables|Default|GetObjectives) (Variables|Default|GetObjectiveCounter))))
    (:NewEnumerator6
      (Rendering|SetVisibility (Variables|Default|GetThoughtBubble) true false))))

(fn ConstructionScript
  (|CallParentFunction))