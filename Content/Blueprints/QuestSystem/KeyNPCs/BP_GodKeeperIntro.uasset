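; Cutscene actor that introduces the God BeeKeeper boss, hiding its stand-in mesh, swatter and the FortuneTeller until needed.
; BeginIntro moves the basket, quiets music and plays an ActorSequence camera shot with keeper animation, sound cues, timeline-driven swatter and logo widget.
; When the sequence finishes, it returns the camera, swaps in the real boss actor, restores FortuneTeller and music, then activates the boss AI controller.
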(event Custom|showLogo
  (bind _beekeeperlogowigref (Variables|Default|GetbeekeeperLogoWigRef))
  (UserInterface|Animation|PlayAnimation _beekeeperlogowigref (Variables|/Game/Widgets/W_beekeeperLogo.W_beekeeperLogo_C|Getanim_beeKeeperLogoPopup _beekeeperlogowigref) 0.0 1 "Forward" 1.0)
  (Widget|SetVisibility (Variables|/Game/Widgets/W_beekeeperLogo.W_beekeeperLogo_C|Getcan_logoHolder _beekeeperlogowigref) "HitTestInvisible"))

(event Custom|BeginIntro
  (params (Basket :type BP%20Basket%20Object%20Reference))
  (bind _godkeeperanim (Variables|Default|GetGodKeeperAnim))
  (bind _actorsequence (Variables|Default|GetActorSequence))
  (bind _basketlocation (Variables|Default|GetBasketLocation))
  (bind _returnvalue (Transformation|GetWorldLocation _basketlocation))
  (bind _sequenceplayer (Variables|/Script/ActorSequence.ActorSequenceComponent|GetSequencePlayer _actorsequence))
  (Utilities|FlowControl|Delay 2.0)
  (Class|ICharacter|SequenceTriggered(Message) (Game|Player|GetPlayerPawn 0) true)
  (Utilities|FlowControl|Sequence
    (:then_0
      (Game|Player|SetViewTargetwithBlend (Game|GetPlayerController 0) self 0.0 "VTBlend_Linear" 0.0 false)
      (Sequencer|Player|Play _sequenceplayer :!class /Script/MovieScene.MovieSceneSequencePlayer)
      (EventDispatchers|BindEventtoOnFinished _sequenceplayer (delegate Custom|Finished%20Intro))
      (Transformation|SetRelativeLocation _godkeeperanim "0, 0, 0" false true)
      (Components|Animation|PlayAnimation _godkeeperanim "/Game/ArtAssets/Animations/Beekeeper/Sequences/GodBeeKeeper_EngineReady.GodBeeKeeper_EngineReady" false)
      (Utilities|FlowControl|Sequence
        (:then_0
          (Utilities|FlowControl|Delay 5.0)
          (Rendering|SetVisibility (Variables|Default|GetSwatter) true false)
          (bind _alpha (Timeline|SwatterLerp PlayFromStart)
            (:Update
              (Transformation|SetRelativeLocation (Variables|Default|GetSwatter) (Math|Vector|Lerp(Vector) (Variables|Default|GetSwatterLocation) (Variables|Default|GetSwatterOrigin) _alpha) false false))
            (:Finished
              (bind _returnvalue_2 (UserInterface|CreateWidget "/Game/Widgets/W_beekeeperLogo.W_beekeeperLogo_C"))
              (Variables|Default|SetbeekeeperLogoWigRef _returnvalue_2)
              (UserInterface|Viewport|AddtoViewport (Variables|Default|GetbeekeeperLogoWigRef) 0)
              (UserInterface|Animation|PlayAnimation (Variables|Default|GetbeekeeperLogoWigRef) (Variables|/Game/Widgets/W_beekeeperLogo.W_beekeeperLogo_C|Getanim_cutsceneBlackEnter (Variables|Default|GetbeekeeperLogoWigRef)) 0.0 1 "Forward" 1.0)
              (Utilities|Time|SetTimerbyEvent (delegate Custom|showLogo) 1.6))))
        (:then_1
          (Utilities|FlowControl|Delay 2.0)
          (Audio|PlaySound2D "/Game/Audio/Dialogue/BeekeeperBoss/Spotted/BeeKeeperSpotted.BeeKeeperSpotted" 1.0 1.0 0.0 0 0))))
    (:then_1
      (Transformation|SetActorLocation Basket (Math|Vector|MakeVector (.x _returnvalue) (.y _returnvalue) (+ (.z _returnvalue) 3e+03)) false true))
    (:then_2
      (bind _outactors (Actor|GetAllActorsOfClass "/Game/Blueprints/Managers/MusicManager.MusicManager_C"))
      (Default|SetQuiet (Utilities|Array|Get(acopy) _outactors))
      (Audio|PlaySound2D "/Game/Audio/Soundtracks/BossIntroCue.BossIntroCue" 0.6 1.0 0.0 0 0))))

(event Custom|Finished%20Intro
  (bind _returnvalue (Game|Player|GetPlayerPawn 0))
  (bind _godkeeperactor (Variables|Default|GetGodKeeperActor))
  (Game|Player|SetViewTargetwithBlend (Game|GetPlayerController 0) (Game|Player|GetPlayerPawn 0) 0.5 "VTBlend_Linear" 0.0 false)
  (Widget|RemovefromParent (Variables|Default|GetbeekeeperLogoWigRef))
  (Utilities|IsValid _godkeeperactor
    (:Is%20Valid
      (Transformation|SetActorLocation _godkeeperactor (Transformation|GetActorLocation) false true)
      (Components|DestroyComponent (Variables|Default|GetGodKeeperAnim))
      (Transformation|SetActorLocation (Variables|Default|GetFortuneTeller) (Variables|Default|GetFortuneTellerLocation) false false)
      (bind _outactors (Actor|GetAllActorsOfClass "/Game/Blueprints/Managers/MusicManager.MusicManager_C"))
      (Default|SetLoud (Utilities|Array|Get(acopy) _outactors))
      (Class|ICharacter|SequenceTriggered(Message) _returnvalue false)
      (bind _asbee_character_bp (Utilities|Casting|CastToBeeCharacter_BP _returnvalue))
      (Default|RevealBoss _asbee_character_bp)
      (bind _asbp_bee_keeper_boss_con (Utilities|Casting|CastToBP_BeeKeeperBossCon (AI|GetAIController (Variables|Default|GetGodKeeperActor))))
      (Default|Activated _asbp_bee_keeper_boss_con))))

(event Custom|TickUp
  (bind _output_get (Variables|Default|SetTime (+ (Variables|Default|GetTime) 0.1)))
  (Development|PrintString (Utilities|String|ToString(Float) _output_get)))

(event EventBeginPlay
  (bind _fortuneteller (Variables|Default|GetFortuneTeller))
  (bind _swatter (Variables|Default|GetSwatter))
  (bind _returnvalue (Transformation|GetActorLocation _fortuneteller))
  (Transformation|SetRelativeLocation (Variables|Default|GetGodKeeperAnim) "0, 0,-3000.000000" false true)
  (Variables|Default|SetSwatterOrigin (Variables|/Script/Engine.SceneComponent|GetRelativeLocation _swatter))
  (Transformation|SetRelativeLocation _swatter (Variables|Default|GetSwatterLocation) false false)
  (Rendering|SetVisibility (Variables|Default|GetSwatter) false false)
  (Variables|Default|SetFortuneTellerLocation _returnvalue)
  (Transformation|SetActorRelativeLocation _fortuneteller (- _returnvalue "0, 0,3000.000000")))

(fn ConstructionScript
  (bind _godkeeperanim (Variables|Default|GetGodKeeperAnim))
  (Utilities|IsValid _godkeeperanim
    (:Is%20Valid
      (for (_array_element _array_index) (Rendering|Material|GetMaterials _godkeeperanim)
        (Rendering|Material|SetMaterial (Variables|Default|GetGodKeeperAnim) _array_index _array_element)))))