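; BP_EndGameCutscene is the end-game cutscene actor, showing the beekeeper's death.
; StartSequence hides the player bee's mesh and to-do list, switches the view to itself and plays its ActorSequence, whose finish sends GameEndMessage to the game mode.
; After a delay, the BeeKeeper, parked far below at BeginPlay, moves up and plays its death montage, with two timelines lerping its position.
; A camera fade and credits widget branch never runs.
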(event Custom|Finished
  (Class|IGameMode|GameEnd(Message) (Game|GetGameMode)))

(event Custom|StartSequence
  (bind _beekeeper (Variables|Default|GetBeeKeeper))
  (bind _beekeeper_2 (Variables|Default|GetBeeKeeper))
  (bind _actorsequence (Variables|Default|GetActorSequence))
  (bind _sequenceplayer (Variables|/Script/ActorSequence.ActorSequenceComponent|GetSequencePlayer _actorsequence))
  (bind _relativelocation (Variables|/Script/Engine.SceneComponent|GetRelativeLocation _beekeeper))
  (Utilities|FlowControl|Delay 2.0)
  (Class|ICharacter|SequenceTriggered(Message) (Game|Player|GetPlayerPawn 0) true)
  (bind _asbee_character_bp (Utilities|Casting|CastToBeeCharacter_BP (Game|Player|GetPlayerPawn 0)))
  (Rendering|SetVisibility (Variables|/Game/Blueprints/Character/BeeCharacter_BP.BeeCharacter_BP_C|Getwigc_todoList _asbee_character_bp) false false)
  (Class|IGameMode|PrepareEnd(Message) (Game|GetGameMode))
  (Game|Player|SetViewTargetwithBlend (Game|GetPlayerController 0) self 0.0 "VTBlend_Linear" 0.0 false)
  (Sequencer|Player|Play _sequenceplayer :!class /Script/MovieScene.MovieSceneSequencePlayer)
  (EventDispatchers|BindEventtoOnFinished _sequenceplayer (delegate Custom|Finished))
  (Utilities|FlowControl|Delay 6.0)
  (Transformation|SetRelativeLocation _beekeeper_2 "0, 0,-50.000000" false false)
  (Utilities|FlowControl|Sequence
    (:then_0
      (Animation|Montage|PlayMontage _beekeeper_2 "/Game/ArtAssets/Animations/Beekeeper/Sequences/Beekeeper_Death_Montage.Beekeeper_Death_Montage"
        (:OnBlendOut
          (bind _alpha (Timeline|Timeline_0 PlayFromStart)
            (:Update
              (Transformation|SetRelativeLocation (Variables|Default|GetBeeKeeper) (Math|Vector|Lerp(Vector) _relativelocation (+ _relativelocation "0, 0,50.000000") _alpha) false false))))))
    (:then_1
      (bind _alpha_2 (Timeline|Lerp PlayFromStart)
        (:Update
          (Transformation|SetRelativeLocation (Variables|Default|GetBeeKeeper) (Math|Vector|Lerp(Vector) (Variables|/Script/Engine.SceneComponent|GetRelativeLocation (Variables|Default|GetBeeKeeper)) "0, 0, 0" _alpha_2) false false))))))

(event EventBeginPlay
  (Transformation|SetRelativeLocation (Variables|Default|GetBeeKeeper) "0, 0,-3000.000000" false false))

(fn ConstructionScript)