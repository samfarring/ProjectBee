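; Quest hot air balloon that bobs in place and explodes the first time it takes damage.
; A looping timer re-triggers a DoOnce-gated timeline that moves the static mesh vertically.
; On damage it spawns a quest basket below and passes it to the intro animation actor.
; With a valid quest it reports back, stops bobbing and removes its meshes; otherwise it destroys itself.
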(event Custom|StopAll
  (bind _height (Timeline|Timeline_0 Stop)
    (:Update
      (Transformation|SetRelativeLocation (Variables|Default|GetStaticMesh) (Math|Vector|MakeVector 0.0 0.0 (Math|Float|Lerp 0.0 1e+02 _height)) false false))
    (:Finished
      (Utilities|FlowControl|DoOnce false) ; enters at Reset
    )))

(event Custom|Height
  (Utilities|FlowControl|DoOnce false :!label _label
    (:Completed
      (bind _height (Timeline|Timeline_0 PlayFromStart)
        (:Update
          (Transformation|SetRelativeLocation (Variables|Default|GetStaticMesh) (Math|Vector|MakeVector 0.0 0.0 (Math|Float|Lerp 0.0 1e+02 _height)) false false))
        (:Finished
          (goto _label Reset))))))

(event EventBeginPlay
  (|CallParentFunction)
  (bind _returnvalue (Utilities|Time|SetTimerbyEvent (delegate Custom|Height) 1e+01 true))
  (Variables|Default|SetMoveTimer _returnvalue)
  (Utilities|FlowControl|DoOnce false :!label _label
    (:Completed
      (bind _height (Timeline|Timeline_0 PlayFromStart)
        (:Update
          (Transformation|SetRelativeLocation (Variables|Default|GetStaticMesh) (Math|Vector|MakeVector 0.0 0.0 (Math|Float|Lerp 0.0 1e+02 _height)) false false))
        (:Finished
          (goto _label Reset))))))

(event Game|Damage|EventAnyDamage
  (params (Damage :type Float%20%28single-precision%29) (DamageType :type Damage%20Type%20Object%20Reference) (InstigatedBy :type Controller%20Object%20Reference) (DamageCauser :type Actor%20Object%20Reference))
  (bind _returnvalue (Transformation|GetActorLocation))
  (bind _introanimactor (Variables|Default|GetIntroAnimActor))
  (Utilities|FlowControl|DoOnce false
    (:Completed
      (Effects|SpawnEmitteratLocation "/Game/Blueprints/Particles/Explosion.Explosion" (Transformation|GetActorLocation) "0, 0, 0" "20.000000,20.000000,20.000000")
      (bind _returnvalue_2 (Game|SpawnActorfromClass "/Game/Blueprints/Puzzles/BP_Basket.BP_Basket_C" (Math|Transform|MakeTransform (Math|Vector|MakeVector (.x _returnvalue) (.y _returnvalue) (- (.z _returnvalue) 4e+02)) "0, 0, 0" "1,1,1") "Undefined" 0 true 0))
      (Utilities|IsValid _introanimactor
        (:Is%20Valid
          (Default|BeginIntro _introanimactor _returnvalue_2))
        (:Is%20Not%20Valid
          _))
      (Utilities|IsValid (stale EventStingNPC Quest)
        (:Is%20Valid
          (Default|StingQuestReturn (stale EventStingNPC Quest))
          (CallFunction|StopAll)
          (Utilities|Time|ClearandInvalidateTimerbyHandle (Variables|Default|GetMoveTimer))
          (Components|DestroyComponent (Variables|Default|GetStaticMesh)))
        (:Is%20Not%20Valid
          (Actor|DestroyActor))))))

(event EventStingNPC
  (params (Quest :type BP%20Quest%20Actor%20Object%20Reference)))

(fn ConstructionScript
  (|CallParentFunction))