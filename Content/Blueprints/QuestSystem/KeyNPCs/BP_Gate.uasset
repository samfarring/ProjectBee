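; Quest gate actor that plays the beekeeper's one-time intro cutscene when its quest event fires.
; It hides the van and beekeepers below ground until an Actor Sequence takes the camera, with music, animation and logo widget.
; A looping timer through a Gate node briefly pushes both metal doors with impulses.
; On finish it restores the view, swaps the stand-in for the real beekeeper and notifies the quest, or removes the world border without one.
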(event OnComponentBeginOverlap(Sphere)
  (params (OverlappedComponent :type Primitive%20Component%20Object%20Reference) (OtherActor :type Actor%20Object%20Reference) (OtherComp :type Primitive%20Component%20Object%20Reference) (OtherBodyIndex :type Integer) (bFromSweep :type Boolean) (SweepResult :type Hit%20Result%20Structure%20%28by%20ref%29))
  ;[1 1 1] Change this to an event connected to the quest
)

(event Custom|showLogo
  (bind _beekeeperlogowigref (Variables|Default|GetbeekeeperLogoWigRef))
  (UserInterface|Animation|PlayAnimation _beekeeperlogowigref (Variables|/Game/Widgets/W_beekeeperLogo.W_beekeeperLogo_C|Getanim_beeKeeperLogoPopup _beekeeperlogowigref) 0.0 1 "Forward" 1.0)
  (Widget|SetVisibility (Variables|/Game/Widgets/W_beekeeperLogo.W_beekeeperLogo_C|Getcan_logoHolder _beekeeperlogowigref) "HitTestInvisible"))

(event Custom|Tick%20Gate%20Movement
  (Utilities|FlowControl|Gate true
    (:Exit
      (Physics|AddImpulse (Variables|Default|Geta_MetalGate1) (* (Math|Vector|GetForwardVector (Variables|Default|GetArrow)) 1e+04) "None" false))))

(event Custom|Finished%20Intro%20Anim
  (bind _returnvalue (Game|Player|GetPlayerPawn 0))
  (bind _beekeeperref (Variables|Default|GetBeeKeeperRef))
  (Game|Player|SetViewTargetwithBlend (Game|GetPlayerController 0) (Game|Player|GetPlayerPawn 0) 0.5 "VTBlend_Linear" 0.0 false)
  (Widget|RemovefromParent (Variables|Default|GetbeekeeperLogoWigRef))
  (bind _outactors (Actor|GetAllActorsOfClass "/Game/Blueprints/Managers/MusicManager.MusicManager_C"))
  (Default|SetLoud (Utilities|Array|Get(acopy) _outactors))
  (Utilities|FlowControl|Sequence
    (:then_0
      (Utilities|IsValid _beekeeperref
        (:Is%20Valid
          (Transformation|SetActorLocation _beekeeperref (Transformation|GetWorldLocation (Variables|Default|GetDefaultSceneRoot)) false false))
        (:Is%20Not%20Valid
          _))
      (Components|DestroyComponent (Variables|Default|GetBeeKeeper))
      (Utilities|IsValid (stale EventEventFiring Quest)
        (:Is%20Valid
          (Default|EventFiringReturn (stale EventEventFiring Quest)))
        (:Is%20Not%20Valid
          ;[1 1 1] Cannot be connected because of level streaming
          (Actor|DestroyActor (Variables|Default|GetWorldBorder))
          (bind _asgm_bee (Utilities|Casting|CastToGM_Bee (Game|GetGameMode)))
          (Default|UIBounds _asgm_bee))))
    (:then_1
      (Class|ICharacter|SequenceTriggered(Message) _returnvalue false)
      (bind _asbee_character_bp (Utilities|Casting|CastToBeeCharacter_BP _returnvalue))
      (Default|RevealBeeK _asbee_character_bp))))

(event EventBeginPlay
  (bind _beekeeper (Variables|Default|GetBeeKeeper))
  (Variables|Default|SetBeginLocationKeeper (Variables|/Script/Engine.SceneComponent|GetRelativeLocation _beekeeper))
  (Variables|Default|SetBeginLocationVan (Variables|/Script/Engine.SceneComponent|GetRelativeLocation (Variables|Default|GetVan)))
  (Transformation|SetRelativeLocation _beekeeper "0, 0,-3000.000000" false false)
  (Transformation|SetActorRelativeLocation (Variables|Default|GetBeeKeeperRef) (Math|Vector|MakeVector (.x (Variables|Default|GetBeginLocationVan)) (.y (Variables|Default|GetBeginLocationVan)) -3e+03) false true))

(event EventEventFiring
  (params (Quest :type BP%20Quest%20Actor%20Object%20Reference) (Bee :type Bee%20Character%20BP%20Object%20Reference))
  (bind _actorsequence (Variables|Default|GetActorSequence))
  (bind _sequenceplayer (Variables|/Script/ActorSequence.ActorSequenceComponent|GetSequencePlayer _actorsequence))
  (Utilities|FlowControl|DoOnce false
    (:Completed
      (Utilities|FlowControl|Delay 2.0)
      (if (not (Variables|Default|GettriggeredSequence))
        (CallFunction|SoundEffects)
        (Variables|Default|SettriggeredSequence true)
        (Game|Player|SetViewTargetwithBlend (Game|GetPlayerController 0) self 0.0 "VTBlend_Linear" 0.0 false)
        (Sequencer|Player|Play _sequenceplayer :!class /Script/MovieScene.MovieSceneSequencePlayer)
        (Transformation|SetRelativeLocation (Variables|Default|GetVan) (Variables|Default|GetBeginLocationVan) false false)
        (Utilities|FlowControl|Sequence
          (:then_0
            (Utilities|FlowControl|Delay 0.25)
            (Transformation|SetRelativeLocation (Variables|Default|GetBeeKeeper) (Variables|Default|GetBeginLocationKeeper) false false)
            (Components|Animation|PlayAnimation (Variables|Default|GetBeeKeeper) "/Game/ArtAssets/Animations/Beekeeper/Sequences/BeeKeeperJumpOuttaVan_EnginerReady.BeeKeeperJumpOuttaVan_EnginerReady" false)
            (bind _returnvalue (Utilities|Time|SetTimerbyEvent (delegate Custom|Tick%20Gate%20Movement) 0.01 true))
            (Utilities|FlowControl|Sequence
              (:then_0
                (Utilities|FlowControl|Gate true) ; enters at Open
              )
              (:then_1
                (Utilities|FlowControl|Delay 4.0)
                (Utilities|Time|ClearandInvalidateTimerbyHandle _returnvalue)
                (Utilities|FlowControl|Gate true) ; enters at Close
              )))
          (:then_1
            (EventDispatchers|BindEventtoOnFinished _sequenceplayer (delegate Custom|Finished%20Intro%20Anim))
            (bind _returnvalue_2 (UserInterface|CreateWidget "/Game/Widgets/W_beekeeperLogo.W_beekeeperLogo_C"))
            (Variables|Default|SetbeekeeperLogoWigRef _returnvalue_2)
            (UserInterface|Viewport|AddtoViewport (Variables|Default|GetbeekeeperLogoWigRef) 0)
            (UserInterface|Animation|PlayAnimation (Variables|Default|GetbeekeeperLogoWigRef) (Variables|/Game/Widgets/W_beekeeperLogo.W_beekeeperLogo_C|Getanim_cutsceneBlackEnter (Variables|Default|GetbeekeeperLogoWigRef)) 0.0 1 "Forward" 1.0)
            (Utilities|Time|SetTimerbyEvent (delegate Custom|showLogo) 1.6)
            (Class|ICharacter|SequenceTriggered(Message) (Game|Player|GetPlayerPawn 0) true)))))))

(fn ConstructionScript
  (bind _beekeeperref (Variables|Default|GetBeeKeeperRef))
  (Utilities|IsValid _beekeeperref
    (:Is%20Valid
      (for (_array_element _array_index) (Rendering|Material|GetMaterials (Variables|/Script/Engine.Character|GetMesh _beekeeperref))
        (Rendering|Material|SetMaterial (Variables|Default|GetBeeKeeper) _array_index _array_element)))))

(fn SoundEffects
  (bind _outactors (Actor|GetAllActorsOfClass "/Game/Blueprints/Managers/MusicManager.MusicManager_C"))
  (Default|SetQuiet (Utilities|Array|Get(acopy) _outactors))
  (Audio|PlaySound2D "/Game/Audio/Soundtracks/BossIntroCue.BossIntroCue" 0.6 1.0 0.0 0 0))