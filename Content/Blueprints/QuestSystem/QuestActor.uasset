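; Quest giver actor that offers a quest when a bee player enters its zone, with status toggling the zone's collision.
; The first objective's type picks the setup: Location spawns a visible trigger sphere, while Sting, with random AI enabled, makes separate random draws for target assignment and stung-event binding.
; Reaching the sphere or the stung event completes the quest, with start and finish broadcast through dispatchers carrying the objectives.
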(event OnComponentBeginOverlap(QuestZone)
  (params (OverlappedComponent :type Primitive%20Component%20Object%20Reference) (OtherActor :type Actor%20Object%20Reference) (OtherComp :type Primitive%20Component%20Object%20Reference) (OtherBodyIndex :type Integer) (bFromSweep :type Boolean) (SweepResult :type Hit%20Result%20Structure%20%28by%20ref%29))
  (bind _isbee (Class|ICharacter|GetBeePlayer(Message) OtherActor OtherActor))
  (Utilities|FlowControl|DoOnce false
    (:Completed
      (if _isbee
        (Development|PrintString "quest started")
        (CallFunction|StatusChange "NewEnumerator3")
        (switch Utilities|FlowControl|Switch|SwitchonObjectiveTypes (.Type (Utilities|Struct|BreakQuestStruct (Utilities|Array|Get(acopy) (Variables|Objectives|GetObjectives))))
          (:NewEnumerator2
            ;[1 1 1] Go To Location
            (Utilities|FlowControl|DoOnce false
              (:Completed
                (bind _returnvalue (AddComponent|AddSphereComponent false (Math|Conversions|ToTransform(Vector) (Variables|Default|GetLocation))))
                (Collision|AssignOnComponentBeginOverlap _returnvalue (delegate Custom|OnComponentBeginOverlap_Event_1))
                (Components|Sphere|SetSphereRadius _returnvalue 128.0 true)
                ;;[1 1 1] Debug
                (Rendering|SetVisibility _returnvalue true false)
                (Development|SetHiddeninGame _returnvalue false false)
                (Development|PrintString "quest created")
                (Default|CallOnStartNewQuest (Variables|Objectives|GetObjectives)))))
          (:NewEnumerator4
            (bind _outactors (Actor|GetAllActorsOfClass "/Game/Blueprints/AI/Character/BP_BackgroundAI_Base.BP_BackgroundAI_Base_C"))
            (if (Variables|Default|GetUseRandomAI)
              (Default|AssignTarget (Utilities|Array|Get(acopy) _outactors (Math|Random|RandomInteger (- (Utilities|Array|Length _outactors) 1))))
              (EventDispatchers|BindEventtoOnStung (Utilities|Array|Get(acopy) _outactors (Math|Random|RandomInteger (- (Utilities|Array|Length _outactors) 1))) (delegate Custom|StungTarget))
              (Default|CallOnStartNewQuest (Variables|Objectives|GetObjectives)))))))))

(event OnComponentEndOverlap(QuestZone)
  (params (OverlappedComponent :type Primitive%20Component%20Object%20Reference) (OtherActor :type Actor%20Object%20Reference) (OtherComp :type Primitive%20Component%20Object%20Reference) (OtherBodyIndex :type Integer))
  (Utilities|FlowControl|DoOnce false) ; enters at Reset
)

(event Custom|StungTarget
  (CallFunction|CompleteQuest))

(event Custom|OnComponentBeginOverlap_Event_1
  (params (OverlappedComponent :type Primitive%20Component%20Object%20Reference) (OtherActor :type Actor%20Object%20Reference) (OtherComp :type Primitive%20Component%20Object%20Reference) (OtherBodyIndex :type Integer) (bFromSweep :type Boolean) (SweepResult :type Hit%20Result%20Structure%20%28by%20ref%29))
  ;[1 1 1] Go To Location
  (bind _isbee (Class|ICharacter|GetBeePlayer(Message) OtherActor OtherActor))
  (if _isbee
    (Development|PrintString "quest over")
    (Default|CallOnFinishQuest (Variables|Objectives|GetObjectives))
    (CallFunction|StatusChange "NewEnumerator4")
    (EventDispatchers|UnbindallEventsfromOnComponentBeginOverlap (stale OnComponentBeginOverlap(QuestZone) _returnvalue))
    (Components|DestroyComponent (stale OnComponentBeginOverlap(QuestZone) _returnvalue))))

(event EventBeginPlay
  (CallFunction|StatusChange "NewEnumerator1"))

(fn ConstructionScript)

(fn StatusChange
  (params (NewStatus :type QuestStatus%20Enum :default "NewEnumerator0"))
  (Collision|SetCollisionEnabled (Variables|Default|GetQuestZone) (Utilities|Select :Index NewStatus :NewEnumerator0 "NoCollision" :NewEnumerator1 "QueryOnly" :NewEnumerator2 "NoCollision" :NewEnumerator3 "NoCollision" :NewEnumerator4 "NoCollision"))
  (Variables|QuestDetails|SetQuestStatus NewStatus)
  (return))

(fn CompleteQuest
  (bind _objectives (Variables|Objectives|GetObjectives))
  (Default|CallOnFinishQuest _objectives)
  (CallFunction|StatusChange "NewEnumerator4")
  (for _array_element _objectives
    (Utilities|Struct|SetmembersinQuestStruct _array_element true)))