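; Parent thought bubble actor for the quest system that shows a configurable item mesh over an animated bubble sprite.
; The construction script applies the display mesh, rotation and scale.
; On BeginPlay it offsets the billboard backward along the arrow from the mesh's bounds center and caches the bee player.
; Tick turns the arrow toward the bee's camera, while a Delay swaps among three random bubble sprites roughly every half second.
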(event EventTick
  (params (DeltaSeconds :type Float%20%28single-precision%29))
  (bind _billboard (Variables|Default|GetBillboard))
  (Utilities|FlowControl|Sequence
    (:then_0
      (Utilities|FlowControl|Delay 0.5)
      (switch int (Math|Random|RandomIntegerinRange 0 2)
        (:0
          (Rendering|Components|Sprite|SetSprite _billboard "/Game/Blueprints/QuestSystem/ThoughtBubbles/Bubble_1.Bubble_1"))
        (:1
          (Rendering|Components|Sprite|SetSprite _billboard "/Game/Blueprints/QuestSystem/ThoughtBubbles/Bubble_2.Bubble_2"))
        (:2
          (Rendering|Components|Sprite|SetSprite _billboard "/Game/Blueprints/QuestSystem/ThoughtBubbles/Bubble_3.Bubble_3"))))
    (:then_1
      (Transformation|SetWorldRotation (Variables|Default|GetArrow) (Math|Rotator|FindLookatRotation (Transformation|GetWorldLocation (Variables|Default|GetArrow)) (Transformation|GetWorldLocation (Variables|/Game/Blueprints/Character/BeeCharacter_BP.BeeCharacter_BP_C|GetCamera (Variables|Default|GetBee)))) false false))))

(event EventBeginPlay
  (Transformation|SetWorldLocation (Variables|Default|GetBillboard) (+ (* (Math|Vector|GetForwardVector (Variables|Default|GetArrow)) -3e+01) (.Origin (Collision|GetComponentBounds (Variables|Default|GetStaticMesh)))) false false)
  (bind _asbee_character_bp (Utilities|Casting|CastToBeeCharacter_BP (Game|Player|GetPlayerPawn 0)))
  (Variables|Default|SetBee _asbee_character_bp))

(fn ConstructionScript
  (bind _staticmesh (Variables|Default|GetStaticMesh))
  (Components|StaticMesh|SetStaticMesh (Variables|Default|GetStaticMesh) (Variables|Default|GetDisplayItem))
  (Transformation|SetRelativeRotation _staticmesh (Variables|Default|GetAlterRotation) false false)
  (Transformation|SetRelativeScale3D _staticmesh (Variables|Default|GetAlterScale)))