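; Base quest actor that starts when the bee player enters its QuestZone and tracks objectives to completion.
; NextObjective sets up Location, Sting, Chase or Fetch objectives, singly or all together, using runtime overlap spheres or a sting binding on an AI target.
; Finished objectives increment a counter that triggers the next one or CompleteQuest.
; Dispatchers announce progress, the player receives UI messages, and quest status toggles the zone's collision.
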(event OnComponentBeginOverlap(QuestZone)
  (params (OverlappedComponent :type Primitive%20Component%20Object%20Reference) (OtherActor :type Actor%20Object%20Reference) (OtherComp :type Primitive%20Component%20Object%20Reference) (OtherBodyIndex :type Integer) (bFromSweep :type Boolean) (SweepResult :type Hit%20Result%20Structure%20%28by%20ref%29))
  (bind _objectives (Variables|Objectives|GetObjectives))
  (bind _canworkonmultipleobjectes (Variables|Objectives|GetCanWorkOnMultipleObjectes))
  (bind _asbee_character_bp (Utilities|Casting|CastToBeeCharacter_BP OtherActor))
  (Variables|Objectives|SetOverlapRef _asbee_character_bp)
  (bind _isbee (Class|ICharacter|GetBeePlayer(Message) _asbee_character_bp _asbee_character_bp))
  (Utilities|FlowControl|DoOnce false
    (:Completed
      (if _isbee
        (Variables|Objectives|SetObjectiveLength (Utilities|Array|Length _objectives))
        (CallFunction|StatusChange "NewEnumerator3")
        (if _canworkonmultipleobjectes
          (for _array_element (Variables|Objectives|GetObjectives)
            (switch Utilities|FlowControl|Switch|SwitchonObjectiveTypes (select _canworkonmultipleobjectes (.Type (Utilities|Struct|BreakQuestStruct _array_element)) (.Type (Utilities|Struct|BreakQuestStruct (Utilities|Array|Get(acopy) _objectives (Variables|Objectives|GetObjectiveCounter)))))
              (:NewEnumerator2
                ;[1 1 1] Go To Location
                (Utilities|FlowControl|DoOnce false
                  (:Completed
                    (bind _returnvalue (AddComponent|AddSphereComponent false (Math|Conversions|ToTransform(Vector) (Variables|Location|GetLocation))))
                    (Collision|AssignOnComponentBeginOverlap _returnvalue (delegate Custom|OnComponentBeginOverlap_Event_1))
                    (Components|Sphere|SetSphereRadius _returnvalue (Variables|Location|GetCompletionOverlapSize) true)
                    ;;[1 1 1] Debug
                    (Rendering|SetVisibility _returnvalue true false)
                    (Development|SetHiddeninGame _returnvalue false false)
                    (Development|PrintString "location started")
                    (CallFunction|StartObjective)
                    (CallFunction|UINewQuest))))
              (:NewEnumerator4
                ;[1 1 1] Sting
                (bind _outactors (Actor|GetAllActorsOfClass "/Game/Blueprints/AI/Character/BP_BackgroundAI_Base.BP_BackgroundAI_Base_C"))
                (Development|PrintString "sting started")
                (if (Variables|AI|GetUseRandomAI)
                  (bind _output_get (Variables|AI|SetAITarget (Utilities|Array|Get(acopy) _outactors (Math|Random|RandomInteger (- (Utilities|Array|Length _outactors) 1)))))
                  (Default|AssignTarget _output_get)
                  (else
                    (Default|AssignTarget (Variables|AI|GetAITarget))))
                (EventDispatchers|BindEventtoOnStung (Variables|AI|GetAITarget) (delegate Custom|StungTarget))
                (CallFunction|StartObjective)
                (CallFunction|UINewQuest))
              (:NewEnumerator5
                (Development|PrintString "chase started")
                ;[1 1 1] Chase
                (bind _outactors_2 (Actor|GetAllActorsOfClass "/Game/Blueprints/AI/Character/BP_CivilianChaseable.BP_CivilianChaseable_C"))
                (if (Variables|AI|GetUseRandomAI)
                  (Variables|AI|SetAITarget (Utilities|Array|Get(acopy) _outactors_2 (Math|Random|RandomInteger (- (Utilities|Array|Length _outactors_2) 1))))
                  (Default|AssignTarget (Utilities|Array|Get(acopy) _outactors_2 (Math|Random|RandomInteger (- (Utilities|Array|Length _outactors_2) 1))))
                  (else
                    (Default|AssignTarget (Variables|AI|GetAITarget))))
                (bind _returnvalue_2 (AddComponent|AddSphereComponent false (Math|Conversions|ToTransform(Vector) (Variables|Location|GetLocation))))
                (Collision|BindEventtoOnComponentBeginOverlap _returnvalue_2 (delegate Custom|Overlap))
                (Components|Sphere|SetSphereRadius _returnvalue_2 (Variables|Location|GetCompletionOverlapSize) true)
                (Rendering|SetVisibility _returnvalue_2 true false)
                (Development|SetHiddeninGame _returnvalue_2 false false)
                (CallFunction|StartObjective)
                (CallFunction|UINewQuest))
              (:NewEnumerator6
                ;[1 1 1] Fetch
                (Development|PrintString "fetch started")
                (Utilities|FlowControl|DoOnce false
                  (:Completed
                    (bind _returnvalue_3 (AddComponent|AddSphereComponent false (Math|Conversions|ToTransform(Vector) (Variables|Location|GetLocation))))
                    (Collision|AssignOnComponentBeginOverlap _returnvalue_3 (delegate Custom|Begin%20Overlap))
                    (Components|Sphere|SetSphereRadius _returnvalue_3 (Variables|Location|GetCompletionOverlapSize) true)
                    (CallFunction|StartObjective)
                    (CallFunction|UINewQuest))))))
          (else
            (switch Utilities|FlowControl|Switch|SwitchonObjectiveTypes (select _canworkonmultipleobjectes (.Type (Utilities|Struct|BreakQuestStruct _array_element)) (.Type (Utilities|Struct|BreakQuestStruct (Utilities|Array|Get(acopy) _objectives (Variables|Objectives|GetObjectiveCounter)))))
              (:NewEnumerator2
                (Utilities|FlowControl|DoOnce false
                  (:Completed
                    (bind _returnvalue_4 (AddComponent|AddSphereComponent false (Math|Conversions|ToTransform(Vector) (Variables|Location|GetLocation))))
                    (Collision|AssignOnComponentBeginOverlap _returnvalue_4 (delegate Custom|OnComponentBeginOverlap_Event_1))
                    (Components|Sphere|SetSphereRadius _returnvalue_4 (Variables|Location|GetCompletionOverlapSize) true)
                    (Rendering|SetVisibility _returnvalue_4 true false)
                    (Development|SetHiddeninGame _returnvalue_4 false false)
                    (Development|PrintString "location started")
                    (CallFunction|StartObjective)
                    (CallFunction|UINewQuest))))
              (:NewEnumerator4
                (bind _outactors_3 (Actor|GetAllActorsOfClass "/Game/Blueprints/AI/Character/BP_BackgroundAI_Base.BP_BackgroundAI_Base_C"))
                (Development|PrintString "sting started")
                (if (Variables|AI|GetUseRandomAI)
                  (bind _output_get_2 (Variables|AI|SetAITarget (Utilities|Array|Get(acopy) _outactors_3 (Math|Random|RandomInteger (- (Utilities|Array|Length _outactors_3) 1)))))
                  (Default|AssignTarget _output_get_2)
                  (else
                    (Default|AssignTarget (Variables|AI|GetAITarget))))
                (EventDispatchers|BindEventtoOnStung (Variables|AI|GetAITarget) (delegate Custom|StungTarget))
                (CallFunction|StartObjective)
                (CallFunction|UINewQuest))
              (:NewEnumerator5
                (Development|PrintString "chase started")
                (bind _outactors_4 (Actor|GetAllActorsOfClass "/Game/Blueprints/AI/Character/BP_CivilianChaseable.BP_CivilianChaseable_C"))
                (if (Variables|AI|GetUseRandomAI)
                  (Variables|AI|SetAITarget (Utilities|Array|Get(acopy) _outactors_4 (Math|Random|RandomInteger (- (Utilities|Array|Length _outactors_4) 1))))
                  (Default|AssignTarget (Utilities|Array|Get(acopy) _outactors_4 (Math|Random|RandomInteger (- (Utilities|Array|Length _outactors_4) 1))))
                  (else
                    (Default|AssignTarget (Variables|AI|GetAITarget))))
                (bind _returnvalue_5 (AddComponent|AddSphereComponent false (Math|Conversions|ToTransform(Vector) (Variables|Location|GetLocation))))
                (Collision|BindEventtoOnComponentBeginOverlap _returnvalue_5 (delegate Custom|Overlap))
                (Components|Sphere|SetSphereRadius _returnvalue_5 (Variables|Location|GetCompletionOverlapSize) true)
                (Rendering|SetVisibility _returnvalue_5 true false)
                (Development|SetHiddeninGame _returnvalue_5 false false)
                (CallFunction|StartObjective)
                (CallFunction|UINewQuest))
              (:NewEnumerator6
                (Development|PrintString "fetch started")
                (Utilities|FlowControl|DoOnce false
                  (:Completed
                    (bind _returnvalue_6 (AddComponent|AddSphereComponent false (Math|Conversions|ToTransform(Vector) (Variables|Location|GetLocation))))
                    (Collision|AssignOnComponentBeginOverlap _returnvalue_6 (delegate Custom|Begin%20Overlap))
                    (Components|Sphere|SetSphereRadius _returnvalue_6 (Variables|Location|GetCompletionOverlapSize) true)
                    (CallFunction|StartObjective)
                    (CallFunction|UINewQuest)))))))))))

(event OnComponentEndOverlap(QuestZone)
  (params (OverlappedComponent :type Primitive%20Component%20Object%20Reference) (OtherActor :type Actor%20Object%20Reference) (OtherComp :type Primitive%20Component%20Object%20Reference) (OtherBodyIndex :type Integer))
  (bind _objectives (Variables|Objectives|GetObjectives))
  (bind _canworkonmultipleobjectes (Variables|Objectives|GetCanWorkOnMultipleObjectes))
  (Utilities|FlowControl|DoOnce false) ; enters at Reset
)

(event Custom|StungTarget
  ;[1 1 1] Sting
  (bind _result (Math|Integer|IncrementInt (Variables|Objectives|GetObjectiveCounter))
    (:%20%20
      (if (== _result (Variables|Objectives|GetObjectiveLength))
        (CallFunction|CompleteQuest)
        (else
          (CallFunction|NewObjective))))))

(event Custom|NextObjective
  (switch Utilities|FlowControl|Switch|SwitchonObjectiveTypes (select (Variables|Objectives|GetCanWorkOnMultipleObjectes) (.Type (Utilities|Struct|BreakQuestStruct (stale OnComponentBeginOverlap(QuestZone) _array_element))) (.Type (Utilities|Struct|BreakQuestStruct (Utilities|Array|Get(acopy) (Variables|Objectives|GetObjectives) (Variables|Objectives|GetObjectiveCounter)))))
    (:NewEnumerator2
      ;[1 1 1] Go To Location
      (Utilities|FlowControl|DoOnce false
        (:Completed
          (bind _returnvalue (AddComponent|AddSphereComponent false (Math|Conversions|ToTransform(Vector) (Variables|Location|GetLocation))))
          (Collision|AssignOnComponentBeginOverlap _returnvalue (delegate Custom|OnComponentBeginOverlap_Event_1))
          (Components|Sphere|SetSphereRadius _returnvalue (Variables|Location|GetCompletionOverlapSize) true)
          ;;[1 1 1] Debug
          (Rendering|SetVisibility _returnvalue true false)
          (Development|SetHiddeninGame _returnvalue false false)
          (Development|PrintString "location started")
          (CallFunction|StartObjective)
          (CallFunction|UINewQuest))))
    (:NewEnumerator4
      ;[1 1 1] Sting
      (bind _outactors (Actor|GetAllActorsOfClass "/Game/Blueprints/AI/Character/BP_BackgroundAI_Base.BP_BackgroundAI_Base_C"))
      (Development|PrintString "sting started")
      (if (Variables|AI|GetUseRandomAI)
        (bind _output_get (Variables|AI|SetAITarget (Utilities|Array|Get(acopy) _outactors (Math|Random|RandomInteger (- (Utilities|Array|Length _outactors) 1)))))
        (Default|AssignTarget _output_get)
        (else
          (Default|AssignTarget (Variables|AI|GetAITarget))))
      (EventDispatchers|BindEventtoOnStung (Variables|AI|GetAITarget) (delegate Custom|StungTarget))
      (CallFunction|StartObjective)
      (CallFunction|UINewQuest))
    (:NewEnumerator5
      (Development|PrintString "chase started")
      ;[1 1 1] Chase
      (bind _outactors_2 (Actor|GetAllActorsOfClass "/Game/Blueprints/AI/Character/BP_CivilianChaseable.BP_CivilianChaseable_C"))
      (if (Variables|AI|GetUseRandomAI)
        (Variables|AI|SetAITarget (Utilities|Array|Get(acopy) _outactors_2 (Math|Random|RandomInteger (- (Utilities|Array|Length _outactors_2) 1))))
        (Default|AssignTarget (Utilities|Array|Get(acopy) _outactors_2 (Math|Random|RandomInteger (- (Utilities|Array|Length _outactors_2) 1))))
        (else
          (Default|AssignTarget (Variables|AI|GetAITarget))))
      (bind _returnvalue_2 (AddComponent|AddSphereComponent false (Math|Conversions|ToTransform(Vector) (Variables|Location|GetLocation))))
      (Collision|BindEventtoOnComponentBeginOverlap _returnvalue_2 (delegate Custom|Overlap))
      (Components|Sphere|SetSphereRadius _returnvalue_2 (Variables|Location|GetCompletionOverlapSize) true)
      (Rendering|SetVisibility _returnvalue_2 true false)
      (Development|SetHiddeninGame _returnvalue_2 false false)
      (CallFunction|StartObjective)
      (CallFunction|UINewQuest))
    (:NewEnumerator6
      ;[1 1 1] Fetch
      (Development|PrintString "fetch started")
      (Utilities|FlowControl|DoOnce false
        (:Completed
          (bind _returnvalue_3 (AddComponent|AddSphereComponent false (Math|Conversions|ToTransform(Vector) (Variables|Location|GetLocation))))
          (Collision|AssignOnComponentBeginOverlap _returnvalue_3 (delegate Custom|Begin%20Overlap))
          (Components|Sphere|SetSphereRadius _returnvalue_3 (Variables|Location|GetCompletionOverlapSize) true)
          (CallFunction|StartObjective)
          (CallFunction|UINewQuest))))))

(event Custom|OnComponentBeginOverlap_Event_1
  (params (OverlappedComponent :type Primitive%20Component%20Object%20Reference) (OtherActor :type Actor%20Object%20Reference) (OtherComp :type Primitive%20Component%20Object%20Reference) (OtherBodyIndex :type Integer) (bFromSweep :type Boolean) (SweepResult :type Hit%20Result%20Structure%20%28by%20ref%29))
  ;[1 1 1] Go To Location
  (bind _isbee (Class|ICharacter|GetBeePlayer(Message) OtherActor OtherActor))
  (if _isbee
    (Development|PrintString "Objective complete")
    (EventDispatchers|UnbindallEventsfromOnComponentBeginOverlap (stale OnComponentBeginOverlap(QuestZone) _returnvalue_4))
    (Components|DestroyComponent (stale OnComponentBeginOverlap(QuestZone) _returnvalue_4))
    (bind _result (Math|Integer|IncrementInt (Variables|Objectives|GetObjectiveCounter))
      (:%20%20
        (if (== _result (Variables|Objectives|GetObjectiveLength))
          (CallFunction|CompleteQuest)
          (else
            (CallFunction|NewObjective)))))))

(event Custom|Overlap
  (params (OverlappedComponent :type Primitive%20Component%20Object%20Reference) (OtherActor :type Actor%20Object%20Reference) (OtherComp :type Primitive%20Component%20Object%20Reference) (OtherBodyIndex :type Integer) (bFromSweep :type Boolean) (SweepResult :type Hit%20Result%20Structure%20%28by%20ref%29))
  ;[1 1 1] Chase
  (if (== OtherActor (Variables|AI|GetAITarget))
    (bind _result (Math|Integer|IncrementInt (Variables|Objectives|GetObjectiveCounter))
      (:%20%20
        (if (== _result (Variables|Objectives|GetObjectiveLength))
          (CallFunction|CompleteQuest)
          (EventDispatchers|UnbindallEventsfromOnComponentBeginOverlap (stale OnComponentBeginOverlap(QuestZone) _returnvalue_5))
          (Components|DestroyComponent (stale OnComponentBeginOverlap(QuestZone) _returnvalue_5))
          (else
            (CallFunction|NewObjective)))))))

(event Custom|Begin%20Overlap
  (params (OverlappedComponent :type Primitive%20Component%20Object%20Reference) (OtherActor :type Actor%20Object%20Reference) (OtherComp :type Primitive%20Component%20Object%20Reference) (OtherBodyIndex :type Integer) (bFromSweep :type Boolean) (SweepResult :type Hit%20Result%20Structure%20%28by%20ref%29))
  ;[1 1 1] Fetch
  (for _array_element (Collision|GetOverlappingActors OverlappedComponent "/Game/Blueprints/Grabbables/BP_Grabbable.BP_Grabbable_C" :!class /Script/Engine.PrimitiveComponent)
    (bind _asbp_grabbable (Utilities|Casting|CastToBP_Grabbable _array_element))
    (if (not (== (Utilities|Array|FindItem (Variables|FetchQuest|GetFetchItems) _asbp_grabbable) -1))
      (bind _result (Math|Integer|IncrementInt (Variables|FetchQuest|GetCounter))
        (:%20%20
          (if (== (Utilities|Array|Length (Variables|FetchQuest|GetFetchItems)) _result)
            (bind _result_2 (Math|Integer|IncrementInt (Variables|Objectives|GetObjectiveCounter))
              (:%20%20
                (if (== _result_2 (Variables|Objectives|GetObjectiveLength))
                  (CallFunction|CompleteQuest)
                  (EventDispatchers|UnbindallEventsfromOnComponentBeginOverlap (stale OnComponentBeginOverlap(QuestZone) _returnvalue_6))
                  (Components|DestroyComponent (stale OnComponentBeginOverlap(QuestZone) _returnvalue_6))
                  (Development|SetHiddeninGame (Variables|/Game/Blueprints/QuestSystem/KeyNPCs/NPC_Key_ParentClass.NPC_Key_ParentClass_C|GetThought%20Bubble (Variables|Default|GetQuestGiver)) true false)
                  (else
                    (CallFunction|NewObjective))))))))))
  (Variables|FetchQuest|SetCounter 0))

(event EventBeginPlay
  (CallFunction|StatusChange "NewEnumerator1"))

(fn ConstructionScript
  (Components|Sphere|SetSphereRadius (Variables|Default|GetQuestZone) (Variables|Location|GetQuestActivationRadius) true))

(fn StatusChange
  (params (NewStatus :type QuestStatus%20Enum :default "NewEnumerator0"))
  (Collision|SetCollisionEnabled (Variables|Default|GetQuestZone) (Utilities|Select :Index NewStatus :NewEnumerator0 "NoCollision" :NewEnumerator1 "QueryOnly" :NewEnumerator2 "NoCollision" :NewEnumerator3 "NoCollision" :NewEnumerator4 "NoCollision"))
  (Variables|QuestDetails|SetQuestStatus NewStatus)
  (return))

(fn CompleteQuest
  (Default|CallOnFinishQuest (Variables|Objectives|GetObjectives))
  (CallFunction|StatusChange "NewEnumerator4")
  (Variables|QuestDetails|SetIsComplete true)
  (Development|PrintString "quest completed"))

(fn UINewQuest
  (bind _overlapref (Variables|Objectives|GetOverlapRef))
  (bind _objectivecounter (Variables|Objectives|GetObjectiveCounter))
  (bind _description (Variables|QuestDetails|GetDescription))
  (bind _title (Variables|QuestDetails|GetTitle))
  (bind _returnvalue (> _objectivecounter 0))
  (switch Utilities|FlowControl|Switch|SwitchonObjectiveTypes (.Type (Utilities|Struct|BreakQuestStruct (Utilities|Array|Get(acopy) (Variables|Objectives|GetObjectives) _objectivecounter)))
    (:NewEnumerator2
      (Class|ICharacter|NewQuestSet(Message) _overlapref _title _description (Variables|Location|GetLocation) _returnvalue :!label _label))
    (:NewEnumerator4
      (Class|ICharacter|NewQuestSet(Message) _overlapref _title _description (Transformation|GetActorLocation (Variables|AI|GetAITarget)) _returnvalue))
    (:NewEnumerator5
      (goto _label))
    (:NewEnumerator6
      (Class|ICharacter|NewQuestSet(Message) _overlapref _title _description "0, 0, 0" _returnvalue))))

(fn NewObjective
  (bind _objectives (Variables|Objectives|GetObjectives))
  (bind _objectivecounter (Variables|Objectives|GetObjectiveCounter))
  (bind _returnvalue (- _objectivecounter 1))
  (bind _output (Utilities|Array|Get(acopy) _objectives _returnvalue))
  (Utilities|Struct|SetmembersinQuestStruct _output true)
  (Default|CallOnObjectiveCompleted _output)
  (CallFunction|NextObjective))

(fn StartObjective
  (bind _objectives (Variables|Objectives|GetObjectives))
  (Default|CallOnStartNewQuest (select (Variables|Objectives|GetCanWorkOnMultipleObjectes) _objectives (Utilities|Array|MakeArray (Utilities|Array|Get(acopy) _objectives (Variables|Objectives|GetObjectiveCounter))))))