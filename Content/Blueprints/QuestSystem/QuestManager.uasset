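; Quest manager that tracks active objectives and keeps the character's to-do list widget in sync.
; On Init it binds to the start, finish and objective-completed events of every BP_QuestActor in the world.
; New objectives are stored, with non-achievement texts added uniquely to a description list that drives the widget.
; Completion marks non-achievement entries by their index in that list; finishing a quest also removes them from the active objectives.
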(event Custom|Init
  (params (CharacterRef :type Bee%20Character%20BP%20Object%20Reference))
  (bind _outactors (Actor|GetAllActorsOfClass "/Game/Blueprints/QuestSystem/BP_QuestActor.BP_QuestActor_C"))
  (for _array_element _outactors
    (EventDispatchers|BindEventtoOnStartNewQuest _array_element (EventDispatchers|CreateEvent :!event Custom|StartNewQuest))
    (EventDispatchers|BindEventtoOnFinishQuest _array_element (EventDispatchers|CreateEvent :!event Custom|CompleteQuest))
    (EventDispatchers|BindEventtoOnObjectiveCompleted _array_element (EventDispatchers|CreateEvent :!event Custom|ObjectiveComplete))))

(event Custom|StartNewQuest
  (params (NewObjectives :type Array%20of%20Quest%20Struct%20Structures))
  (bind _objectivedescriptions (Variables|Default|GetObjectiveDescriptions))
  (for _array_element NewObjectives
    (Utilities|Array|Add (Variables|Default|GetCurrentObjectives) _array_element)
    (if (not (.Achievement? (Utilities|Struct|BreakQuestStruct _array_element)))
      (if (not (Utilities|Array|ContainsItem (Variables|Default|GetObjectiveDescriptions) (.ObjectiveText (Utilities|Struct|BreakQuestStruct _array_element))))
        (Utilities|Array|AddUnique _objectivedescriptions (.ObjectiveText (Utilities|Struct|BreakQuestStruct _array_element))))))
  (Default|UpdateObjectiveList (Variables|/Game/Blueprints/Character/BeeCharacter_BP.BeeCharacter_BP_C|GetWigToDoListRef (stale Custom|Init CharacterRef)) _objectivedescriptions))

(event Custom|CompleteQuest
  (params (Completed%20Objectives :type Array%20of%20Quest%20Struct%20Structures))
  (bind _currentobjectives (Variables|Default|GetCurrentObjectives))
  (for _array_element Completed%20Objectives
    (if (not (.Achievement? (Utilities|Struct|BreakQuestStruct _array_element)))
      (if (Utilities|Array|ContainsItem _currentobjectives _array_element)
        (Utilities|Array|RemoveItem _currentobjectives _array_element)
        (Default|CompletedObjective (Variables|/Game/Blueprints/Character/BeeCharacter_BP.BeeCharacter_BP_C|GetWigToDoListRef (stale Custom|Init CharacterRef)) (Utilities|Array|FindItem (Variables|Default|GetObjectiveDescriptions) (.ObjectiveText (Utilities|Struct|BreakQuestStruct _array_element))))))))

(event Custom|ObjectiveComplete
  (params (Objective :type Quest%20Struct%20Structure))
  (bind (_objectivetext _type _iscomplete _achievement_) (Utilities|Struct|BreakQuestStruct Objective))
  (if (not _achievement_)
    (Default|CompletedObjective (Variables|/Game/Blueprints/Character/BeeCharacter_BP.BeeCharacter_BP_C|GetWigToDoListRef (stale Custom|Init CharacterRef)) (Utilities|Array|FindItem (Variables|Default|GetObjectiveDescriptions) _objectivetext))))