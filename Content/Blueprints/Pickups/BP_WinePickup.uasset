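; Wine pickup that gives the character a timed wine effect and toggles a matching message through its controller.
; Pickup shows the message and passes itself and the duration to the character's GetWinePickUp.
; Disable turns off sphere collision, removes the mesh and starts a timer, keeping the actor alive until Destroy fires.
; Destroy calls Undo to hide the message, then destroys the actor.
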(event Custom|Destroy
  (CallFunction|Undo)
  (Actor|DestroyActor))

(event EventDisable
  (bind _returnvalue (Utilities|Time|SetTimerbyEvent (delegate Custom|Destroy) (Variables|Default|GetTime)))
  (Variables|Default|SetWinePUHandle _returnvalue)
  (Collision|SetCollisionEnabled (Variables|Default|GetSphere) "NoCollision")
  (Components|DestroyComponent (Variables|Default|GetStaticMesh)))

(fn ConstructionScript
  (|CallParentFunction))

(fn Pickup
  (bind _character (Variables|Default|GetCharacter))
  (Class|IControls|WinePickup(Message) (Pawn|GetController _character) true)
  (Default|GetWinePickUp _character self (Variables|Default|GetTime))
  (return true))

(fn Undo
  (Class|IControls|WinePickup(Message) (Pawn|GetController (Variables|Default|GetCharacter)) false)
  (return))