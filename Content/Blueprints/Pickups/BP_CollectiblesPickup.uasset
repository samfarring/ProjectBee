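; BP_CollectiblesPickup is a pickup Blueprint that records a numbered collectible on the character.
; Its Pickup override adds the collectible number to the character's CollectiblesCollected map with a "Collectible #N" text label and reports success.
; The Disable event destroys the actor, and the construction script only runs the parent's setup.
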(event EventDisable
  (Actor|DestroyActor))

(fn ConstructionScript
  (|CallParentFunction))

(fn Pickup
  (bind _collectiblenumber (Variables|Default|GetCollectibleNumber))
  (Utilities|Map|Add (Variables|/Game/Blueprints/Character/BeeCharacter_BP.BeeCharacter_BP_C|GetCollectiblesCollected (Variables|Default|GetCharacter)) _collectiblenumber (Utilities|Text|ToText(String) (Utilities|String|Append "Collectible #" (Utilities|String|ToString(Integer) _collectiblenumber))))
  (return true))