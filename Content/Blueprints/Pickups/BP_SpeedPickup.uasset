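; Speed pickup actor that temporarily raises the character's FloatingPawnMovement max speed to a sprint value.
; Pickup applies the boost and passes the pickup to the character through GetSpeedPickUp.
; Disable stores a timer handle, turns off sphere collision and destroys the mesh, keeping the actor alive for the boost duration.
; When the timer fires, Undo restores the starting speed and the actor destroys itself.
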(event Custom|Destroy
  (CallFunction|Undo)
  (Actor|DestroyActor))

(event EventBeginPlay)

(event Collision|EventActorBeginOverlap
  (params (OtherActor :type Actor%20Object%20Reference)))

(event EventTick
  (params (DeltaSeconds :type Float%20%28single-precision%29)))

(event EventDisable
  (bind _returnvalue (Utilities|Time|SetTimerbyEvent (delegate Custom|Destroy) (Variables|Default|GetTime)))
  (Variables|Default|SetSpeedPUHandle _returnvalue)
  (Collision|SetCollisionEnabled (Variables|Default|GetSphere) "NoCollision")
  (Components|DestroyComponent (Variables|Default|GetStaticMesh)))

(fn ConstructionScript
  (|CallParentFunction))

(fn Pickup
  (bind _character (Variables|Default|GetCharacter))
  (Variables|/Script/Engine.FloatingPawnMovement|SetMaxSpeed (Variables|/Game/Blueprints/Character/BeeCharacter_BP.BeeCharacter_BP_C|GetFloatingPawnMovement _character) (Variables|Default|GetSprintSpeed))
  (Default|GetSpeedPickUp _character self)
  (return false))

(fn Undo
  (Variables|/Script/Engine.FloatingPawnMovement|SetMaxSpeed (Variables|/Game/Blueprints/Character/BeeCharacter_BP.BeeCharacter_BP_C|GetFloatingPawnMovement (Variables|Default|GetCharacter)) (Variables|Default|GetStartSpeed))
  (return))