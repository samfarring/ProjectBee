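; AI controller for the beekeeper boss that schedules its Beyblade attack and announces the boss fight to the game mode.
; A looping timer, started on Activated, periodically rolls a weighted chance to set the BeybladeActive blackboard key, pause the timer and trigger BossFightTrigger on the player bee.
; Attack end clears the key, notifies the controlled pawn and restarts the timer.
; SetBossFight makes an immediate attack roll.
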(event Custom|ResetBeybladeAttack
  (bind _returnvalue (Utilities|Time|SetTimerbyEvent (delegate Custom|StartBeybladeAttack) 2e+01 true)))

(event Custom|Activated
  (bind _returnvalue (Utilities|Time|SetTimerbyEvent (delegate Custom|StartBeybladeAttack) 2e+01 true)))

(event Custom|StartBeybladeAttack
  (bind _self self)
  (bind _returnvalue (AI|GetBlackboard _self))
  (if (Math|Random|RandomBoolwithWeight 0.35)
    (Utilities|IsValid _returnvalue
      (:Is%20Valid
        (AI|Components|Blackboard|SetValueasBool _returnvalue (Variables|Default|GetBeybladeActive) true)
        (Utilities|Time|ClearandInvalidateTimerbyHandle (Variables|Default|GetResetStateHandle))
        (Utilities|Time|ClearandInvalidateTimerbyHandle (stale Custom|ResetBeybladeAttack _returnvalue))
        (bind _asbee_character_bp (Utilities|Casting|CastToBeeCharacter_BP (Game|Player|GetPlayerPawn 0)))
        (Default|BossFightTrigger _asbee_character_bp)))))

(event EventBeginPlay
  (|CallParentFunction))

(event EventSetBossFight
  (CallFunction|StartBeybladeAttack)
  (Class|IGameMode|BossFightStarted(Message) (Game|GetGameMode)))

(event EventBeybladeAttackEnd
  (bind _self self)
  (bind _returnvalue (AI|GetBlackboard _self))
  (Utilities|IsValid _returnvalue
    (:Is%20Valid
      (AI|Components|Blackboard|SetValueasBool _returnvalue (Variables|Default|GetBeybladeActive) false)
      (Class|IAI|BeybladeAttackEnd(Message) (Pawn|GetControlledPawn))
      (CallFunction|ResetBeybladeAttack))))

(fn ConstructionScript
  (|CallParentFunction))