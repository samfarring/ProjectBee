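; AI controller for background characters that patrol zones and can react to the bee character.
; Init starts looping timers for AI ticks, random patrol zone picks and chance-based activities, then runs a behavior tree.
; Perceiving the bee switches state to flee, or to an aggressive state for aggressive pawns, with a timed reset.
; Getters expose state, target, zone and church marker; several others return fixed stub values.
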(event OnTargetPerceptionUpdated(AIPerception)
  (params (Actor :type Actor%20Object%20Reference) (Stimulus :type AI%20Stimulus%20Structure))
  ;[1 1 1] Perception
  (bind _info (Class|AIPerceptionComponent|GetActorsPerception (Variables|Default|GetAIPerception) Actor))
  (if (and (== (Utilities|GetClass (.Target (Utilities|Struct|BreakActorPerceptionBlueprintInfo _info))) "/Game/Blueprints/Character/BeeCharacter_BP.BeeCharacter_BP_C") (Variables|States|GetWillReactToBee))
    (Variables|Perception|SetPerceptionTarget (.Target (Utilities|Struct|BreakActorPerceptionBlueprintInfo _info)))
    (if (Variables|States|GetIsAggressive)
      (Variables|States|SetStates "NewEnumerator3")
      (else
        (Variables|States|SetStates "NewEnumerator2")))
    (CallFunction|ResetStateTimer (.ExpirationAge (Utilities|Struct|BreakAIStimulus (Utilities|Array|Get(acopy) (.LastSensedStimuli (Utilities|Struct|BreakActorPerceptionBlueprintInfo _info))))))))

(event Custom|PatrolChange
  ;[1 1 1] Patrol
  (Variables|Patrol|SetDesiredLocation (Utilities|Select :Index (Math|Random|RandomInteger 7) :Option%200 "NewEnumerator2" :Option%201 "NewEnumerator3" :Option%202 "NewEnumerator4" :Option%203 "NewEnumerator5" :Option%204 "NewEnumerator6" :Option%205 "NewEnumerator7" :Option%206 "NewEnumerator8"))
  (for _array_element (Variables|Patrol|GetPatrolZones)
    (Utilities|IsValid _array_element
      (:Is%20Valid
        (if (Utilities|Enum|Equal(Enum) (Variables|/Game/Blueprints/AI/BP_PatrolZone.BP_PatrolZone_C|GetLocation _array_element) (Variables|Patrol|GetDesiredLocation))
          (Variables|Patrol|SetSetPatrolZone _array_element))))))

(event Custom|ActivityTimer
  (if (Variables|Default|GetCanDoActivities)
    (bind _returnvalue (Utilities|Time|SetTimerbyEvent (delegate Custom|StartActivity) (Variables|Default|GetActivityTime) true))))

(event Custom|AI_Tick
  (bind _patroltimerhandle (Variables|Patrol|GetPatrolTimerHandle))
  ;[1 1 1] Tick
  (Class|IAI|SetStateText(Message) (Pawn|GetControlledPawn) (Variables|States|GetStates))
  (if (Utilities|Enum|Equal(Enum) (Variables|States|GetStates) "NewEnumerator1")
    (if (Variables|Patrol|GetPatrolTimerPaused)
      (Utilities|Time|UnpauseTimerbyHandle _patroltimerhandle)
      (Variables|Patrol|SetPatrolTimerPaused false))
    (elif (Variables|Patrol|GetPatrolTimerPaused)
      (Utilities|Time|PauseTimerbyHandle _patroltimerhandle)
      (Variables|Patrol|SetPatrolTimerPaused true))))

(event Custom|ResetState
  ;[1 1 1] Reset
  (Variables|States|SetStates "NewEnumerator1"))

(event Custom|StartActivity
  (if (and (Math|Random|RandomBoolwithWeight (Variables|Default|GetActivityChance)) (Variables|Default|GetCanBeActive))
    (Variables|Default|SetActivityActive true)
    (Utilities|Time|ClearandInvalidateTimerbyHandle (stale Custom|ActivityTimer _returnvalue))))

(event Custom|ResetActivity
  (Variables|Default|SetActivityActive false)
  (CallFunction|ActivityTimer))

(event EventIsCowering
  (params (IsCowering :type Boolean))
  ;[1 1 1] Cower Anim
  (Variables|States|SetIsCower IsCowering))

(event EventInit
  (params (ControlledPawn :type BP%20Background%20AI%20Base%20Object%20Reference))
  ;[1 1 1] Init
  (Variables|States|SetIsAggressive (Variables|/Game/Blueprints/AI/Character/BP_BackgroundAI_Base.BP_BackgroundAI_Base_C|GetIsAggressive ControlledPawn))
  (Variables|States|SetWillReactToBee (Variables|/Game/Blueprints/AI/Character/BP_BackgroundAI_Base.BP_BackgroundAI_Base_C|GetWillReactToBee ControlledPawn))
  (Utilities|Time|SetTimerbyEvent (EventDispatchers|CreateEvent :!event Custom|AI_Tick) (Variables|Tick|GetAITickRate) true)
  (CallFunction|PatrolZoneInit)
  (CallFunction|PatrolChange)
  (CallFunction|LocationMarkerInit)
  (bind _returnvalue (Utilities|Time|SetTimerbyEvent (EventDispatchers|CreateEvent :!event Custom|PatrolChange) (Variables|Patrol|GetPatrolTimer) true))
  (Variables|Patrol|SetPatrolTimerHandle _returnvalue)
  (CallFunction|InitVariables)
  (CallFunction|ActivityTimer)
  (AI|RunBehaviorTree (Variables|Default|GetBTTree)))

(event EventSetFlee
  ;[1 1 1] Set Flee
  (Variables|States|SetStates "NewEnumerator2")
  (CallFunction|ResetStateTimer (Variables|Timer|GetResetTime)))

(event EventDeleteCon
  (Utilities|FlowControl|Delay 1.0)
  (Actor|DestroyActor))

(fn ConstructionScript)

(fn InitVariables
  (Variables|States|SetStates "NewEnumerator1"))

(fn PatrolZoneInit
  (bind _outactors (Actor|GetAllActorsOfClass "/Game/Blueprints/AI/BP_PatrolZone.BP_PatrolZone_C"))
  (Variables|Patrol|SetPatrolZones _outactors))

(fn ResetStateTimer
  (params (Time :type Float%20%28single-precision%29))
  (Utilities|Time|SetTimerbyEvent (EventDispatchers|CreateEvent :!event Custom|ResetState) (Variables|Timer|GetResetTime)))

(fn LocationMarkerInit
  (bind _outactors (Actor|GetAllActorsOfClass "/Game/Blueprints/AI/BP_LocationMarker.BP_LocationMarker_C"))
  (for _array_element _outactors
    (if (Utilities|Enum|Equal(Enum) (Variables|/Game/Blueprints/AI/BP_LocationMarker.BP_LocationMarker_C|GetLocation _array_element) "NewEnumerator2")
      (Variables|Default|SetChurchMarker _array_element))))

(fn CanPatrol
  (return false))

(fn GetActivity
  (return "NewEnumerator0"))

(fn GetActivityActive
  (return (Variables|Default|GetActivityActive)))

(fn GetBaseLocation
  (return "NewEnumerator0"))

(fn GetChurchMarker
  (return (Variables|Default|GetChurchMarker)))

(fn GetGender
  (return false))

(fn GetIsChaseable
  (return false))

(fn GetPatrolZone
  (bind _setpatrolzone (Variables|Patrol|GetSetPatrolZone))
  (Utilities|IsValid _setpatrolzone
    (:Is%20Valid
      (return (Variables|Patrol|GetDesiredLocation) (Transformation|GetActorLocation _setpatrolzone)))))

(fn GetPerceptionTarget
  (return (Variables|Perception|GetPerceptionTarget)))

(fn GetStateChange
  (return (Variables|States|GetStates)))