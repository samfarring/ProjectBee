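; AI controller for the BeeKeeper boss that triggers its Beyblade attack and plays random voice lines.
; On BeginPlay it starts a looping timer and, after a delay, sets the BeybladeActive blackboard flag to enable the attack.
; A dialogue event waits a short random delay, then plays a random-lines sound cue at the controlled pawn's location.
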(event Custom|RandomDialogue
  (Utilities|FlowControl|Delay (Math|Random|RandomFloatinRange 0.0 5.0))
  (Audio|PlaySoundatLocation "/Game/Audio/Dialogue/Beekeeper/BeeKeeperRandomLinesCue.BeeKeeperRandomLinesCue" (Transformation|GetActorLocation (Pawn|GetControlledPawn)) "0, 0, 0" 1.0 1.0 0.0 0 0 0))

(event Custom|StartBeybladeAttack
  (bind _self self)
  (bind _returnvalue (AI|GetBlackboard _self))
  (Utilities|IsValid _returnvalue
    (:Is%20Valid
      (AI|Components|Blackboard|SetValueasBool _returnvalue (Variables|Default|GetBeybladeActive) true))))

(event EventBeginPlay
  (|CallParentFunction)
  (Utilities|Time|SetTimerbyEvent (EventDispatchers|CreateEvent :!event Custom|RandomDialogue) 1e+01 true)
  (Utilities|FlowControl|Delay 1e+01)
  (CallFunction|StartBeybladeAttack))

(fn ConstructionScript
  (|CallParentFunction))