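; BP_LocationMarker is an AI-related actor that marks a named place in the level, such as the Van, Church, Park or Pub.
; Its construction script maps the Location value to a display name and writes it to a text render component, leaving it blank when unset.
; The event graph holds only disabled default events, so the marker has no runtime logic of its own.
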(event EventBeginPlay)

(event Collision|EventActorBeginOverlap
  (params (OtherActor :type Actor%20Object%20Reference)))

(event EventTick
  (params (DeltaSeconds :type Float%20%28single-precision%29)))

(fn ConstructionScript
  (Rendering|Components|TextRender|SetText (Variables|Default|GetTextRender) (Utilities|Select :Index (Variables|Default|GetLocation) :NewEnumerator0 "" :NewEnumerator1 (Utilities|Text|MakeLiteralText "Van") :NewEnumerator2 (Utilities|Text|MakeLiteralText "Church") :NewEnumerator3 (Utilities|Text|MakeLiteralText "Park") :NewEnumerator4 (Utilities|Text|MakeLiteralText "Farmhouse") :NewEnumerator5 (Utilities|Text|MakeLiteralText "School") :NewEnumerator6 (Utilities|Text|MakeLiteralText "Cafe") :NewEnumerator7 (Utilities|Text|MakeLiteralText "Pub") :NewEnumerator8 (Utilities|Text|MakeLiteralText "Market"))))