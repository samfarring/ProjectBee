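; Beekeeper AI character that kills bee players with a swatter attached to its right hand at BeginPlay.
; Attack plays a swat animation, then sphere-traces forward and upward for pawns after a short delay.
; A separate Beyblade spin attack re-sockets the swatter and repeats a radius trace on a looping timer until ended.
; Bee hits get physics impulses and random spin, lose input, then take damage after KillDelay.
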(event Custom|BBAttack
  (bind _returnvalue (Transformation|GetActorLocation))
  (bind _self self)
  (bind _minimpulse (Variables|Combat|GetMinImpulse))
  (bind _maximpulse (Variables|Default|GetMaxImpulse))
  (bind (_outhit _returnvalue_2) (Collision|SphereTraceForObjects _returnvalue (* (+ _returnvalue (Transformation|GetActorForwardVector)) 1.0) (Variables|Default|GetBeyBladeRadius) (Utilities|Array|MakeArray "ObjectTypeQuery3") false 0 "None" true "(R=1.000000,G=0.000000,B=0.000000,A=1.000000)" "(R=0.000000,G=1.000000,B=0.000000,A=1.000000)" 0.2))
  (bind _isbee (Class|ICharacter|GetBeePlayer(Message) (.HitActor (Collision|BreakHitResult _outhit)) (.HitActor (Collision|BreakHitResult _outhit))))
  (if (and _returnvalue_2 _isbee)
    (Physics|AddImpulseatLocation (.HitComponent (Collision|BreakHitResult _outhit)) "10000.000000,10000.000000,10000.000000" (.Location (Collision|BreakHitResult _outhit)) "None")
    (Class|PrimitiveComponent|AddAngularImpulseinDegrees (.HitComponent (Collision|BreakHitResult _outhit)) (Math|Vector|MakeVector (Math|Random|RandomFloatinRange _minimpulse _maximpulse) (Math|Random|RandomFloatinRange _minimpulse _maximpulse) (Math|Random|RandomFloatinRange _minimpulse _maximpulse)) "None" true)
    (bind _playerref (Class|ICharacter|GetBeePlayer(Message) (.HitActor (Collision|BreakHitResult _outhit)) (.HitActor (Collision|BreakHitResult _outhit))))
    (Default|DisableInputs _playerref)
    (Utilities|FlowControl|Delay (Variables|Default|GetKillDelay))
    (Game|Damage|ApplyDamage _playerref 1e+02 (AI|GetAIController _self) _self)))

(event Custom|OnAttackStart)

(event EventBeginPlay
  (bind _mesh (Variables|Character|GetMesh))
  (|CallParentFunction)
  (bind _returnvalue (AddComponent|AddStaticMeshComponent false (Transformation|GetSocketTransform _mesh (Class|SkinnedMeshComponent|GetSocketBoneName _mesh "BeekeeperRArmRHandSocket") "RTS_Actor")))
  (Variables|Default|SetSwatterMesh _returnvalue)
  (Components|StaticMesh|SetStaticMesh _returnvalue "/Game/ArtAssets/Animations/Beekeeper/Skeleton/Swatter/a_swatter.a_swatter")
  (Transformation|AttachComponentToComponent _returnvalue (Variables|Character|GetMesh) "BeekeeperRArmRHandSocket" "KeepRelative" "KeepRelative" "KeepRelative" true))

(event EventAttack
  (params (Attacker :type Actor%20Object%20Reference))
  (bind _array (Utilities|Array|MakeArray "ObjectTypeQuery3"))
  (bind _self self)
  (bind _minimpulse (Variables|Combat|GetMinImpulse))
  (bind _maximpulse (Variables|Default|GetMaxImpulse))
  (bind _mesh (Variables|Character|GetMesh))
  (bind _attackstart (Variables|Default|GetAttackStart))
  (bind _returnvalue (Transformation|GetWorldLocation _attackstart))
  (Utilities|FlowControl|Sequence
    (:then_0
      (Components|Animation|SetAnimationMode _mesh "AnimationSingleNode")
      (Components|Animation|PlayAnimation _mesh "/Game/ArtAssets/Animations/Beekeeper/Sequences/BeeKeeper_SwatEngineReady.BeeKeeper_SwatEngineReady" false))
    (:then_1
      (CallFunction|OnAttackStart)
      (Utilities|FlowControl|Delay 0.6)
      (bind (_outhit _returnvalue_2) (Collision|SphereTraceForObjects _returnvalue (+ _returnvalue (* (Math|Vector|GetForwardVector _attackstart) (Variables|Default|GetStingRadius))) 1e+02 _array false 0 "None" true "(R=1.000000,G=0.000000,B=0.000000,A=1.000000)" "(R=0.000000,G=1.000000,B=0.000000,A=1.000000)" 2.0))
      (Variables|Default|SetHitActor (.HitActor (Collision|BreakHitResult _outhit)))
      (Variables|Default|SetHitLoc (.Location (Collision|BreakHitResult _outhit)))
      (bind (_outhit_2 _returnvalue_3) (Collision|SphereTraceForObjects (Transformation|GetWorldLocation (Variables|Default|GetAttackUp)) (Transformation|GetWorldLocation (Variables|Default|GetAttackUpEnd)) 8e+01 _array false 0 "None" true "(R=1.000000,G=0.000000,B=0.000000,A=1.000000)" "(R=0.000000,G=1.000000,B=0.000000,A=1.000000)" 2.0))
      (Variables|Default|SetHitActor (.HitActor (Collision|BreakHitResult _outhit_2)))
      (Variables|Default|SetHitLoc (.Location (Collision|BreakHitResult _outhit_2)))
      (bind (_isbee _conref _playerref) (Class|ICharacter|GetBeePlayer(Message) (Variables|Default|GetHitActor) (Variables|Default|GetHitActor)))
      (Utilities|FlowControl|Sequence
        (:then_0
          (Utilities|FlowControl|Delay 0.8)
          (Components|Animation|SetAnimationMode (Variables|Character|GetMesh) "AnimationBlueprint"))
        (:then_1
          (if (and _isbee (or _returnvalue_2 _returnvalue_3))
            (Physics|AddRadialImpulse (.HitComponent (Collision|BreakHitResult _outhit_2)) (Variables|Default|GetHitLoc) 2e+02 1e+03 "RIF_Constant" true)
            (Class|PrimitiveComponent|AddAngularImpulseinDegrees (.HitComponent (Collision|BreakHitResult _outhit_2)) (Math|Vector|MakeVector (Math|Random|RandomFloatinRange _minimpulse _maximpulse) (Math|Random|RandomFloatinRange _minimpulse _maximpulse) (Math|Random|RandomFloatinRange _minimpulse _maximpulse)) "None" true)
            (Default|DisableInputs _playerref)
            (Utilities|FlowControl|Delay (Variables|Default|GetKillDelay))
            (Game|Damage|ApplyDamage _playerref 1e+02 (AI|GetAIController _self) _self)))))))

(event EventBeybladeAttack
  (Variables|Default|SetIsBeybladeAttack true)
  (bind _returnvalue (Utilities|Time|SetTimerbyEvent (delegate Custom|BBAttack) 0.1 true))
  (Variables|Default|SetBeybladeTimerHandle _returnvalue)
  (Transformation|AttachComponentToComponent (Variables|Default|GetSwatterMesh) (Variables|Character|GetMesh) "BeekeeperRArmRHandSocket_Beyblade" "KeepRelative" "KeepRelative" "KeepRelative" true))

(event EventBeybladeAttackEnd
  (Utilities|Time|ClearandInvalidateTimerbyHandle (Variables|Default|GetBeybladeTimerHandle)))

(fn ConstructionScript
  (bind _mesh (Variables|Character|GetMesh))
  (|CallParentFunction)
  (Class|SkinnedMeshComponent|SetSkeletalMesh _mesh "/Game/ArtAssets/Animations/Beekeeper/Skeleton/Skeleton/Beekeeper_Mesh.Beekeeper_Mesh" true)
  (Components|SkeletalMesh|SetAnimInstanceClass _mesh "/Game/ArtAssets/Animations/Beekeeper/AP_BeeKeeper.AP_BeeKeeper_C"))

(fn OnAttack)