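; BP_BeeKeeperBoss is the beekeeper boss character, handling its voice lines, boss-fight start and death.
; A quest event sends the boss-fight message to its AI controller, while timers, aggression changes, stings and attacks drive audio gated partly by a talking flag.
; Hitting a BP_Spire kills it, playing the death line, ending the Beyblade attack, notifying the quest and starting the end-game cutscene.
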(event OnComponentHit(CapsuleComponent)
  (params (HitComponent :type Primitive%20Component%20Object%20Reference) (OtherActor :type Actor%20Object%20Reference) (OtherComp :type Primitive%20Component%20Object%20Reference) (NormalImpulse :type Vector :default "0, 0, 0") (Hit :type Hit%20Result%20Structure%20%28by%20ref%29))
  (if (== (Utilities|GetClass OtherActor) "/Game/Blueprints/Puzzles/BP_Spire.BP_Spire_C")
    (CallFunction|Death)))

(event OnAudioFinished(RandomDialogue)
  (Variables|Default|SetIsTalking_0 false))

(event OnAudioFinished(BeeKeeperlaugh_Cue)
  (Variables|Default|SetIsTalking_0 false))

(event Custom|BreathingTimer
  (Class|AudioComponent|SetPaused (Variables|Default|GetBreathingCue) (or (Variables|Default|GetIsTalking_0) (Variables|Default|GetIsDead))))

(event Custom|DialoguerTimer
  (if (and (Math|Random|RandomBoolwithWeight 0.75) (not (Variables|Default|GetIsTalking_0)))
    (Audio|Components|Audio|SetSound (Variables|Default|GetRandomDialogue) "/Game/Audio/Dialogue/BeekeeperBoss/RandomLines/BeeKeeperRandomLinesCue.BeeKeeperRandomLinesCue")
    (Audio|Components|Audio|Play (Variables|Default|GetRandomDialogue) 0.0)
    (Variables|Default|SetIsTalking_0 true)))

(event Custom|Death
  (bind _randomdialogue (Variables|Default|GetRandomDialogue))
  (Audio|Components|Audio|SetSound _randomdialogue "/Game/Audio/Dialogue/BeekeeperBoss/Death/BeeKeeperDeath_Cue.BeeKeeperDeath_Cue")
  (Class|AudioComponent|SetPaused (Variables|Default|GetBeeKeeperlaugh_Cue) true)
  (Audio|Components|Audio|Play _randomdialogue 0.0)
  (Variables|Default|SetIsDead true)
  (Class|IAI|BeybladeAttackEnd(Message) (AI|GetAIController self))
  (CallFunction|BeeKeeperDeath)
  (Default|EventFiringReturn (stale EventEventFiring Quest))
  (bind _outactors (Actor|GetAllActorsOfClass "/Game/Blueprints/QuestSystem/KeyNPCs/BP_EndGameCutscene.BP_EndGameCutscene_C"))
  (Default|StartSequence (Utilities|Array|Get(acopy) _outactors)))

(event Custom|AggressionSet
  (bind _randomdialogue (Variables|Default|GetRandomDialogue))
  (Utilities|FlowControl|DoOnce false
    (:Completed
      (Audio|Components|Audio|SetSound _randomdialogue "/Game/Audio/Dialogue/BeekeeperBoss/Spotted/BeeKeeperSpotted_Cue.BeeKeeperSpotted_Cue")
      (Variables|Default|SetIsTalking_0 true)
      (Audio|Components|Audio|Play _randomdialogue 0.0))))

(event Custom|NormalSet
  (bind _randomdialogue (Variables|Default|GetRandomDialogue))
  (Utilities|FlowControl|DoOnce false) ; enters at Reset
)

(event EventBeginPlay
  (|CallParentFunction)
  (Utilities|Time|SetTimerbyEvent (delegate Custom|BreathingTimer) 1.0 true)
  (Utilities|Time|SetTimerbyEvent (EventDispatchers|CreateEvent :!event Custom|DialoguerTimer) (Variables|Default|GetDialogueTime) true)
  (EventDispatchers|BindEventtoOnAggressive (EventDispatchers|CreateEvent :!event Custom|AggressionSet))
  (EventDispatchers|BindEventtoOnNormal (EventDispatchers|CreateEvent :!event Custom|NormalSet))
  (Transformation|AttachComponentToComponent (Variables|Default|GetBrassHat) (Variables|Character|GetMesh) "BeekeeperHeadSocket" "KeepRelative" "KeepRelative" "KeepRelative" true))

(event EventGotStung
  (bind _randomdialogue (Variables|Default|GetRandomDialogue))
  (Audio|Components|Audio|SetSound _randomdialogue "/Game/Audio/Dialogue/BeekeeperBoss/Stung/BeeKeeperStungCue.BeeKeeperStungCue")
  (Audio|Components|Audio|Play _randomdialogue 0.0)
  (Variables|Default|SetIsTalking_0 true))

(event EventOnAttackStart
  (if (not (Variables|Default|GetIsTalking_0))
    (Audio|Components|Audio|Play (Variables|Default|GetBeeKeeperlaugh_Cue) 0.0)
    (Variables|Default|SetIsTalking_0 true)))

(event EventEventFiring
  (params (Quest :type BP%20Quest%20Actor%20Object%20Reference) (Bee :type Bee%20Character%20BP%20Object%20Reference))
  (Class|IAI|SetBossFight(Message) (AI|GetAIController self)))

(event EventTick
  (params (DeltaSeconds :type Float%20%28single-precision%29))
  (|CallParentFunction DeltaSeconds))

(fn ConstructionScript
  (Class|SkinnedMeshComponent|SetSkeletalMesh (Variables|Character|GetMesh) "/Game/ArtAssets/Animations/Beekeeper/Skeleton/Skeleton/Beekeeper_Mesh.Beekeeper_Mesh" true))