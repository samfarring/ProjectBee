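; Civilian AI character that plays a scripted, one-shot fall into a pond, ending in a drowning loop.
; PlayPondSequence spawns smoke, switches the mesh to single-node animation, turns the actor and plays the fall animation.
; The Fall timeline lerps X/Y from the current location toward hardcoded world coordinates.
; On finish it loops the drowning animation, teleports the capsule to a fixed transform and unpossesses the AI controller.
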(event EventBeginPlay
  (|CallParentFunction) ; This node is disabled and will not be called.\nDrag off pins to build functionality.
)

(event Collision|EventActorBeginOverlap
  (params (OtherActor :type Actor%20Object%20Reference))
  (|CallParentFunction OtherActor) ; This node is disabled and will not be called.\nDrag off pins to build functionality.
)

(event EventTick
  (params (DeltaSeconds :type Float%20%28single-precision%29))
  (|CallParentFunction DeltaSeconds) ; This node is disabled and will not be called.\nDrag off pins to build functionality.
)

(event EventPlayPondSequence
  (bind _returnvalue (Transformation|GetActorLocation))
  (bind _mesh (Variables|Character|GetMesh))
  (Utilities|FlowControl|DoOnce false
    (:Completed
      (Effects|SpawnEmitteratLocation "/Game/Blueprints/Particles/SmokeParticle.SmokeParticle" (Transformation|GetActorLocation) "0, 0, 0" "3.000000,3.000000,3.000000")
      (Components|Animation|SetAnimationMode _mesh "AnimationSingleNode")
      (Components|Animation|PlayAnimation _mesh "/Game/ArtAssets/Animations/Man/Sequences/MaleFallingForwardExportMaleFallingForward.MaleFallingForwardExportMaleFallingForward" false)
      (Transformation|SetActorRotation "0,-90.000000, 0")
      (bind _fall (Timeline|Fall Play)
        (:Update
          (Transformation|SetActorLocation (Math|Vector|MakeVector (Math|Float|Lerp (.x _returnvalue) 3686.0 _fall) (Math|Float|Lerp (.y _returnvalue) 6.25e+03 _fall) (.z _returnvalue)) false false))
        (:Finished
          (Components|Animation|PlayAnimation _mesh "/Game/ArtAssets/Animations/Man/Sequences/MaleNPC_Drowning_EngineReady.MaleNPC_Drowning_EngineReady" true)
          (Transformation|SetWorldTransform (Variables|Default|GetCapsuleComponent) (Math|Transform|MakeTransform "3780.000000,6161.000000,200.000000" "0.000000,-85.000000,0.000000") false true)
          (Pawn|UnPossess (AI|GetAIController self)))))))

(fn ConstructionScript
  (|CallParentFunction))