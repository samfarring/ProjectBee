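; Base Character for background human NPCs that can be stung, chased or targeted for quests, with a state widget and stub interface getters.
; Quest calls make the AI controller flee; chases poll a zone overlap and report when the NPC leaves.
; Damage triggers spine-down partial ragdoll, notifies the quest and recovers after a timed reset.
; BeybladeActive is set on the blackboard after a startup delay and on damage; capsule-follow ragdoll code is disconnected.
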(event Custom|GoRagdoll
  (bind _returnvalue (Utilities|Name|MakeLiteralName "HumanNPCRIGSpine1"))
  (bind _mesh (Variables|Character|GetMesh))
  ;[1 1 1] Ragdoll Controls
  (if (Variables|Ragdoll|GetCanRagdoll)
    (Class|SkeletalMeshComponent|SetAllBodiesBelowSimulatePhysics _mesh _returnvalue true true)
    (Class|SkeletalMeshComponent|SetAllBodiesBelowPhysicsBlendWeight _mesh _returnvalue 0.5 false true)
    (Variables|Ragdoll|SetInRagdoll true)
    (Pawn|Components|CharacterMovement|SetMovementMode (Variables|Character|GetCharacterMovement) "MOVE_Walking" 0)))

(event Custom|Init_AI_UI
  ;[1 1 1] Spacial UI
  (bind _returnvalue (UserInterface|CreateWidget "/Game/Widgets/W_stateAIwidget.W_stateAiWidget_C"))
  (bind _output_get (Variables|UI|SetstateUIref _returnvalue))
  (UserInterface|SetWidget (Variables|Default|GetstateUI) _output_get))

(event Custom|StungReset
  ;[1 1 1] On Stung
  (Rendering|SetVisibility (Variables|Default|GetStungText) false false)
  (Utilities|FlowControl|Delay 1e+01)
  (CallFunction|NoRagdoll))

(event Custom|ChaseZoneCheck
  (if (not (Class|PrimitiveComponent|IsOverlappingComponent (Variables|Collision|GetCapsuleComponent) (stale EventChaseNPC Zone)))
    (Utilities|FlowControl|DoOnce false
      (:Completed
        (Default|ChaseNPCReturn (stale EventChaseNPC Quest))
        (Utilities|Time|ClearandInvalidateTimerbyHandle (stale EventChaseNPC _returnvalue))))))

(event Custom|NoRagdoll
  ;[1 1 1] Ragdoll Controls
  (Variables|Ragdoll|SetPhysicsAlpha 0.0)
  (Variables|Ragdoll|SetRecovering true)
  (Utilities|FlowControl|Delay 0.5)
  (Variables|Ragdoll|SetRecovering false)
  (Pawn|Components|CharacterMovement|SetMovementMode (Variables|Character|GetCharacterMovement) "MOVE_Walking" 0)
  (Variables|Ragdoll|SetInRagdoll false)
  (Class|SkeletalMeshComponent|SetAllBodiesBelowSimulatePhysics (Variables|Character|GetMesh) (Utilities|Name|MakeLiteralName "HumanNPCRIGSpine1") false false))

(event Custom|StartBeybladeAttack
  (AI|Components|Blackboard|SetValueasBool (AI|GetBlackboard self) (Variables|Combat|GetBeybladeActive) true))

(event EventTick
  (params (DeltaSeconds :type Float%20%28single-precision%29)))

(event EventSetCharacterSpeed
  (params (Speed :type Float%20%28single-precision%29))
  (Variables|/Script/Engine.CharacterMovementComponent|SetMaxWalkSpeed (Variables|Character|GetCharacterMovement) Speed))

(event Game|Damage|EventAnyDamage
  (params (Damage :type Float%20%28single-precision%29) (DamageType :type Damage%20Type%20Object%20Reference) (InstigatedBy :type Controller%20Object%20Reference) (DamageCauser :type Actor%20Object%20Reference))
  ;[1 1 1] On Stung
  (CallFunction|GoRagdoll)
  (Math|Integer|IncrementInt (Variables|Combat|GetStungAmount)
    (:%20%20
      (Rendering|SetVisibility (Variables|Default|GetStungText) true false)
      (Utilities|Time|SetTimerbyEvent (delegate Custom|StungReset) (Variables|Combat|GetStingResetTime))
      (Utilities|IsValid (stale EventStingNPC Quest)
        (:Is%20Valid
          (Default|StingQuestReturn (stale EventStingNPC Quest)))
        (:Is%20Not%20Valid
          _))
      (Default|CallOnStung)
      (AI|Components|Blackboard|SetValueasBool (AI|GetBlackboard self) (Variables|Combat|GetBeybladeActive) true)
      (if (Variables|Combat|GetIsTarget)
        (bind _output_get (Variables|Combat|SetIsTarget false))
        (Rendering|SetVisibility (Variables|Default|GetTargetText) _output_get false)))))

(event EventBeginPlay
  (bind _self self)
  ;[1 1 1] Init
  (Class|IAI|Init(Message) (AI|GetAIController _self) _self)
  (CallFunction|InitAIUI)
  (Utilities|FlowControl|Delay 1e+01)
  (CallFunction|StartBeybladeAttack))

(event EventAssignTarget
  (bind _output_get (Variables|Combat|SetIsTarget true))
  (Rendering|SetVisibility (Variables|Default|GetTargetText) _output_get false))

(event EventChaseNPC
  (params (Quest :type BP%20Quest%20Actor%20Object%20Reference) (Zone :type Sphere%20Component%20Object%20Reference))
  (Utilities|FlowControl|Sequence
    (:then_0
      (Utilities|FlowControl|DoOnce false) ; enters at Reset
    )
    (:then_1
      (bind _returnvalue (Utilities|Time|SetTimerbyEvent (delegate Custom|ChaseZoneCheck) 0.1 true))
      (Class|IAI|SetFlee(Message) (AI|GetAIController self)))))

(event EventStingNPC
  (params (Quest :type BP%20Quest%20Actor%20Object%20Reference))
  (Class|IAI|SetFlee(Message) (AI|GetAIController self)))

(event EventSetStateText
  (params (State :type E_AI_States%20Enum :default "NewEnumerator0"))
  ;[1 1 1] Spacial UI
  (Rendering|Components|TextRender|SetText (Variables|Default|GetStateText) (Utilities|Text|ToText(String) (Utilities|String|ToString(Byte) State)))
  (Default|TriggerStateChange (Variables|UI|GetstateUIref) State))

(fn ConstructionScript)

(fn CanPatrol
  (return (Variables|Movement|GetCanPatrolLevel)))

(fn GetCharacter
  (return self))

(fn GetChurchMarker
  (return 0))

(fn GetIsChaseable
  (return (Variables|Combat|GetIsChaseable)))

(fn GetPatrolZone
  (return "NewEnumerator0" "0, 0, 0"))

(fn GetPerceptionTarget
  (return 0))

(fn GetStateChange
  (return "NewEnumerator0"))