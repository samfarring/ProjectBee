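; BP_PeepingTom is an AI character that periodically pops its mesh up from a lowered position and sinks back.
; A looping timer plays a timeline that lerps mesh height, reversing after a pause.
; Damage fires OnStung, disables collision, stops the peep timer and sinks the mesh via a fast interpolation timer.
; After a delay it restores state, state widget and query collision, but does not restart peeping.
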(event Custom|Peep
  (if (Utilities|Enum|Equal(Enum) (Variables|Default|GetState) "NewEnumerator1")
    (bind (_direction _peep) (Timeline|PeepLine PlayFromStart)
      (:Update
        (if (not (Variables|Movement|GetIsStung))
          (Transformation|SetRelativeLocation (Variables|Default|GetSkeletalMesh) (Math|Vector|MakeVector 0.0 0.0 (Math|Float|Lerp -5e+01 0.0 _peep)) false true)))
      (:Finished
        (Utilities|FlowControl|Delay 4.0)
        (if (Utilities|Enum|Equal(Enum) _direction "Forward")
          (Timeline|PeepLine ReverseFromEnd))))))

(event Custom|Init_AI_UI
  (bind _returnvalue (UserInterface|CreateWidget "/Game/Widgets/W_stateAIwidget.W_stateAiWidget_C"))
  (bind _output_get (Variables|Default|SetstateUIref _returnvalue))
  (UserInterface|SetWidget (Variables|Default|GetstateUI) _output_get))

(event Custom|InterpLocation
  (bind _skeletalmesh (Variables|Default|GetSkeletalMesh))
  (bind _output_get (Variables|Movement|SetCurrentZ (Math|Interpolation|FInterptoConstant (.z (Variables|/Script/Engine.SceneComponent|GetRelativeLocation (Variables|Default|GetSkeletalMesh))) -5e+01 (Utilities|Time|GetWorldDeltaSeconds) 6e+01)))
  (Transformation|SetRelativeLocation _skeletalmesh (Math|Vector|MakeVector 0.0 0.0 _output_get) false false)
  (if (== (.z (Variables|/Script/Engine.SceneComponent|GetRelativeLocation _skeletalmesh)) -5e+01)
    (Utilities|FlowControl|Delay 5.0)
    (Utilities|Time|ClearandInvalidateTimerbyHandle (Variables|Movement|GetFleeHandle))
    (Variables|Default|SetState "NewEnumerator1")
    (Default|TriggerStateChange (Variables|Default|GetstateUIref) "NewEnumerator1")
    (Collision|SetCollisionEnabled (Variables|Default|GetSkeletalMesh) "QueryOnly")))

(event EventBeginPlay
  (Variables|Default|SetState "NewEnumerator1")
  (Transformation|SetRelativeLocation (Variables|Default|GetSkeletalMesh) "0, 0,-50.000000" false true)
  (CallFunction|InitAIUI)
  (bind _returnvalue (Utilities|Time|SetTimerbyEvent (delegate Custom|Peep) (Variables|Default|GetPeepTimer) true))
  (Variables|Movement|SetPeepHandle _returnvalue))

(event Game|Damage|EventAnyDamage
  (params (Damage :type Float%20%28single-precision%29) (DamageType :type Damage%20Type%20Object%20Reference) (InstigatedBy :type Controller%20Object%20Reference) (DamageCauser :type Actor%20Object%20Reference))
  (if (Utilities|Enum|Equal(Enum) (Variables|Default|GetState) "NewEnumerator1")
    (Variables|Default|SetState "NewEnumerator2")
    (Collision|SetCollisionEnabled (Variables|Default|GetSkeletalMesh) "NoCollision")
    (Default|CallOnStung)
    (Variables|Movement|SetIsStung true)
    (Utilities|Time|ClearandInvalidateTimerbyHandle (Variables|Movement|GetPeepHandle))
    (Default|TriggerStateChange (stale Custom|Init_AI_UI _output_get) "NewEnumerator3")
    (bind _returnvalue (Utilities|Time|SetTimerbyEvent (delegate Custom|InterpLocation) 0.01 true))
    (Variables|Movement|SetFleeHandle _returnvalue)))

(fn ConstructionScript)