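; AI controller for background bee-game pawns that react when they perceive the player-type BeeCharacter_BP.
; On init it copies the pawn's aggression and reaction flags, runs AI_BaseTree and starts a looping timer for the AI tick, which updates the pawn's state text.
; Perception switches between two reaction states by aggressiveness, then a timer restores the default.
; Getters expose state and target, and always report not chaseable.
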(event OnPerceptionUpdated(AIPerception)
  (params (UpdatedActors :type Array%20of%20Actor%20Object%20References))
  (for _array_element UpdatedActors
    (bind _info (Class|AIPerceptionComponent|GetActorsPerception (Variables|Default|GetAIPerception) _array_element))
    (Variables|Perception|SetPerceptionTarget (.Target (Utilities|Struct|BreakActorPerceptionBlueprintInfo _info)))
    (if (and (== (Utilities|GetClass (.Target (Utilities|Struct|BreakActorPerceptionBlueprintInfo _info))) "/Game/Blueprints/Character/BeeCharacter_BP.BeeCharacter_BP_C") (Variables|States|GetWillReactToBee))
      (if (Variables|States|GetIsAggressive)
        (Variables|States|SetStates "NewEnumerator3")
        (else
          (Variables|States|SetStates "NewEnumerator2")))
      (Utilities|Time|SetTimerbyEvent (EventDispatchers|CreateEvent :!event Custom|ResetState) (Variables|Timer|GetResetTime)))))

(event Custom|AI_Tick
  (Class|IAI|SetStateText(Message) (Pawn|GetControlledPawn) (Variables|States|GetStates)))

(event Custom|ResetState
  (Variables|States|SetStates "NewEnumerator1"))

(event EventInit
  (params (ControlledPawn :type BP%20Background%20AI%20Base%20Object%20Reference))
  (Variables|States|SetIsAggressive (Variables|/Game/Blueprints/AI/Character/BP_BackgroundAI_Base.BP_BackgroundAI_Base_C|GetIsAggressive ControlledPawn))
  (Variables|States|SetWillReactToBee (Variables|/Game/Blueprints/AI/Character/BP_BackgroundAI_Base.BP_BackgroundAI_Base_C|GetWillReactToBee ControlledPawn))
  (Utilities|Time|SetTimerbyEvent (EventDispatchers|CreateEvent :!event Custom|AI_Tick) (Variables|Tick|GetAITickRate) true)
  (CallFunction|InitVariables)
  (AI|RunBehaviorTree "/Game/Blueprints/AI/Tree/AI_BaseTree.AI_BaseTree"))

(fn ConstructionScript)

(fn InitVariables
  (Variables|States|SetStates "NewEnumerator1"))

(fn GetIsChaseable
  (return false))

(fn GetPerceptionTarget
  (return (Variables|Perception|GetPerceptionTarget)))

(fn GetStateChange
  (return (Variables|States|GetStates)))