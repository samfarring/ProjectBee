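; AI controller for the BeeKeeper boss, toggling its Beyblade attack through the Blackboard.
; StartBeybladeAttack sets the BeybladeActive key, and BeybladeAttackEnd clears it and sends an end message to the controlled pawn.
; BeginPlay starts a looping timer whose bound event is not evident, plus a delay with nothing after it.
; RandomDialogue is an empty stub, and some disconnected nodes never run.
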(event Custom|RandomDialogue)

(event Custom|StartBeybladeAttack
  (bind _self self)
  (bind _returnvalue (AI|GetBlackboard _self))
  (Utilities|IsValid _returnvalue
    (:Is%20Valid
      (AI|Components|Blackboard|SetValueasBool _returnvalue (Variables|Default|GetBeybladeActive) true))))

(event EventBeginPlay
  (|CallParentFunction)
  (Utilities|Time|SetTimerbyEvent (EventDispatchers|CreateEvent :!event Custom|RandomDialogue) 1e+01 true)
  (Utilities|FlowControl|Delay 1e+01))

(event EventBeybladeAttackEnd
  (bind _self self)
  (bind _returnvalue (AI|GetBlackboard _self))
  (Utilities|IsValid _returnvalue
    (:Is%20Valid
      (AI|Components|Blackboard|SetValueasBool _returnvalue (Variables|Default|GetBeybladeActive) false)
      (Class|IAI|BeybladeAttackEnd(Message) (Pawn|GetControlledPawn)))))

(fn ConstructionScript
  (|CallParentFunction))