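; I_AI is a Blueprint interface for AI characters and their controllers, declaring shared calls with no implementation.
; It covers state changes and display text, movement speed, pawn setup, perception targets, chasing, cowering, fleeing and attacks, including a start and end pair for a Beyblade attack.
; It also exposes queries for patrol permission and zones, a church marker, gender and current activity, suggesting villager-style NPCs alongside combatants.
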(fn GetStateChange
  (return "NewEnumerator0"))

(fn SetStateText
  (params (State :type E_AI_States%20Enum :default "NewEnumerator0")))

(fn SetCharacterSpeed
  (params (Speed :type Float%20%28single-precision%29)))

(fn GetPerceptionTarget
  (return 0))

(fn Init
  (params (ControlledPawn :type BP%20Background%20AI%20Base%20Object%20Reference)))

(fn AssignTarget)

(fn GetIsChaseable
  (return false))

(fn IsCowering
  (params (IsCowering :type Boolean))
  (return))

(fn Attack
  (params (Attacker :type Actor%20Object%20Reference)))

(fn CanPatrol
  (return false))

(fn GetPatrolZone
  (return "NewEnumerator0" "0, 0, 0"))

(fn SetFlee)

(fn BeybladeAttack)

(fn BeybladeAttackEnd)

(fn GetChurchMarker
  (return 0))

(fn GetGender
  (return false))

(fn GetActivity
  (return "NewEnumerator0"))

(fn GetActivityActive
  (return false))