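; Test pawn for the game's UI, with a viewport widget and a to-do list of prank objectives on a widget component.
; Show and hide events start looping timers that ease an alpha, sliding the list vertically through LerpLocalOffset.
; Debug keys complete objectives, swap the objective list, trigger a checkpoint on the UI widget and show or hide the list.
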(event Custom|MoveTodoListUp
  ;[0.5211 0.2619 1] WidgetComponentSmoothLerpMovement
  (Utilities|LerpLocalOffset)
  (bind _output_get (Variables|Default|SettodoListLerpAlph (- (Variables|Default|GettodoListLerpAlph) (* (Variables|Default|GettodoListLerpAlph) 0.1))))
  (if (< _output_get 0.001)
    (Variables|Default|SettodoListLerpAlph 0.0)
    (Utilities|Time|ClearandInvalidateTimerbyHandle (Variables|Default|GetMoveTodoListUpTimerRef))))

(event Custom|MoveTodoListDown
  ;[0.5211 0.2619 1] WidgetComponentSmoothLerpMovement
  (Utilities|LerpLocalOffset)
  (if (< (Variables|Default|GettodoListLerpAlph) 0.99)
    (Variables|Default|SettodoListLerpAlph (+ (Variables|Default|GettodoListLerpAlph) (* (Variables|Default|GettodoListLerpAlph) 0.1) 0.002))
    (else
      (Variables|Default|SettodoListLerpAlph 1.0)
      (Utilities|Time|ClearandInvalidateTimerbyHandle (Variables|Default|GetMoveTodoListDownTimerRef)))))

(event Custom|ShowTodoList
  ;[0.5211 0.2619 1] WidgetComponentSmoothLerpMovement
  (Utilities|Time|ClearandInvalidateTimerbyHandle (Variables|Default|GetMoveTodoListUpTimerRef))
  (Utilities|Time|ClearandInvalidateTimerbyHandle (Variables|Default|GetMoveTodoListDownTimerRef))
  (bind _returnvalue (Utilities|Time|SetTimerbyEvent (EventDispatchers|CreateEvent :!event Custom|MoveTodoListUp) 0.01 true))
  (Variables|Default|SetMoveTodoListUpTimerRef _returnvalue))

(event Custom|HideTodoList
  ;[0.5211 0.2619 1] WidgetComponentSmoothLerpMovement
  (Utilities|Time|ClearandInvalidateTimerbyHandle (Variables|Default|GetMoveTodoListUpTimerRef))
  (Utilities|Time|ClearandInvalidateTimerbyHandle (Variables|Default|GetMoveTodoListDownTimerRef))
  (bind _returnvalue (Utilities|Time|SetTimerbyEvent (EventDispatchers|CreateEvent :!event Custom|MoveTodoListDown) 0.01 true))
  (Variables|Default|SetMoveTodoListDownTimerRef _returnvalue))

(event Custom|Init_Pawn
  (bind _returnvalue (UserInterface|CreateWidget 0))
  (bind _output_get (Variables|Default|Setwig_UIRef 0 _returnvalue))
  (UserInterface|Viewport|AddtoViewport _output_get 0)
  (bind _returnvalue_2 (UserInterface|CreateWidget 0))
  (bind _output_get_2 (Variables|Default|Setwig_toDoListRef 0 _returnvalue_2))
  (UserInterface|SetWidget (Variables|Default|Getwigc_todoList) _output_get_2)
  (CallFunction|InitWigTodoList (.wig_toDoListRef (Variables|Default|Getwig_toDoListRef)))
  (Transformation|SetRelativeLocation (Variables|Default|Getwigc_todoList) (Math|Vector|MakeVector 24.0 -7.0 -3e+01) false false)
  (CallFunction|UpdateObjectiveList (.wig_toDoListRef (Variables|Default|Getwig_toDoListRef)) (Utilities|Array|MakeArray "Knock the fruit and veg stall over" "Smell the flowers at the flower stall " "Get the dog an ice cream")))

(event EventBeginPlay
  (bind _returnvalue (UserInterface|CreateWidget 0))
  (bind _output_get (Variables|Default|Setwig_UIRef 0 _returnvalue))
  (UserInterface|Viewport|AddtoViewport _output_get 0)
  (bind _returnvalue_2 (UserInterface|CreateWidget 0))
  (bind _output_get_2 (Variables|Default|Setwig_toDoListRef 0 _returnvalue_2))
  (UserInterface|SetWidget (Variables|Default|Getwigc_todoList) _output_get_2)
  (CallFunction|InitWigTodoList (.wig_toDoListRef (Variables|Default|Getwig_toDoListRef)))
  (Transformation|SetRelativeLocation (Variables|Default|Getwigc_todoList) (Math|Vector|MakeVector 24.0 -7.0 -3e+01) false false)
  (CallFunction|UpdateObjectiveList (.wig_toDoListRef (Variables|Default|Getwig_toDoListRef)) (Utilities|Array|MakeArray "Knock the fruit and veg stall over" "Smell the flowers at the flower stall " "Get the dog an ice cream")))

(event Input|KeyboardEvents|C
  (params (Key :type Key%20Structure))
  ;[1 0.8639 0.08897 0.156] Debug
  (:Pressed
    (CallFunction|TriggerCheckpoint (.wig_UIRef (Variables|Default|Getwig_UIRef)))))

(event Input|KeyboardEvents|Up
  (params (Key :type Key%20Structure))
  ;[1 0.8639 0.08897 0.156] Debug
  (:Pressed
    (CallFunction|ShowTodoList)))

(event Input|KeyboardEvents|Down
  (params (Key :type Key%20Structure))
  ;[1 0.8639 0.08897 0.156] Debug
  (:Pressed
    (CallFunction|HideTodoList)))

(event Input|KeyboardEvents|1
  (params (Key :type Key%20Structure))
  ;[1 0.8639 0.08897 0.156] Debug
  (:Pressed
    (CallFunction|CompletedObjective (.wig_toDoListRef (Variables|Default|Getwig_toDoListRef)))))

(event Input|KeyboardEvents|2
  (params (Key :type Key%20Structure))
  ;[1 0.8639 0.08897 0.156] Debug
  (:Pressed
    (CallFunction|CompletedObjective (.wig_toDoListRef (Variables|Default|Getwig_toDoListRef)) 1)))

(event Input|KeyboardEvents|3
  (params (Key :type Key%20Structure))
  ;[1 0.8639 0.08897 0.156] Debug
  (:Pressed
    (CallFunction|CompletedObjective (.wig_toDoListRef (Variables|Default|Getwig_toDoListRef)) 2)))

(event Input|KeyboardEvents|4
  (params (Key :type Key%20Structure))
  ;[1 0.8639 0.08897 0.156] Debug
  (:Pressed
    (CallFunction|CompletedObjective (.wig_toDoListRef (Variables|Default|Getwig_toDoListRef)) 3)))

(event Input|KeyboardEvents|5
  (params (Key :type Key%20Structure))
  ;[1 0.8639 0.08897 0.156] Debug
  (:Pressed
    (CallFunction|CompletedObjective (.wig_toDoListRef (Variables|Default|Getwig_toDoListRef)) 4)))

(event Input|KeyboardEvents|0
  (params (Key :type Key%20Structure))
  ;[1 0.8639 0.08897 0.156] Debug
  (:Pressed
    (CallFunction|UpdateObjectiveList (.wig_toDoListRef (Variables|Default|Getwig_toDoListRef)) (Utilities|Array|MakeArray "bounce on the trampoline" "Push the child off the swings " "Turn on the sprinklers " "Knock a brick on to the other end of a see saw makes a child go flying" "Bounce on the trampoline "))))

(fn ConstructionScript)