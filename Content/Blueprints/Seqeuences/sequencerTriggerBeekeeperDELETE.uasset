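; Trigger volume that starts the beekeeper cutscene once, when the player's bee character (BeeCharacter_BP) overlaps its box.
; It plays the referenced level sequence and adds the beekeeper logo widget with a black cutscene-enter animation.
; A short timer then plays the logo popup and shows its holder.
; A SequenceEnded event, not bound or called within this Blueprint, removes the widget.
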(event OnComponentBeginOverlap(Box)
  (params (OverlappedComponent :type Primitive%20Component%20Object%20Reference) (OtherActor :type Actor%20Object%20Reference) (OtherComp :type Primitive%20Component%20Object%20Reference) (OtherBodyIndex :type Integer) (bFromSweep :type Boolean) (SweepResult :type Hit%20Result%20Structure%20%28by%20ref%29))
  (Utilities|Casting|CastToBeeCharacter_BP OtherActor)
  (if (not (Variables|Default|GettriggeredSequence))
    (Variables|Default|SettriggeredSequence true)
    (Sequencer|Player|Play (Variables|/Script/LevelSequence.LevelSequenceActor|GetSequencePlayer (Variables|Default|GetbeekeeperSequenceRef)) :!class /Script/MovieScene.MovieSceneSequencePlayer)
    (bind _returnvalue (UserInterface|CreateWidget "/Game/Widgets/W_beekeeperLogo.W_beekeeperLogo_C"))
    (bind _output_get (Variables|Default|SetbeekeeperLogoWigRef _returnvalue))
    (UserInterface|Viewport|AddtoViewport _output_get 0)
    (UserInterface|Animation|PlayAnimation _output_get (Variables|/Game/Widgets/W_beekeeperLogo.W_beekeeperLogo_C|Getanim_cutsceneBlackEnter _output_get) 0.0 1 "Forward" 1.0)
    (Utilities|Time|SetTimerbyEvent (delegate Custom|showLogo) 1.6)))

(event Custom|showLogo
  (UserInterface|Animation|PlayAnimation (stale OnComponentBeginOverlap(Box) _output_get) (Variables|/Game/Widgets/W_beekeeperLogo.W_beekeeperLogo_C|Getanim_beeKeeperLogoPopup (stale OnComponentBeginOverlap(Box) _output_get)) 0.0 1 "Forward" 1.0)
  (Widget|SetVisibility (Variables|/Game/Widgets/W_beekeeperLogo.W_beekeeperLogo_C|Getcan_logoHolder (stale OnComponentBeginOverlap(Box) _output_get)) "HitTestInvisible"))

(event Custom|SequenceEnded
  (Widget|RemovefromParent (Variables|Default|GetbeekeeperLogoWigRef)))

(fn ConstructionScript)